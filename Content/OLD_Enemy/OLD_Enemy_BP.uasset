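; Legacy enemy Blueprint that roams between preset target actors and triggers game over when it hits the FirstPersonCharacter.
; On BeginPlay, and when Tick finds it within tolerance of its target, it picks a random preset location and writes it to the AI blackboard's TargetLocation key.
; Hitting the player shows the GameOver widget, disables their input and reveals the cursor.
; Debug output draws a line to the target and prints each new location.
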(event `self.ReceiveBeginPlay`
  (`self.SetNewRandomLocation`))

(event `self.ReceiveTick`
  (params (DeltaSeconds :type "Float (single-precision)"))
  (`self.DebugDrawLineToTarget`)
  (if (== (- (`self.K2_GetActorLocation`) (`self.CurrentTargetLocation`)) (0.0 0.0 0.0) :`ErrorTolerance` 200.0)
    (`self.SetNewRandomLocation`)))

(event `self.ReceiveHit`
  (params (MyComp :type "PrimitiveComponent Object Reference") (Other :type "Actor Object Reference") (OtherComp :type "PrimitiveComponent Object Reference") (bSelfMoved :type Boolean) (HitLocation :type "Vector Structure") (HitNormal :type "Vector Structure") (NormalImpulse :type "Vector Structure") (Hit :type "HitResult Structure (by ref)"))
  (bind _returnvalue (`GameplayStatics.GetPlayerController` 0))
  (bind _asfirst_person_character (cast `/Game/Blueprints/FirstPersonCharacter` Other))
  (bind _returnvalue_2 (`|CreateWidget` "/Game/Blueprints/GameOver_WidgetBP.GameOver_WidgetBP_C" _returnvalue))
  (`UserWidget.AddToViewport` _returnvalue_2 0)
  (`self.DisableInput` _asfirst_person_character _returnvalue)
  (set `PlayerController.bShowMouseCursor` true _returnvalue))

(fn `DebugDrawLineToTarget`
  (`KismetSystemLibrary.DrawDebugLine` (+ (`self.K2_GetActorLocation`) (0.0 0.0 5.0)) (+ (`self.CurrentTargetLocation`) (0.0 0.0 5.0)) (struct :`A` 1.0) 0.01 8.0))

(fn `SetNewRandomLocation`
  (bind _presettargets (`self.PresetTargets`))
  (bind _output_get (set `self.CurrentTargetLocation` (`self.K2_GetActorLocation` (`|GetArrayItem` _presettargets (`KismetMathLibrary.RandomInteger` (`KismetArrayLibrary.Array_Length` _presettargets))))))
  (`BlackboardComponent.SetValueAsVector` (`AIBlueprintHelperLibrary.GetBlackboard` (`AIBlueprintHelperLibrary.GetAIController` self)) "TargetLocation" _output_get)
  (`KismetSystemLibrary.PrintString` (`KismetStringLibrary.Conv_VectorToString` _output_get)))

(fn `UserConstructionScript`)