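; Legacy enemy AI controller that runs a behavior tree for patrolling guard points and reacting to noise.
; On BeginPlay it starts the tree and writes four guard points to the Blackboard, leaving patrol order to the tree.
; PawnSensing hearing events store the noise location as the Blackboard's TargetLocation.
; A random wandering loop and a debug print remain in the graph but never run.
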(event `self.ReceiveBeginPlay`
  (`self.RunBehaviorTree` (`self.BehaviourTree`))
  ;[1 1 1] For setting 4 target points for the enemy - sequence order can be changed in behaviour tree
  (cast `` (`self.K2_GetPawn`))
  (`BlackboardComponent.SetValueAsObject` (`AIBlueprintHelperLibrary.GetBlackboard` self) "GuardPoint1" (`self.GuardPoint1`))
  (`BlackboardComponent.SetValueAsObject` (`AIBlueprintHelperLibrary.GetBlackboard` self) "GuardPoint2" (`self.GuardPoint2`))
  (`BlackboardComponent.SetValueAsObject` (`AIBlueprintHelperLibrary.GetBlackboard` self) "GuardPoint3" (`self.GuardPoint3`))
  (`BlackboardComponent.SetValueAsObject` (`AIBlueprintHelperLibrary.GetBlackboard` self) "GuardPoint4" (`self.GuardPoint4`)))

(event `self.PawnSensing.OnHearNoise`
  (params (Instigator :type "Pawn Object Reference") (Location :type "Vector Structure (by ref)") (Volume :type "Float (single-precision)"))
  (cast `` (`self.K2_GetPawn`))
  (bind _output_get (set `self.CurrentTargetLocation` Location))
  (`BlackboardComponent.SetValueAsVector` (`AIBlueprintHelperLibrary.GetBlackboard` self) "TargetLocation" _output_get))

(fn `UserConstructionScript`)