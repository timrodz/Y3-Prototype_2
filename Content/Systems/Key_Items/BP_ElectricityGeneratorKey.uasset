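; Key item pickup that represents a missing piece of an electricity generator.
; Interact calls the parent, then uses MissingPieceNumber in an insert into the referenced Generator's MissingPiecesCollected array.
; It then hides itself, flags itself as picked up and destroys the actor.
; If PlaySound is set, it plays a 2D piano effect and returns the picked-up flag, with that return wired only on this branch.
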(fn `Interact`
  (params (ActorInstigator :type "Actor Object Reference"))
  (returns (ReturnValue :type Boolean))
  (`parent.Interact` null)
  (`KismetArrayLibrary.Array_Insert` (`/Game/Systems/Key_Items/BP_ElectricityGenerator.MissingPiecesCollected` (`self.Generator`)) 1 (`self.Missing Piece Number`))
  (`self.SetActorHiddenInGame` true)
  (bind _output_get (set `self.IsPickedUp` true))
  (`self.K2_DestroyActor`)
  (if (`self.PlaySound`)
    (`GameplayStatics.PlaySound2D` "/Game/Audio/Piano_FX.Piano_FX")
    (return _output_get)))

(fn `UserConstructionScript`)