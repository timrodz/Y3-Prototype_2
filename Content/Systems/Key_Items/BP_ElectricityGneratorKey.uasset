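; Pickup key item that serves as a missing piece for BP_ElectricityGenerator.
; Actor overlap toggles an interact flag, allowing a T key press to collect the piece.
; Collection inserts an entry into the first found generator's MissingPiecesCollected array using this piece's number, then flags the item as picked up.
; The pickup also calls SetActorHiddenInGame with false, so the actor is not hidden.
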(event `self.ReceiveActorBeginOverlap`
  (params (OtherActor :type "Actor Object Reference"))
  (set `self.InteractQuery` true))

(event `self.ReceiveActorEndOverlap`
  (params (OtherActor :type "Actor Object Reference"))
  (set `self.InteractQuery` false))

(event `Key|T`
  (params (Key :type "Key Structure" :default "AnyKey"))
  (:`Pressed`
    (if (`self.InteractQuery`)
      (bind _outactors (`GameplayStatics.GetAllActorsOfClass` "/Game/Systems/Key_Items/BP_ElectricityGenerator.BP_ElectricityGenerator_C"))
      (`KismetArrayLibrary.Array_Insert` (`/Game/Systems/Key_Items/BP_ElectricityGenerator.MissingPiecesCollected` (`|GetArrayItem` _outactors)) 1 (`self.Missing Piece Number`))
      (`self.SetActorHiddenInGame` false)
      (set `self.IsPickedUp` true))))

(fn `UserConstructionScript`)