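; Key item actor for an electricity generator with missing pieces to be fitted into slots, currently an unfinished interaction prototype.
; Pressing E sets an interact flag, and slot hits by the first-person character then print the component name; other hits clear the flag.
; AttachMissingPiece swaps in slot meshes and counts pieces, but nothing here calls it.
; Its case 2 reuses slot 0's mesh and component.
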(event `Key|E`
  (params (Key :type "Key Structure" :default "AnyKey"))
  (:`Pressed`
    (set `self.InteractQuery` true)))

(event `self.Slot_0.OnComponentHit`
  (params (HitComponent :type "PrimitiveComponent Object Reference") (OtherActor :type "Actor Object Reference") (OtherComp :type "PrimitiveComponent Object Reference") (NormalImpulse :type "Vector Structure") (Hit :type "HitResult Structure (by ref)"))
  (`self.CanInteractWithComponent` HitComponent OtherActor))

(event `self.Slot_1.OnComponentHit`
  (params (HitComponent :type "PrimitiveComponent Object Reference") (OtherActor :type "Actor Object Reference") (OtherComp :type "PrimitiveComponent Object Reference") (NormalImpulse :type "Vector Structure") (Hit :type "HitResult Structure (by ref)"))
  (`self.CanInteractWithComponent` HitComponent OtherActor))

(event `self.Slot_2.OnComponentHit`
  (params (HitComponent :type "PrimitiveComponent Object Reference") (OtherActor :type "Actor Object Reference") (OtherComp :type "PrimitiveComponent Object Reference") (NormalImpulse :type "Vector Structure") (Hit :type "HitResult Structure (by ref)"))
  (`self.CanInteractWithComponent` HitComponent OtherActor))

(fn `AttachMissingPiece`
  (params (PieceNumber :type Integer))
  (switch `int` PieceNumber
    (:`0`
      ;[0.7916 0.2622 1] Attach missing piece #0
      (`StaticMeshComponent.SetStaticMesh` (`self.Slot_0`) (`self.Missing_Piece_0`)))
    (:`1`
      ;[0.7916 0.2622 1] Attach missing piece #1
      (`StaticMeshComponent.SetStaticMesh` (`self.Slot_1`) (`self.Missing_Piece_1`)))
    (:`2`
      ;[0.7916 0.2622 1] Attach missing piece #2
      (`StaticMeshComponent.SetStaticMesh` (`self.Slot_0`) (`self.Missing_Piece_0`))))
  (`/Engine/EditorBlueprintResources/StandardMacros.IncrementInt` (`self.MissingPiecesAttached`)))

(fn `CanInteractWithComponent`
  (params (`Main Collider` :type "PrimitiveComponent Object Reference") (`Other Collider` :type "Actor Object Reference"))
  (returns (CanInteract :type Boolean))
  (cast `/Game/Blueprints/FirstPersonCharacter` `Other Collider`
    (:`then`
      (if (`self.InteractQuery`)
        (`KismetSystemLibrary.PrintString` (`KismetStringLibrary.Concat_StrStr` "Collision with: " (`KismetSystemLibrary.GetDisplayName` `Main Collider`)))
        (return (`self.InteractQuery`))))
    (:`CastFailed`
      (set `self.InteractQuery` false)
      (return false))))

(fn `UserConstructionScript`)