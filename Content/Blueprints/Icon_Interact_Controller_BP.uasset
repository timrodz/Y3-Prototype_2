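; Controller that switches the interact icon on interactable objects between keyboard and gamepad variants.
; CheckKey tests whether the given key is a gamepad key and tracks the last input type, which starts as keyboard on BeginPlay.
; Only when the input type changes, it finds every BP_InteractableObject in the level and sets its InteractIcon to A_Button for gamepad or Door_Button for keyboard.
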(event `self.ReceiveBeginPlay`
  (set `self.LastPressKeyboard` true))

(fn `CheckKey`
  (params (Key :type "Key Structure" :default "AnyKey"))
  (bind _lastpresskeyboard (`self.LastPressKeyboard`))
  (if (`KismetInputLibrary.Key_IsGamepadKey` Key)
    (if _lastpresskeyboard
      (set `self.LastPressKeyboard` false)
      (bind _outactors (`GameplayStatics.GetAllActorsOfClass` "/Game/Blueprints/BaseClasses/BP_InteractableObject.BP_InteractableObject_C"))
      (for _array_element _outactors
        (set `InteractableObject.InteractIcon` "/Game/Icons/A_Button.A_Button" _array_element)))
    (elif (not _lastpresskeyboard)
      (set `self.LastPressKeyboard` true)
      (bind _outactors_2 (`GameplayStatics.GetAllActorsOfClass` "/Game/Blueprints/BaseClasses/BP_InteractableObject.BP_InteractableObject_C"))
      (for _array_element_2 _outactors_2
        (set `InteractableObject.InteractIcon` "/Game/Assets/2D/UI/Door_Button.Door_Button" _array_element_2)))))

(fn `UserConstructionScript`)