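; Pushable interactable Blueprint, currently an unfinished stub with no push movement.
; Interact calls the parent implementation, then hides the instigator in game if it is a FirstPersonCharacter, and returns the parent's result.
; The event graph holds disconnected debug logic that compares world X/Y positions to print the character's side as Left, Right, Front or Back; it never runs.
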(event `self.ReceiveActorBeginOverlap`
  (params (OtherActor :type "Actor Object Reference")))

(fn `Interact`
  (params (ActorInstigator :type "Actor Object Reference"))
  (returns (ReturnValue :type Boolean))
  (bind _returnvalue (`parent.Interact` null))
  (bind _asfirst_person_character (cast `/Game/Blueprints/FirstPersonCharacter` ActorInstigator))
  (`self.SetActorHiddenInGame` _asfirst_person_character true)
  (return _returnvalue))

(fn `UserConstructionScript`
  (`parent.UserConstructionScript`))