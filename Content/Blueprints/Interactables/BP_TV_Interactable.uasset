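; Interactable TV that the player toggles on and off, starting in the off state.
; BeginPlay spawns an attenuated, non-auto-destroying static noise sound, stops it at once, and keeps it for reuse.
; Interact calls its parent, then flips the On flag while starting or stopping the static, swapping the screen material, playing a switch click and toggling an optional referenced light's visibility.
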(event `self.ReceiveBeginPlay`
  (bind _light (`self.Light`))
  (bind _returnvalue (`GameplayStatics.SpawnSoundAtLocation` "/Game/Audio/Sounds/Static/continuous-static.continuous-static" (`self.K2_GetActorLocation`) (struct) 0.35 1.0 0.0 "/Game/Audio/Attenuation/TV_Attenuation.TV_Attenuation" null false))
  (bind _output_get (set `self.StaticNoiseAudioComponent` _returnvalue))
  (`AudioComponent.Stop` _output_get)
  (`PrimitiveComponent.SetMaterial` (`self.TV_Mesh`) 1 (`self.MaterialOff`))
  (`/Engine/EditorBlueprintResources/StandardMacros.IsValid` _light
    (:`Is Valid`
      (`SceneComponent.SetVisibility` (`Light.LightComponent` _light) false false))))

(fn `Interact`
  (params (ActorInstigator :type "Actor Object Reference"))
  (returns (ReturnValue :type Boolean))
  (bind _tv_mesh (`self.TV_Mesh`))
  (bind _light (`self.Light`))
  (bind _light_2 (`self.Light`))
  (bind _returnvalue (`SceneComponent.K2_GetComponentLocation` _tv_mesh))
  (bind _returnvalue_2 (`parent.Interact` null))
  (if (`self.bOn`)
    (`AudioComponent.Stop` (`self.StaticNoiseAudioComponent`))
    (`PrimitiveComponent.SetMaterial` _tv_mesh 1 (`self.MaterialOff`))
    (`GameplayStatics.PlaySoundAtLocation` "/Game/Audio/Sounds/Buttons/Others/Switch_Push_1.Switch_Push_1" _returnvalue)
    (`/Engine/EditorBlueprintResources/StandardMacros.IsValid` _light_2
      (:`Is Valid`
        (`SceneComponent.SetVisibility` (`Light.LightComponent` _light_2) false false))
      (:`Is Not Valid`
        _))
    (else
      (`AudioComponent.Play` (`self.StaticNoiseAudioComponent`) 0.0)
      (`PrimitiveComponent.SetMaterial` _tv_mesh 1 (`self.MaterialOn`))
      (`GameplayStatics.PlaySoundAtLocation` "/Game/Audio/Sounds/Buttons/Others/Switch_Push_3.Switch_Push_3" _returnvalue)
      (`/Engine/EditorBlueprintResources/StandardMacros.IsValid` _light
        (:`Is Valid`
          (`SceneComponent.SetVisibility` (`Light.LightComponent` _light) true false))
        (:`Is Not Valid`
          _))))
  (set `self.bOn` (not (`self.bOn`)))
  (return _returnvalue_2))

(fn `UserConstructionScript`
  (`parent.UserConstructionScript`))