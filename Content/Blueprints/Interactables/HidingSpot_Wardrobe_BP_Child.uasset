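; Wardrobe hiding spot interactable that lets the player hide inside, with a breath-holding hint on early uses.
; Player interaction toggles hiding: timelines swing the doors and lerp the player's capsule in or out while input and collision are disabled.
; An overlapping enemy plays a shaking sound and builds a timer while the player hides.
; When it expires, an enemy whose blackboard target is nearby opens the doors, killing the player.
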(event `self.ReceiveBeginPlay`
  (bind _returnvalue (`GameplayStatics.SpawnSoundAtLocation` "/Game/Audio/Sounds/Impacts/Earthquake_Shake.Earthquake_Shake" (`self.K2_GetActorLocation`) (struct) 1.0 1.0 0.0 "/Game/Audio/Attenuation/TV_Attenuation.TV_Attenuation" null false))
  (bind _output_get (set `self.ShakingSoundAudioComponent` _returnvalue))
  (`AudioComponent.Stop` _output_get)
  (bind _returnvalue_2 (`GameplayStatics.SpawnSoundAtLocation` "/Game/Audio/Sounds/Doors/Wardrobe_Open_Close_Short.Wardrobe_Open_Close_Short" (`self.K2_GetActorLocation`) (struct) 1.0 1.0 0.0 "/Game/Audio/Attenuation/TV_Attenuation.TV_Attenuation" null false))
  (bind _output_get_2 (set `self.OpenCloseAudioComponent` _returnvalue_2))
  (`AudioComponent.Stop` _output_get_2))

(event `self.ReceiveTick`
  (params (DeltaSeconds :type "Float (single-precision)"))
  (if (and (`self.EnemyIsOverlapping`) (`self.PlayerHidingInside`))
    (set `self.EnemyTimer` (+ DeltaSeconds (`self.EnemyTimer`)))
    (if (not (`AudioComponent.IsPlaying` (`self.ShakingSoundAudioComponent`)))
      (`AudioComponent.Play` (`self.ShakingSoundAudioComponent`) 0.0))
    (if (> (`self.EnemyTimer`) 12.0)
      (`AudioComponent.FadeOut` (`self.ShakingSoundAudioComponent`) 1.0 0.0)
      (set `self.EnemyTimer` 0.0)
      (if (`self.PlayerHidingInside`)
        (if (<= (`KismetMathLibrary.VSize` (- (`BlackboardComponent.GetValueAsVector` (`AIBlueprintHelperLibrary.GetBlackboard` (`self.Enemy`)) "TargetLocation") (`self.K2_GetActorLocation`))) 250.0)
          (`self.Interact` (`self.Enemy`)))))))

(event `Play`
  (params (Player :type "/Game/Blueprints/FirstPersonCharacter/FirstPersonCharacter Object Reference"))
  (bind _asplayer_controller (cast `PlayerController` (`Pawn.GetController` Player) :!pure true))
  (`/Engine/EditorBlueprintResources/StandardMacros.FlipFlop`
    (:`A`
      (`self.DisableInput` Player _asplayer_controller)
      (bind (_direction _rotationto90) (`Timeline|SwingDoors` :!via `PlayFromStart` :!label _label)
        (:`Update`
          (`|ExecutionSequence`
            (:`then_0`
              (`SceneComponent.K2_SetRelativeRotation` (`self.StaticMesh1`) (`KismetMathLibrary.MakeRotator` 0.0 0.0 _rotationto90) false false))
            (:`then_1`
              (`SceneComponent.K2_SetRelativeRotation` (`self.StaticMesh`) (`KismetMathLibrary.MakeRotator` 0.0 0.0 (* _rotationto90 -1.0)) false false))))
        (:`Finished`
          (`/Engine/EditorBlueprintResources/StandardMacros.FlipFlop`
            (:`A`
              (`PrimitiveComponent.SetCollisionEnabled` (`self.Cube`) "NoCollision")
              (`PrimitiveComponent.SetCollisionEnabled` (`self.StaticMesh`) "NoCollision")
              (`PrimitiveComponent.SetCollisionEnabled` (`self.StaticMesh1`) "NoCollision")
              (`self.Camera_Anim` Player)
              (goto _label :!via `ReverseFromEnd`))
            (:`B`
              (`PrimitiveComponent.SetCollisionEnabled` (`self.Cube`) "QueryAndPhysics")
              (`PrimitiveComponent.SetCollisionEnabled` (`self.StaticMesh`) "QueryAndPhysics")
              (`PrimitiveComponent.SetCollisionEnabled` (`self.StaticMesh1`) "QueryAndPhysics")
              (`self.EnableInput` Player _asplayer_controller))))))
    (:`B`
      (goto _label :!via `PlayFromStart`))))

(event `Camera_Anim`
  (params (Player :type "/Game/Blueprints/FirstPersonCharacter/FirstPersonCharacter Object Reference"))
  (bind _capsulecomponent (`Character.CapsuleComponent` Player))
  (bind _isa (`/Engine/EditorBlueprintResources/StandardMacros.FlipFlop`)
    (:`A`
      (bind (_direction _newtrack_1) (`Timeline|Camera_Lerp` :!via `PlayFromStart` :!label _label_2)
        (:`Update`
          (if _isa
            (`SceneComponent.K2_SetWorldLocationAndRotation` _capsulecomponent (`KismetMathLibrary.VLerp` (`SceneComponent.K2_GetComponentLocation` _capsulecomponent) (`SceneComponent.K2_GetComponentLocation` (`self.Scene`)) _newtrack_1) (`KismetMathLibrary.RLerp` (`SceneComponent.K2_GetComponentRotation` _capsulecomponent) (`SceneComponent.K2_GetComponentRotation` (`self.Cube`)) _newtrack_1) false false)
            (else
              (`SceneComponent.K2_SetWorldLocationAndRotation` _capsulecomponent (`KismetMathLibrary.VLerp` (`SceneComponent.K2_GetComponentLocation` _capsulecomponent) (`SceneComponent.K2_GetComponentLocation` (`self.Return`)) _newtrack_1) (`KismetMathLibrary.RLerp` (`SceneComponent.K2_GetComponentRotation` _capsulecomponent) (`SceneComponent.K2_GetComponentRotation` (`self.Cube`)) _newtrack_1) false false))))))
    (:`B`
      (goto _label_2 :!via `PlayFromStart`))))

(event `EnemyPlayOpen`
  (bind _opencloseaudiocomponent (`self.OpenCloseAudioComponent`))
  (`AudioComponent.SetPitchMultiplier` _opencloseaudiocomponent (`KismetMathLibrary.RandomFloatInRange` 0.6 1.4))
  (`AudioComponent.Play` _opencloseaudiocomponent 0.0)
  (bind (_direction _rotationto90) (`Timeline|EnemyOpen`)
    (:`Update`
      (`|ExecutionSequence`
        (:`then_0`
          (`SceneComponent.K2_SetRelativeRotation` (`self.StaticMesh1`) (`KismetMathLibrary.MakeRotator` 0.0 0.0 _rotationto90) false false))
        (:`then_1`
          (`SceneComponent.K2_SetRelativeRotation` (`self.StaticMesh`) (`KismetMathLibrary.MakeRotator` 0.0 0.0 (* _rotationto90 -1.0)) false false))))
    (:`Finished`
      (if (`self.PlayerHidingInside`)
        (`/Game/Blueprints/FirstPersonCharacter/FirstPersonCharacter.Die` (`self.Player`))
        (`AudioComponent.FadeOut` (`self.ShakingSoundAudioComponent`) 1.0 0.0)
        (set `self.PlayerHidingInside` false)
        (`KismetSystemLibrary.Delay` 0.2)
        (`TimelineComponent.ReverseFromEnd` (`self.EnemyOpen`))
        (`KismetSystemLibrary.Delay` 1.0)
        (set `/Game/Blueprints/FirstPersonCharacter/FirstPersonCharacter.Dying` false (`self.Player`))))))

(event `self.ReceiveActorBeginOverlap`
  (params (OtherActor :type "Actor Object Reference"))
  (bind _asbp_enemy_character (cast `/Game/Blueprints/Enemy/BP_EnemyCharacter` OtherActor))
  (`/Engine/EditorBlueprintResources/StandardMacros.IsValid` (`self.Enemy`)
    (:`Is Valid`
      _)
    (:`Is Not Valid`
      (set `self.Enemy` _asbp_enemy_character)))
  (set `self.EnemyIsOverlapping` true))

(event `self.ReceiveActorEndOverlap`
  (params (OtherActor :type "Actor Object Reference"))
  (cast `/Game/Blueprints/Enemy/BP_EnemyCharacter` OtherActor)
  (set `self.EnemyIsOverlapping` false)
  (set `self.EnemyTimer` 0.0)
  (`AudioComponent.FadeOut` (`self.ShakingSoundAudioComponent`) 1.0 0.0))

(fn `AddWeight`)

(fn `GetInteractLocation`
  (returns (ReturnValue :type "Vector Structure"))
  (bind _returnvalue (`parent.GetInteractLocation`))
  (return _returnvalue))

(fn `Interact`
  (params (ActorInstigator :type "Actor Object Reference"))
  (returns (ReturnValue :type Boolean))
  (bind _opencloseaudiocomponent (`self.OpenCloseAudioComponent`))
  (bind _returnvalue (`parent.Interact` ActorInstigator))
  (bind _asfirst_person_character (cast `/Game/Blueprints/FirstPersonCharacter/FirstPersonCharacter` ActorInstigator)
    (:`then`
      (`/Engine/EditorBlueprintResources/StandardMacros.IsValid` (`self.Player`)
        (:`Is Valid`
          _)
        (:`Is Not Valid`
          (set `self.Player` _asfirst_person_character)))
      (`AudioComponent.SetPitchMultiplier` _opencloseaudiocomponent (`KismetMathLibrary.RandomFloatInRange` 0.6 1.4))
      (`AudioComponent.Play` _opencloseaudiocomponent 0.0)
      (`self.Play` _asfirst_person_character)
      (bind _output_get (set `/Game/Blueprints/FirstPersonCharacter/FirstPersonCharacter.IsHiding` (not (`/Game/Blueprints/FirstPersonCharacter/FirstPersonCharacter.IsHiding` _asfirst_person_character)) _asfirst_person_character))
      (if _output_get
        (if (< (`self.TimesHidden`) 3)
          (`/Game/Blueprints/FirstPersonCharacter/FirstPersonCharacter.AddSubtitle` _asfirst_person_character "Hold breath to stay quiet" 4.0 1.0 2.0)
          (bind _result (`/Engine/EditorBlueprintResources/StandardMacros.IncrementInt` (`self.TimesHidden`))
            (:`  `
              (set `self.TimesHidden` _result)))))
      (set `self.PlayerHidingInside` (not (`self.PlayerHidingInside`)))
      (return _returnvalue))
    (:`CastFailed`
      (cast `/Game/Blueprints/Enemy/BP_EnemyCharacter` ActorInstigator)
      (`self.EnemyPlayOpen`))))

(fn `UserConstructionScript`
  (`parent.UserConstructionScript`))