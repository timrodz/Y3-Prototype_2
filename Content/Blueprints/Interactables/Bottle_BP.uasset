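; Bottle_BP is a one-use interactable bottle that the player drinks from, causing a drunk effect.
; Interacting turns it to the instigator's line of sight by yaw, attaches it, then plays a sound and a timeline that lifts and tilts it.
; When finished, it detaches and drops with physics.
; After short delays, a second timeline drives chromatic aberration and grain jitter on the player camera, followed by a drunk camera shake.
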(event `self.ReceiveBeginPlay`
  (bind _asfirst_person_character (cast `/Game/Blueprints/FirstPersonCharacter/FirstPersonCharacter` (`GameplayStatics.GetPlayerPawn` 0)))
  (set `self.Player` _asfirst_person_character)
  (set `self.OriginalPos` (`self.K2_GetActorLocation`)))

(event `Drink`
  (bind _staticmesh (`self.StaticMesh`))
  (bind (_returnvalue_location _returnvalue_rotation) (`KismetMathLibrary.BreakTransform` (`SceneComponent.GetRelativeTransform` (`self.StaticMesh`))))
  (`GameplayStatics.PlaySound2D` "/Game/Audio/Sounds/Liquids/Drinking.Drinking")
  (bind (_direction _rotation _location) (`Timeline|DrinkFromBottle`)
    (:`Update`
      (`SceneComponent.K2_SetRelativeLocationAndRotation` (`self.DefaultSceneRoot`) (`KismetMathLibrary.MakeVector` (+ (.x (`self.OriginalPos`)) (* _location 0.2)) (.y (`self.OriginalPos`)) (+ (.z (`self.OriginalPos`)) (* _location 1.5))) (`KismetMathLibrary.MakeRotator` (.roll _returnvalue_rotation) _rotation (.yaw _returnvalue_rotation)) false false))
    (:`Finished`
      (`self.K2_DetachFromActor` "KeepWorld" "KeepWorld" "KeepWorld")
      (`PrimitiveComponent.SetSimulatePhysics` _staticmesh true)
      (`PrimitiveComponent.SetCollisionEnabled` _staticmesh "PhysicsOnly")
      (`KismetSystemLibrary.Delay` 0.5)
      (`self.Effects`)
      (`KismetSystemLibrary.Delay` 5.0)
      (`GameplayStatics.PlayWorldCameraShake` "/Game/Blueprints/Camera/Drunk_CameraShake_BP.Drunk_CameraShake_BP_C" (`self.K2_GetActorLocation` (`self.Player`)) 5.0 500.0))))

(event `Effects`
  (bind (_direction _effect) (`Timeline|Effect Timeline` :!via `PlayFromStart`)
    (:`Update`
      (set `CameraComponent.PostProcessSettings` (make `PostProcessSettings` :`SceneFringeIntensity` (* _effect 0.8) :`GrainJitter` _effect) (`/Game/Blueprints/FirstPersonCharacter/FirstPersonCharacter.Camera` (`self.Player`))))))

(fn `GetInteractLocation`
  (returns (ReturnValue :type "Vector Structure"))
  (`parent.GetInteractLocation`)
  (return (`SceneComponent.K2_GetComponentLocation` (`self.InteractLocation`))))

(fn `Interact`
  (params (ActorInstigator :type "Actor Object Reference"))
  (returns (ReturnValue :type Boolean))
  (bind _returnvalue_location (`KismetMathLibrary.BreakTransform` (`SceneComponent.GetRelativeTransform` (`self.DefaultSceneRoot`))))
  (bind (_returnvalue_roll _returnvalue_pitch _returnvalue_yaw) (`KismetMathLibrary.BreakRotator` (`KismetMathLibrary.FindLookAtRotation` (`self.K2_GetActorLocation` ActorInstigator) (`self.K2_GetActorLocation`))))
  (if (not (`self.bUsed`))
    (set `self.bUsed` true)
    (bind _returnvalue (`parent.Interact` null))
    (`self.K2_SetActorRotation` (`KismetMathLibrary.MakeRotator` 0.0 0.0 _returnvalue_yaw))
    (`self.K2_AttachToActor` ActorInstigator "None" "KeepWorld" "KeepWorld" "KeepWorld" false)
    (set `self.OriginalPos` _returnvalue_location)
    (`self.Drink`)
    (return _returnvalue)))

(fn `UserConstructionScript`
  (`parent.UserConstructionScript`))