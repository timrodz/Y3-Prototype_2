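; Bed hiding spot interactable that glides the first-person character to a marked spot on the bed when interacted with.
; Interact calls the parent, then disables player input and Cube collision before starting the camera animation.
; A timeline lerps the player's capsule to the Scene component's location and rotation, then restores collision on Cube and input.
; FlipFlops gate these steps with only their A paths doing work, so no exit move is implemented.
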(event `Play`
  (params (Player :type "/Game/Blueprints/FirstPersonCharacter Object Reference"))
  (`/Engine/EditorBlueprintResources/StandardMacros.FlipFlop`
    (:`A`
      (`self.DisableInput` Player (cast `PlayerController` (`Pawn.GetController` Player) :!pure true))
      (`/Engine/EditorBlueprintResources/StandardMacros.FlipFlop`
        (:`A`
          (`PrimitiveComponent.SetCollisionEnabled` (`self.Cube`) "NoCollision")
          (`self.Camera_Anim` Player))))))

(event `Camera_Anim`
  (params (Player :type "/Game/Blueprints/FirstPersonCharacter Object Reference"))
  (bind _capsulecomponent (`Character.CapsuleComponent` Player))
  (bind _capsulecomponent_2 (`Character.CapsuleComponent` Player))
  (bind _scene (`self.Scene`))
  (`/Engine/EditorBlueprintResources/StandardMacros.FlipFlop`
    (:`A`
      (`PrimitiveComponent.SetCollisionEnabled` _capsulecomponent "NoCollision"))
    (:`B`
      _))
  (`PrimitiveComponent.SetConstraintMode` _capsulecomponent "None")
  (bind (_direction _newtrack_1) (`Timeline|Camera_Lerp`)
    (:`Update`
      (`SceneComponent.K2_SetWorldLocationAndRotation` _capsulecomponent_2 (`KismetMathLibrary.VLerp` (`SceneComponent.K2_GetComponentLocation` _capsulecomponent_2) (`SceneComponent.K2_GetComponentLocation` _scene) _newtrack_1) (`KismetMathLibrary.RLerp` (`SceneComponent.K2_GetComponentRotation` _capsulecomponent_2) (`SceneComponent.K2_GetComponentRotation` _scene) _newtrack_1) false false))
    (:`Finished`
      (`/Engine/EditorBlueprintResources/StandardMacros.FlipFlop`
        (:`A`
          (`PrimitiveComponent.SetCollisionEnabled` (`self.Cube`) "QueryAndPhysics")
          (`self.EnableInput` Player null))))))

(fn `Interact`
  (params (ActorInstigator :type "Actor Object Reference"))
  (returns (ReturnValue :type Boolean))
  (bind _returnvalue (`parent.Interact` ActorInstigator))
  (bind _asfirst_person_character (cast `/Game/Blueprints/FirstPersonCharacter` ActorInstigator))
  (`self.Play` _asfirst_person_character)
  (return _returnvalue))

(fn `UserConstructionScript`
  (`parent.UserConstructionScript`))