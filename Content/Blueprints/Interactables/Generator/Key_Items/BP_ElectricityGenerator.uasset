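; Interactable electricity generator that serves as the win objective, repaired by attaching three missing pieces.
; Slot colliders set the active piece index, and Interact reveals that piece's zero-scaled mesh if it is marked collected.
; The third attachment toggles every BP_Lamp through PlayerInteraction, plays an engine sound, destroys all enemies and shows the win widget with UI-only input.
; Interact ignores the CanInteractWithComponent result, and AllMissingPiecesAttached never gates the win.
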(event `self.ReceiveBeginPlay`
  (set `self.Number of pieces attached` 0)
  (for _ (range 3)
    (`KismetArrayLibrary.Array_Add` (`self.MissingPiecesCollected`)))
  ;[1 1 1] Find all the lamps in the map and add them to an array
  (bind _outactors (`GameplayStatics.GetAllActorsOfClass` "/Game/Blueprints/Interactables/Lights/BP_Lamp.BP_Lamp_C"))
  (for _array_element _outactors
    (`KismetArrayLibrary.Array_Add` (`self.LampsInMap`) _array_element))
  ;[1 1 1] Set the scale of the missing pieces to 0
  (`SceneComponent.SetWorldScale3D` (`self.Slot_1 - Handle`) (0.0 0.0 0.0))
  (`SceneComponent.SetWorldScale3D` (`self.Slot_0 - Back Piece`) (0.0 0.0 0.0))
  (`SceneComponent.SetWorldScale3D` (`self.Slot_2 - Top Piece`) (0.0 0.0 0.0)))

(event `self.Box_0_Collider.OnComponentBeginOverlap`
  (params (OverlappedComponent :type "PrimitiveComponent Object Reference") (OtherActor :type "Actor Object Reference") (OtherComp :type "PrimitiveComponent Object Reference") (OtherBodyIndex :type Integer) (bFromSweep :type Boolean) (SweepResult :type "HitResult Structure (by ref)"))
  ;[1 0.3721 0.13] Check for attaching missing pieces
  (`self.SetActiveComponent` OverlappedComponent OtherActor))

(event `self.Box_0_Collider.OnComponentEndOverlap`
  (params (OverlappedComponent :type "PrimitiveComponent Object Reference") (OtherActor :type "Actor Object Reference") (OtherComp :type "PrimitiveComponent Object Reference") (OtherBodyIndex :type Integer))
  ;[1 0.3721 0.13] Check for attaching missing pieces
  (set `self.ActiveComponent` null))

(event `self.Box_1_Collider.OnComponentBeginOverlap`
  (params (OverlappedComponent :type "PrimitiveComponent Object Reference") (OtherActor :type "Actor Object Reference") (OtherComp :type "PrimitiveComponent Object Reference") (OtherBodyIndex :type Integer) (bFromSweep :type Boolean) (SweepResult :type "HitResult Structure (by ref)"))
  ;[1 0.3721 0.13] Check for attaching missing pieces
  (`self.SetActiveComponent` OverlappedComponent OtherActor 1))

(event `self.Box_1_Collider.OnComponentEndOverlap`
  (params (OverlappedComponent :type "PrimitiveComponent Object Reference") (OtherActor :type "Actor Object Reference") (OtherComp :type "PrimitiveComponent Object Reference") (OtherBodyIndex :type Integer))
  ;[1 0.3721 0.13] Check for attaching missing pieces
  (set `self.ActiveComponent` null))

(event `self.Box_2_Collider.OnComponentBeginOverlap`
  (params (OverlappedComponent :type "PrimitiveComponent Object Reference") (OtherActor :type "Actor Object Reference") (OtherComp :type "PrimitiveComponent Object Reference") (OtherBodyIndex :type Integer) (bFromSweep :type Boolean) (SweepResult :type "HitResult Structure (by ref)"))
  ;[1 0.3721 0.13] Check for attaching missing pieces
  (`self.SetActiveComponent` OverlappedComponent OtherActor 2))

(event `self.Box_2_Collider.OnComponentEndOverlap`
  (params (OverlappedComponent :type "PrimitiveComponent Object Reference") (OtherActor :type "Actor Object Reference") (OtherComp :type "PrimitiveComponent Object Reference") (OtherBodyIndex :type Integer))
  ;[1 0.3721 0.13] Check for attaching missing pieces
  (set `self.ActiveComponent` null))

(fn `AttachMissingPiece`
  (params (PieceNumber :type Integer))
  (locals (AllMissingPiecesAttached :type Boolean))
  (bind _returnvalue (`GameplayStatics.GetPlayerController` 0))
  (`/Engine/EditorBlueprintResources/StandardMacros.CompareInt` (`|GetArrayItem` (`self.MissingPiecesCollected`) PieceNumber) 1
    (:`==`
      (switch `int` PieceNumber
        (:`0`
          ;[0.7916 0.2622 1] Attach missing piece #0
          (`SceneComponent.SetWorldScale3D` (`self.Slot_0 - Back Piece`) (1.0 1.0 1.0)))
        (:`1`
          ;[0.7916 0.2622 1] Attach missing piece #1
          (`SceneComponent.SetWorldScale3D` (`self.Slot_1 - Handle`) (1.0 1.0 1.0)))
        (:`2`
          ;[0.7916 0.2622 1] Attach missing piece #2
          (`SceneComponent.SetWorldScale3D` (`self.Slot_2 - Top Piece`) (1.0 1.0 1.0))))
      (`KismetArrayLibrary.Array_Insert` (`self.MissingPiecesCollected`) 0 PieceNumber)
      (`KismetSystemLibrary.PrintString` "Attached generator piece!")
      (bind _result (`/Engine/EditorBlueprintResources/StandardMacros.IncrementInt` (`self.Number of pieces attached`))
        (:`  `
          (bind _output_get (set `self.Number of pieces attached` _result))
          (set `local.AllMissingPiecesAttached` true)
          (for _array_element (`self.MissingPiecesCollected`)
            (`/Engine/EditorBlueprintResources/StandardMacros.CompareInt` _array_element 1
              (:`>`
                _)
              (:`<`
                _))
            (set `local.AllMissingPiecesAttached` false))
          (`/Engine/EditorBlueprintResources/StandardMacros.CompareInt` (`self.Number of pieces attached`) 3
            (:`==`
              (`self.TurnLampsOn`)
              (`GameplayStatics.PlaySoundAtLocation` "/Game/Audio/Engine.Engine")
              (bind _outactors (`GameplayStatics.GetAllActorsOfClass` "/Game/Blueprints/Enemy/BP_EnemyCharacter.BP_EnemyCharacter_C"))
              (for _array_element_2 _outactors
                (`self.K2_DestroyActor` _array_element_2))
              (`WidgetLayoutLibrary.RemoveAllWidgets`)
              (bind _returnvalue_2 (`|CreateWidget` "/Game/Blueprints/Widgets/WinGame_WidgetBP.WinGame_WidgetBP_C"))
              (`UserWidget.AddToViewport` _returnvalue_2 0)
              (`self.DisableInput` _returnvalue)
              (set `PlayerController.bShowMouseCursor` true _returnvalue)
              (`WidgetBlueprintLibrary.SetInputMode_UIOnlyEx` _returnvalue _returnvalue_2 "LockOnCapture"))))))))

(fn `CanInteractWithComponent`
  (returns (`Can Interact` :type Boolean))
  (if (`KismetSystemLibrary.IsValid` (`self.ActiveComponent`))
    (return true)
    (else
      (return false))))

(fn `Interact`
  (params (ActorInstigator :type "Actor Object Reference"))
  (returns (ReturnValue :type Boolean))
  (bind _returnvalue (`parent.Interact` null))
  (`self.CanInteractWithComponent`)
  (`self.AttachMissingPiece` (`self.ActiveMissingPiece`))
  (return _returnvalue))

(fn `SetActiveComponent`
  (params (`Main Collider` :type "PrimitiveComponent Object Reference") (`Other Collider` :type "Actor Object Reference") (`Missing Piece Number` :type Integer))
  (set `self.ActiveMissingPiece` `Missing Piece Number`)
  (cast `/Game/Blueprints/FirstPersonCharacter/FirstPersonCharacter` `Other Collider`)
  (set `self.ActiveComponent` `Main Collider`))

(fn `TurnLampsOff`
  (for _array_element (`self.LampsInMap`)
    (bind _asbp_lamp (cast `/Game/Blueprints/Interactables/Lights/BP_Lamp` _array_element))
    (`/Game/Blueprints/Interactables/Lights/BP_Lamp.PlayerInteraction` _asbp_lamp)))

(fn `TurnLampsOn`
  (for _array_element (`self.LampsInMap`)
    (bind _asbp_lamp (cast `/Game/Blueprints/Interactables/Lights/BP_Lamp` _array_element))
    (`/Game/Blueprints/Interactables/Lights/BP_Lamp.PlayerInteraction` _asbp_lamp)))

(fn `UserConstructionScript`)