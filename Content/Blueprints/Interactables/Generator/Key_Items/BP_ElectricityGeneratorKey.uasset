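; Collectible key piece for the electricity generator, picked up through the Interact function.
; Interact calls the parent, then sets this piece's numbered slot in the referenced generator's MissingPiecesCollected array.
; It prints a found message, hides and destroys itself, then makes the first-person player emit noise and optionally plays a piano sound.
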(fn `Interact`
  (params (ActorInstigator :type "Actor Object Reference"))
  (returns (ReturnValue :type Boolean))
  (`parent.Interact` null)
  (`KismetArrayLibrary.Array_Set` (`/Game/Blueprints/Interactables/Generator/Key_Items/BP_ElectricityGenerator.MissingPiecesCollected` (`self.Generator`)) (`self.Missing Piece Number`) 1)
  (`KismetSystemLibrary.PrintString` "Found missing generator piece!")
  (`self.SetActorHiddenInGame` true)
  (bind _output_get (set `self.IsPickedUp` true))
  (`self.K2_DestroyActor`)
  (bind _asfirst_person_character (cast `/Game/Blueprints/FirstPersonCharacter/FirstPersonCharacter` (`GameplayStatics.GetPlayerPawn` 0)))
  (`/Game/Blueprints/FirstPersonCharacter/FirstPersonCharacter.PlayerMakeNoise` _asfirst_person_character)
  (if (`self.PlaySound`)
    (`GameplayStatics.PlaySound2D` "/Game/Audio/Piano_FX.Piano_FX"))
  (return _output_get))

(fn `UserConstructionScript`)