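; Interactable actor that shows fullscreen text when a FirstPersonCharacter interacts with it.
; Interact calls the parent implementation, then formats each Text entry in place, replacing {nextline} tokens intended as line breaks.
; It passes the array to the character's ShowFullscreenText and destroys itself if DestroyAfterInspecting is set.
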(fn `Interact`
  (params (ActorInstigator :type "Actor Object Reference"))
  (returns (ReturnValue :type Boolean))
  (bind _text (`self.Text`))
  (bind _returnvalue (`parent.Interact` ActorInstigator))
  (bind _asfirst_person_character (cast `/Game/Blueprints/FirstPersonCharacter/FirstPersonCharacter` ActorInstigator))
  ;[0.7067 0.2338 1] Adds a new line every time you write {nextline}
  (for (_array_element _array_index) _text
    (`KismetArrayLibrary.Array_Set` _text _array_index (`|FormatText` (`KismetSystemLibrary.MakeLiteralText` _array_element) " \n")))
  (`/Game/Blueprints/FirstPersonCharacter/FirstPersonCharacter.ShowFullscreenText` _asfirst_person_character (`self.Text`))
  (if (`self.DestroyAfterInspecting?`)
    (`self.K2_DestroyActor`))
  (return _returnvalue))

(fn `UserConstructionScript`)