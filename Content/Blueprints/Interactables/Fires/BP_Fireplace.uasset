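; BP_Fireplace is an interactable fireplace with a fuel stack that sets the light scale of its particle effect.
; On BeginPlay, a non-empty Stack passes a DoOnce, waits StackBurnTime, loses one unit and updates the LightScale particle parameter to match.
; The DoOnce then resets, but nothing re-triggers it, so only one unit burns.
; Interact is an empty stub, with its return node unconnected.
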(event `self.ReceiveBeginPlay`
  (if (> (`self.Stack`) 0)
    (`/Engine/EditorBlueprintResources/StandardMacros.DoOnce` false :!label _label
      (:`Completed`
        (`KismetSystemLibrary.Delay` (`self.StackBurnTime`))
        (`/Engine/EditorBlueprintResources/StandardMacros.DecrementInt` (`self.Stack`)
          (:`  `
            (`ParticleSystemComponent.SetVectorParameter` (`self.ParticleSystem`) "LightScale" (* (1.0 1.0 1.0) (`self.Stack`)))
            (goto _label :!via `Reset`)))))))

(fn `Interact`
  (params (ActorInstigator :type "Actor Object Reference"))
  (returns (ReturnValue :type Boolean)))

(fn `UserConstructionScript`)