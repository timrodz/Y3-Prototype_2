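; BP_Key is an interactable key pickup that tracks whether the player has taken it.
; Interact calls the parent, then branches on whether the instigator is the first-person player or an enemy character.
; Player interaction marks the key taken and active, hides the actor, plays a pickup sound and tells its Zone to update items.
; Enemy interaction changes nothing and only returns whether the key has been taken.
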(event `self.ReceiveBeginPlay`
  (set `self.HasBeenTaken` false))

(fn `EnemyInteraction`
  (params (Enemy :type "/Game/Blueprints/Enemy/BP_EnemyCharacter Object Reference"))
  (returns (HasBeenTaken :type Boolean))
  (return (`self.HasBeenTaken`)))

(fn `Interact`
  (params (ActorInstigator :type "Actor Object Reference"))
  (returns (ReturnValue :type Boolean))
  (`parent.Interact` ActorInstigator)
  (bind _asfirst_person_character (cast `/Game/Blueprints/FirstPersonCharacter/FirstPersonCharacter` ActorInstigator)
    (:`then`
      (`self.PlayerInteraction` _asfirst_person_character)
      (return true))
    (:`CastFailed`
      (bind _asbp_enemy_character (cast `/Game/Blueprints/Enemy/BP_EnemyCharacter` ActorInstigator))
      (bind _hasbeentaken (`self.EnemyInteraction` _asbp_enemy_character))
      (return _hasbeentaken))))

(fn `PlayerInteraction`
  (params (Player :type "/Game/Blueprints/FirstPersonCharacter/FirstPersonCharacter Object Reference"))
  (set `self.HasBeenTaken` true)
  (`self.SetActorHiddenInGame` true)
  (`GameplayStatics.PlaySound2D` "/Game/Audio/key_pick_up.key_pick_up")
  (set `self.ActiveState` true)
  (`Zone.UpdateZoneItems` (`self.Zone`)))

(fn `UserConstructionScript`
  (set `self.HasBeenTaken` false))