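; BP_Drawer is an interactable drawer that slides open and closed when a player interacts with it.
; Interact calls the parent, then fires Slide, whose FlipFlop alternately plays and reverses a timeline.
; Each update moves the whole actor along its root's right vector, scaled by Distance, from the location cached in the construction script.
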(event `Slide`
  (`/Engine/EditorBlueprintResources/StandardMacros.FlipFlop`
    (:`A`
      (bind (_direction _newtrack_0) (`Timeline|Slider` :!label _label)
        (:`Update`
          (`self.K2_SetActorLocation` (+ (* (`SceneComponent.GetRightVector` (`self.DefaultSceneRoot`)) (* _newtrack_0 (`self.Distance`))) (`self.OriginalLocation`))))))
    (:`B`
      (goto _label :!via `Reverse`))))

(fn `Interact`
  (params (ActorInstigator :type "Actor Object Reference"))
  (returns (ReturnValue :type Boolean))
  (bind _returnvalue (`parent.Interact` null))
  (`self.Slide`)
  (return _returnvalue))

(fn `UserConstructionScript`
  (`parent.UserConstructionScript`)
  (set `self.OriginalLocation` (`self.K2_GetActorLocation`)))