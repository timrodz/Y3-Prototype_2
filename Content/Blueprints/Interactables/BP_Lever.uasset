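; Interactable puzzle lever that flips between two rotations and reports to the level's Puzzle_Lever_Controller_BP, found at BeginPlay.
; Interact calls Toggle, then asks the controller to check the solution.
; Gate levers trigger the controller's gate check; others toggle linked lights' particles and point lights, whooshing if any becomes visible.
; A Tick-accumulated timer suppresses the switch sound during the first second, when Toggle calls Interacted instead.
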(event `self.ReceiveBeginPlay`
  (bind _outactors (`GameplayStatics.GetAllActorsOfClass` "/Game/Blueprints/Puzzles/Puzzle_Lever_Controller_BP.Puzzle_Lever_Controller_BP_C"))
  (for _array_element _outactors
    (set `self.LeverController` _array_element)
    (if (`self.GateLever`)
      (set `self.IsPointingUp` true))))

(event `self.ReceiveTick`
  (params (DeltaSeconds :type "Float (single-precision)"))
  (set `self.Timer` (+ DeltaSeconds (`self.Timer`))))

(fn `Interact`
  (params (ActorInstigator :type "Actor Object Reference"))
  (returns (ReturnValue :type Boolean))
  (`parent.Interact` null)
  (bind _leverpointingup (`self.Toggle` (`self.IsPointingUp`)))
  (`/Game/Blueprints/Puzzles/Puzzle_Lever_Controller_BP.NewCheckSolution` (`self.LeverController`))
  (return _leverpointingup))

(fn `PointDown`
  (set `self.IsPointingUp` false)
  (`SceneComponent.K2_SetRelativeRotation` (`self.Lever`) (struct :`Pitch` 90.0) false false))

(fn `Toggle`
  (params (IsLeverPointingUp :type Boolean))
  (returns (LeverPointingUp :type Boolean))
  (bind _ispointingup (`self.IsPointingUp`))
  (bind _lever (`self.Lever`))
  (if IsLeverPointingUp
    (set `self.IsPointingUp` false)
    (`SceneComponent.K2_SetRelativeRotation` _lever (struct :`Pitch` 30.0) false false) ; UP
    (else
      (set `self.IsPointingUp` true)
      (`SceneComponent.K2_SetRelativeRotation` _lever (struct :`Pitch` 90.0) false false) ; DOWN
    ))
  (set `self.AnyVisible` false)
  (if (`self.GateLever`)
    (`/Game/Blueprints/Puzzles/Puzzle_Lever_Controller_BP.Gate Lever Check` (`self.LeverController`))
    (else
      (for _array_element (`self.Lights`)
        (`/Engine/EditorBlueprintResources/StandardMacros.IsValid` _array_element
          (:`Is Valid`
            (bind _particlesystem (`/Game/Blueprints/LeverFlame_BP.ParticleSystem` _array_element))
            (`SceneComponent.ToggleVisibility` _particlesystem false)
            (`SceneComponent.ToggleVisibility` (`/Game/Blueprints/LeverFlame_BP.PointLight` _array_element) false)
            (if (`SceneComponent.bVisible` _particlesystem)
              (set `self.AnyVisible` true)))))
      (if (`self.AnyVisible`)
        (`GameplayStatics.PlaySoundAtLocation` "/Game/Audio/Sounds/Fire/Flame_Poof_Whoosh.Flame_Poof_Whoosh" (`self.K2_GetActorLocation`)))))
  (if (> (`self.Timer`) 1.0)
    (`GameplayStatics.PlaySound2D` "/Game/Audio/Sounds/Buttons/Breaker_Switch_1.Breaker_Switch_1" 0.6)
    (else
      (`self.Interacted` null _ispointingup)))
  (return _ispointingup))

(fn `ToggleElementRotation`
  (`/Engine/EditorBlueprintResources/StandardMacros.FlipFlop`))

(fn `UserConstructionScript`)