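; BP_ProjectDecalTrigger is a trigger actor that briefly shows a decal when the FirstPersonCharacter overlaps it.
; On BeginPlay it caches the placed decal's base material, size and world transform, then quickly fades that decal out.
; Each qualifying overlap spawns a new decal with those cached values, attached to the root, which fades out after a short delay without destroying the actor.
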(event `self.ReceiveBeginPlay`
  (bind _decal (`self.Decal`))
  (bind (_returnvalue_location _returnvalue_rotation) (`KismetMathLibrary.BreakTransform` (`SceneComponent.K2_GetComponentToWorld` _decal)))
  (bind _returnvalue (`MaterialInterface.GetBaseMaterial` (`DecalComponent.GetDecalMaterial` (`self.Decal`))))
  (set `self.DecalRef` _returnvalue)
  (set `self.Size` (`DecalComponent.DecalSize` _decal))
  (set `self.Loc` _returnvalue_location)
  (set `self.Rot` _returnvalue_rotation)
  (`DecalComponent.SetFadeOut` (`self.Decal`) 0.1 0.1 false))

(event `self.ReceiveActorBeginOverlap`
  (params (OtherActor :type "Actor Object Reference"))
  (cast `/Game/Blueprints/FirstPersonCharacter/FirstPersonCharacter` OtherActor)
  (bind _returnvalue (`GameplayStatics.SpawnDecalAttached` (`self.DecalRef`) (`self.Size`) (`self.DefaultSceneRoot`) "None" (`self.Loc`) (`self.Rot`) "KeepWorldPosition" 0.0))
  (`DecalComponent.SetFadeOut` _returnvalue 1.0 2.0 false))

(fn `UserConstructionScript`)