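; BP_Table is a table actor that lays out a grid of point components, with no runtime logic in its event graph.
; The construction script clears the Components array, then builds an X by Y grid of scene components around the origin, offset by Spacing.
; Each point is stored in Components and paired with a small collision-free sphere component at the same transform.
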(event `self.ReceiveBeginPlay`)

(fn `UserConstructionScript`
  (bind (_spacing_x _spacing_y) (`KismetMathLibrary.BreakVector` (`self.Spacing`)))
  (`KismetArrayLibrary.Array_Clear` (`self.Components`))
  (for _index (range 1 (+ (`self.X`) 1))
    (for _index_2 (range 1 (+ (`self.Y`) 1))
      (bind _returnvalue (`AddComponent|NODE_AddSceneComponent-0` :`RelativeTransform` (`KismetMathLibrary.MakeTransform` (`KismetMathLibrary.MakeVector` (* (- _index (/ (`self.X`) 2)) _spacing_x) (* (- _index_2 (/ (`self.Y`) 2)) _spacing_y)))))
      (`KismetArrayLibrary.Array_Add` (`self.Components`) _returnvalue)
      (bind _returnvalue_2 (`AddComponent|NODE_AddSphereComponent-1` :`RelativeTransform` (`SceneComponent.GetRelativeTransform` _returnvalue)))
      (`PrimitiveComponent.SetCollisionEnabled` _returnvalue_2 "NoCollision")
      (`SceneComponent.SetRelativeScale3D` _returnvalue_2 (0.25 0.25 0.25)))))