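; BP_ClearTheArea is an area marker that removes itself once its box volume holds no static mesh actors.
; Both begin and end overlap on the box count the overlapping StaticMeshActors and swap the plane's material between occupied and clear.
; When the count reaches zero, the actor destroys itself after a short delay, without rechecking.
; The construction script scales the plane to match the box extent.
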(event `self.ReceiveBeginPlay`)

(event `self.Box.OnComponentEndOverlap`
  (params (OverlappedComponent :type "PrimitiveComponent Object Reference") (OtherActor :type "Actor Object Reference") (OtherComp :type "PrimitiveComponent Object Reference") (OtherBodyIndex :type Integer))
  (bind _plane (`self.Plane`))
  (if (== (`KismetArrayLibrary.Array_Length` (`PrimitiveComponent.GetOverlappingActors` (`self.Box`) "/Script/Engine.StaticMeshActor")) 0) :!label _label
    (`PrimitiveComponent.SetMaterial` _plane 0 "/Game/Assets/Furniture/Kitchen/Materials/blinn1.blinn1")
    (`KismetSystemLibrary.Delay` 2.5)
    (`self.K2_DestroyActor`)
    (else
      (`PrimitiveComponent.SetMaterial` _plane 0 "/Game/Assets/SmallAssets/BookTextures/book_green_Mat.book_green_Mat"))))

(event `self.Box.OnComponentBeginOverlap`
  (params (OverlappedComponent :type "PrimitiveComponent Object Reference") (OtherActor :type "Actor Object Reference") (OtherComp :type "PrimitiveComponent Object Reference") (OtherBodyIndex :type Integer) (bFromSweep :type Boolean) (SweepResult :type "HitResult Structure (by ref)"))
  (goto _label))

(fn `UserConstructionScript`
  (`SceneComponent.SetWorldScale3D` (`self.Plane`) (/ (`BoxComponent.GetScaledBoxExtent` (`self.Box`)) 50.0)))