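; Interactable double-door fridge that opens or closes each time it is interacted with, overriding its parent's Interact and interact-location functions.
; Interact calls AnimateFridge, then flips IsOpen; one timeline swings both doors in mirrored yaw.
; Interacting mid-animation reverses the swing from its current position without restarting the sound.
; A single audio component, spawned at BeginPlay, swaps open and close sounds, delaying the close sound.
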(event `self.ReceiveBeginPlay`
  (set `self.IsOpen` false)
  (set `self.IsAnimating` false)
  (bind _returnvalue (`GameplayStatics.SpawnSoundAtLocation` "/Game/Audio/Sounds/Fridge/FridgeOpen.FridgeOpen" (`self.K2_GetActorLocation`) (struct) 1.0 1.0 0.0 null null false))
  (bind _output_get (set `self.AudioComponent` _returnvalue))
  (`AudioComponent.Stop` _output_get))

(event `Animate Fridge`
  (bind _audiocomponent (`self.AudioComponent`))
  (if (`self.IsOpen`)
    (if (`self.IsAnimating`)
      (bind (_direction _newtrack_0) (`Timeline|Open_Timeline` :!via `Reverse` :!label _label)
        (:`Update`
          (set `self.IsAnimating` true)
          (`SceneComponent.K2_SetRelativeRotation` (`self.RightDoor`) (`KismetMathLibrary.MakeRotator` 0.0 0.0 _newtrack_0) false false)
          (`SceneComponent.K2_SetRelativeRotation` (`self.LeftDoor`) (`KismetMathLibrary.MakeRotator` 0.0 0.0 (* _newtrack_0 -1.0)) false false))
        (:`Finished`
          (set `self.IsAnimating` false)))
      (else
        (`AudioComponent.SetSound` _audiocomponent "/Game/Audio/Sounds/Fridge/FridgeClose2.FridgeClose2")
        (`self.FridgeCloseSound`)
        (goto _label :!via `ReverseFromEnd`)))
    (elif (`self.IsAnimating`)
      (goto _label)
      (else
        (`AudioComponent.SetSound` _audiocomponent "/Game/Audio/Sounds/Fridge/FridgeOpen.FridgeOpen")
        (`AudioComponent.Play` _audiocomponent 0.0)
        (goto _label :!via `PlayFromStart`)))))

(event `FridgeCloseSound`
  (`KismetSystemLibrary.Delay` 0.6)
  (`AudioComponent.Play` (`self.AudioComponent`) 0.0))

(fn `GetInteractLocation`
  (returns (ReturnValue :type "Vector Structure"))
  (`parent.GetInteractLocation`)
  (return (`SceneComponent.K2_GetComponentLocation` (`self.InteractLocation`))))

(fn `Interact`
  (params (ActorInstigator :type "Actor Object Reference"))
  (returns (ReturnValue :type Boolean))
  (bind _returnvalue (`parent.Interact` null))
  (`self.Animate Fridge`)
  (set `self.IsOpen` (not (`self.IsOpen`)))
  (return _returnvalue))

(fn `UserConstructionScript`
  (`parent.UserConstructionScript`))