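; Interactable wardrobe hiding spot that moves a first-person character in or out and toggles its IsHiding flag.
; Interact triggers a timeline that swings both doors open, then drops collision, starts the move and closes them, restoring collision and input afterwards.
; A second timeline lerps the player's capsule to the hiding or return point, with FlipFlops alternating direction and door phases.
; Input is disabled only on the entering pass.
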(event `Play`
  (params (Player :type "/Game/Blueprints/FirstPersonCharacter/FirstPersonCharacter Object Reference"))
  (bind _asplayer_controller (cast `PlayerController` (`Pawn.GetController` Player) :!pure true))
  (`/Engine/EditorBlueprintResources/StandardMacros.FlipFlop`
    (:`A`
      (`self.DisableInput` Player _asplayer_controller)
      (bind (_direction _rotationto90) (`Timeline|SwingDoors` :!via `PlayFromStart` :!label _label)
        (:`Update`
          (`|ExecutionSequence`
            (:`then_0`
              (`SceneComponent.K2_SetRelativeRotation` (`self.StaticMesh1`) (`KismetMathLibrary.MakeRotator` 0.0 0.0 _rotationto90) false false))
            (:`then_1`
              (`SceneComponent.K2_SetRelativeRotation` (`self.StaticMesh`) (`KismetMathLibrary.MakeRotator` 0.0 0.0 (* _rotationto90 -1.0)) false false))))
        (:`Finished`
          (`/Engine/EditorBlueprintResources/StandardMacros.FlipFlop`
            (:`A`
              (`PrimitiveComponent.SetCollisionEnabled` (`self.Cube`) "NoCollision")
              (`PrimitiveComponent.SetCollisionEnabled` (`self.StaticMesh`) "NoCollision")
              (`PrimitiveComponent.SetCollisionEnabled` (`self.StaticMesh1`) "NoCollision")
              (`self.Camera_Anim` Player)
              (goto _label :!via `ReverseFromEnd`))
            (:`B`
              (`PrimitiveComponent.SetCollisionEnabled` (`self.Cube`) "QueryAndPhysics")
              (`PrimitiveComponent.SetCollisionEnabled` (`self.StaticMesh`) "QueryAndPhysics")
              (`PrimitiveComponent.SetCollisionEnabled` (`self.StaticMesh1`) "QueryAndPhysics")
              (`self.EnableInput` Player _asplayer_controller))))))
    (:`B`
      (goto _label :!via `PlayFromStart`))))

(event `Camera_Anim`
  (params (Player :type "/Game/Blueprints/FirstPersonCharacter/FirstPersonCharacter Object Reference"))
  (bind _capsulecomponent (`Character.CapsuleComponent` Player))
  (bind _isa (`/Engine/EditorBlueprintResources/StandardMacros.FlipFlop`)
    (:`A`
      (bind (_direction _newtrack_1) (`Timeline|Camera_Lerp` :!via `PlayFromStart` :!label _label_2)
        (:`Update`
          (if _isa
            (`SceneComponent.K2_SetWorldLocationAndRotation` _capsulecomponent (`KismetMathLibrary.VLerp` (`SceneComponent.K2_GetComponentLocation` _capsulecomponent) (`SceneComponent.K2_GetComponentLocation` (`self.Scene`)) _newtrack_1) (`KismetMathLibrary.RLerp` (`SceneComponent.K2_GetComponentRotation` _capsulecomponent) (`SceneComponent.K2_GetComponentRotation` (`self.Cube`)) _newtrack_1) false false)
            (else
              (`SceneComponent.K2_SetWorldLocationAndRotation` _capsulecomponent (`KismetMathLibrary.VLerp` (`SceneComponent.K2_GetComponentLocation` _capsulecomponent) (`SceneComponent.K2_GetComponentLocation` (`self.Return`)) _newtrack_1) (`KismetMathLibrary.RLerp` (`SceneComponent.K2_GetComponentRotation` _capsulecomponent) (`SceneComponent.K2_GetComponentRotation` (`self.Cube`)) _newtrack_1) false false))))))
    (:`B`
      (goto _label_2 :!via `PlayFromStart`))))

(fn `AddWeight`)

(fn `Interact`
  (params (ActorInstigator :type "Actor Object Reference"))
  (returns (ReturnValue :type Boolean))
  (bind _returnvalue (`parent.Interact` ActorInstigator))
  (bind _asfirst_person_character (cast `/Game/Blueprints/FirstPersonCharacter/FirstPersonCharacter` ActorInstigator))
  (`self.Play` _asfirst_person_character)
  (set `/Game/Blueprints/FirstPersonCharacter/FirstPersonCharacter.IsHiding` (not (`/Game/Blueprints/FirstPersonCharacter/FirstPersonCharacter.IsHiding` _asfirst_person_character)) _asfirst_person_character)
  (return _returnvalue))

(fn `UserConstructionScript`
  (`parent.UserConstructionScript`))