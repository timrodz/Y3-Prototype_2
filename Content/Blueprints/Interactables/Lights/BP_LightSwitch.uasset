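; BP_LightSwitch is an interactable wall-style light switch that controls an array of linked lights.
; Interact flips LightIsOff, then calls ToggleLights on each light, clearing its blinking when off or applying ShouldLightsBlink when on.
; It also tilts the Switch component and plays a matching plastic click sound for each state.
; The construction script's initial-intensity loop has no array connected, so Lights is unused there.
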(event `self.ReceiveTick`
  (params (DeltaSeconds :type "Float (single-precision)")))

(fn `Interact`
  (params (ActorInstigator :type "Actor Object Reference"))
  (returns (ReturnValue :type Boolean))
  (bind _switch (`self.Switch`))
  (bind _returnvalue (`SceneComponent.K2_GetComponentLocation` (`self.Lightstwitch`)))
  (bind _returnvalue_2 (`parent.Interact` null))
  (bind _output_get (set `self.LightIsOff` (not (`self.LightIsOff`))))
  (for _array_element (`self.Lights`)
    (if (`self.LightIsOff`)
      (set `/Game/Blueprints/Props/Ceiling_Light_BP.IsBlinking?` false _array_element)
      (else
        (set `/Game/Blueprints/Props/Ceiling_Light_BP.IsBlinking?` (`self.ShouldLightsBlink?`) _array_element)))
    (`/Game/Blueprints/Props/Ceiling_Light_BP.ToggleLights` _array_element))
  (if (`self.LightIsOff`)
    (`GameplayStatics.PlaySoundAtLocation` "/Game/Audio/Sounds/Buttons/Others/Switch_Small_Plastic_1.Switch_Small_Plastic_1" _returnvalue)
    (`SceneComponent.K2_SetRelativeRotation` _switch (struct :`Roll` -12.0) false false)
    (else
      (`GameplayStatics.PlaySoundAtLocation` "/Game/Audio/Sounds/Buttons/Others/Switch_Small_Plastic_2.Switch_Small_Plastic_2" _returnvalue)
      (`SceneComponent.K2_SetRelativeRotation` _switch (struct :`Roll` 12.0) false false))))

(fn `UserConstructionScript`
  (for _array_element _
    (`LightComponent.SetIntensity` (`Light.LightComponent` _array_element) (* (- 1.0 (`KismetMathLibrary.Conv_BoolToDouble` (`self.LightIsOff`))) (`self.InitialBrightness`)))))