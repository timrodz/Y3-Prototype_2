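; Inspectable interactable actor that the first-person character can pull up in front of the camera and rotate with mouse input.
; BeginInspect disables player movement, binds mouse input and plays a timeline lerping the object from its original transform to the player's InspectLocation, adjusting scale and depth-of-field blur.
; EndInspect unbinds input, restores walking and reverses the timeline.
; BeginPlay briefly plays and stops the timeline so it initializes for use inside functions.
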(event `self.ReceiveBeginPlay`
  (bind _insp_timeline (`self.Insp_Timeline`))
  ;[1 1 1] DO NOT DELETE. Useless in essence, but is required to initialize timeline. If no refferences to timeline exist in the main event graph, it'll discard it, and won't be callable from the End and Begin functions
  (`TimelineComponent.Play` _insp_timeline)
  (`TimelineComponent.Stop` _insp_timeline)
  (set `self.OriginalScale` (`SceneComponent.K2_GetComponentScale` (`self.StaticMesh`))))

(event `self.ReceiveDestroyed`
  (bind _playerbindref (`self.PlayerBindRef`))
  (`/Engine/EditorBlueprintResources/StandardMacros.IsValid` _playerbindref
    (:`Is Valid`
      (remove `/Game/Blueprints/FirstPersonCharacter/FirstPersonCharacter.MouseInput` _playerbindref (`|CreateDelegate` :!event `PlayerMouseInputHandler`)))))

(event `self.OnBeginInspect`
  (params (Actor :type "Actor Object Reference"))
  (`self.BeginInspect` Actor))

(event `self.OnEndInspect`
  (`self.EndInspect`))

(event `PlayerMouseInputHandler`
  (params (TurnRate :type "Float (double-precision)") (LookUpRate :type "Float (double-precision)"))
  (bind (_returnvalue_roll _returnvalue_pitch _returnvalue_yaw) (`KismetMathLibrary.BreakRotator` (`SceneComponent.K2_GetComponentRotation` (`/Game/Blueprints/FirstPersonCharacter/FirstPersonCharacter.Camera` (`self.PlayerBindRef`)))))
  (`self.K2_SetActorRotation` (`KismetMathLibrary.ComposeRotators` (`KismetMathLibrary.RotatorFromAxisAndAngle` (`KismetMathLibrary.GetUpVector` (`KismetMathLibrary.MakeRotator` _returnvalue_roll)) TurnRate) (`KismetMathLibrary.ComposeRotators` (`SceneComponent.K2_GetComponentRotation` (`self.StaticMesh`)) (`KismetMathLibrary.RotatorFromAxisAndAngle` (`KismetMathLibrary.GetRightVector` (`KismetMathLibrary.MakeRotator` 0.0 _returnvalue_pitch _returnvalue_yaw)) LookUpRate)))))

(fn `BeginInspect`
  (params (Object :type "Object Object Reference"))
  (bind _asfirst_person_character (cast `/Game/Blueprints/FirstPersonCharacter/FirstPersonCharacter` Object))
  (bind _output_get (set `self.PlayerBindRef` _asfirst_person_character))
  (add `/Game/Blueprints/FirstPersonCharacter/FirstPersonCharacter.MouseInput` _output_get (`|CreateDelegate` :!event `PlayerMouseInputHandler`))
  (`CharacterMovementComponent.DisableMovement` (`Character.CharacterMovement` (`self.PlayerBindRef`)))
  (`TimelineComponent.PlayFromStart` (`self.Insp_Timeline`))
  (`self.Event_OnBeginInspect`)
  (return))

(fn `DisablePlayer`)

(fn `EnablePlayer`)

(fn `EndInspect`
  (bind _playerbindref (`self.PlayerBindRef`))
  (`/Engine/EditorBlueprintResources/StandardMacros.IsValid` _playerbindref
    (:`Is Valid`
      (remove `/Game/Blueprints/FirstPersonCharacter/FirstPersonCharacter.MouseInput` _playerbindref (`|CreateDelegate` :!event `PlayerMouseInputHandler`))
      (`CharacterMovementComponent.SetMovementMode` (`Character.CharacterMovement` (`self.PlayerBindRef`)) "MOVE_Walking" 0)
      (`TimelineComponent.ReverseFromEnd` (`self.Insp_Timeline`))
      (`self.Event_OnEndInspect`))))

(fn `UserConstructionScript`
  (bind _staticmesh (`self.StaticMesh`))
  (`parent.UserConstructionScript`)
  (set `self.OriginalLocation` (`SceneComponent.K2_GetComponentLocation` _staticmesh))
  (set `self.OriginalRotation` (`SceneComponent.K2_GetComponentRotation` _staticmesh)))