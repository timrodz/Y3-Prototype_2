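; Hanging ceiling toy interactable with a moon and three stars that bob vertically and play a baby rattle sound when interacted with.
; BeginPlay gathers child meshes, caches start locations and starts four timelines that apply scaled Z offsets to each piece.
; Interact calls the parent, sets Interacted, plays the attenuated sound and restarts all timelines.
; The last star's timeline clears Interacted when finished.
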(event `self.ReceiveBeginPlay`
  (for _array_element (`SceneComponent.GetChildrenComponents` (`self.Toys`) false)
    (bind _asstatic_mesh_component (cast `StaticMeshComponent` _array_element))
    (`KismetArrayLibrary.Array_Add` (`self.ToyArray`) _asstatic_mesh_component)
    (set `self.MoonStartLocation` (`SceneComponent.K2_GetComponentLocation` (`self.Moon`)))
    (set `self.Star1StartLocation` (`SceneComponent.K2_GetComponentLocation` (`self.Star1`)))
    (set `self.Star2StartLocation` (`SceneComponent.K2_GetComponentLocation` (`self.Star2`)))
    (set `self.Star3StartLocation` (`SceneComponent.K2_GetComponentLocation` (`self.Star3`)))
    (`|ExecutionSequence`
      (:`then_0`
        (bind (_direction _floattrack) (`Timeline|Timeline_0` :!via `PlayFromStart`)
          (:`Update`
            (`SceneComponent.K2_SetWorldLocation` (`self.Moon`) (+ (`KismetMathLibrary.MakeVector` 0.0 0.0 (* _floattrack 2.0)) (`self.MoonStartLocation`)) false false))))
      (:`then_1`
        (bind (_direction_2 _floattrack_2) (`Timeline|Timeline_1` :!via `PlayFromStart`)
          (:`Update`
            (`SceneComponent.K2_SetWorldLocation` (`self.Star1`) (+ (`KismetMathLibrary.MakeVector` 0.0 0.0 (* _floattrack_2 2.0)) (`self.Star1StartLocation`)) false false))))
      (:`then_2`
        (bind (_direction_3 _floattrack_3) (`Timeline|Timeline_2` :!via `PlayFromStart`)
          (:`Update`
            (`SceneComponent.K2_SetWorldLocation` (`self.Star2`) (+ (`KismetMathLibrary.MakeVector` 0.0 0.0 (* _floattrack_3 2.0)) (`self.Star2StartLocation`)) false false))))
      (:`then_3`
        (bind (_direction_4 _floattrack_4) (`Timeline|Timeline_3` :!via `PlayFromStart`)
          (:`Update`
            (`SceneComponent.K2_SetWorldLocation` (`self.Star3`) (+ (`KismetMathLibrary.MakeVector` 0.0 0.0 (* _floattrack_4 2.0)) (`self.Star3StartLocation`)) false false))
          (:`Finished`
            (set `self.Interacted` false)))))))

(fn `Interact`
  (params (ActorInstigator :type "Actor Object Reference"))
  (returns (ReturnValue :type Boolean))
  (bind _returnvalue (`parent.Interact` ActorInstigator))
  (set `self.Interacted` true)
  (`GameplayStatics.PlaySoundAtLocation` "/Game/Audio/Sounds/Baby/baby-bell-rattle-04.baby-bell-rattle-04" (`self.K2_GetActorLocation`) (struct) 1.0 1.0 0.0 "/Game/Audio/Attenuation/Phonograph_Attenuation.Phonograph_Attenuation")
  (`TimelineComponent.PlayFromStart` (`self.Timeline_0`))
  (`TimelineComponent.PlayFromStart` (`self.Timeline_1`))
  (`TimelineComponent.PlayFromStart` (`self.Timeline_2`))
  (`TimelineComponent.PlayFromStart` (`self.Timeline_3`))
  (return _returnvalue))

(fn `UserConstructionScript`
  (`parent.UserConstructionScript`))