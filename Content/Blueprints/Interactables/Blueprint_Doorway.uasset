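; Interactable swinging door that enemies open on trigger overlap or interaction and other actors toggle through Interact.
; A timeline drives the yaw, reversing if retriggered mid-swing, with NegateSwing setting its direction and the construction script posing initially open doors.
; An OpenMutex flag blocks toggling after an enemy opens it until one leaves the trigger.
; Lock state selects the sound but does not gate the swing.
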(event `self.ReceiveBeginPlay`
  (if (not (`self.isUnlocked`))
    (set `self.WasPreviouslyLocked` true)))

(event `self.DoorTrigger.OnComponentBeginOverlap`
  (params (OverlappedComponent :type "PrimitiveComponent Object Reference") (OtherActor :type "Actor Object Reference") (OtherComp :type "PrimitiveComponent Object Reference") (OtherBodyIndex :type Integer) (bFromSweep :type Boolean) (SweepResult :type "HitResult Structure (by ref)"))
  ;[1 1 1] Event Overlap - Enable Disable Input
  (cast `/Game/Blueprints/Enemy/BP_EnemyCharacter` OtherActor)
  (`self.OpenDoor_Mutex`))

(event `self.DoorTrigger.OnComponentEndOverlap`
  (params (OverlappedComponent :type "PrimitiveComponent Object Reference") (OtherActor :type "Actor Object Reference") (OtherComp :type "PrimitiveComponent Object Reference") (OtherBodyIndex :type Integer))
  ;[1 1 1] Event Overlap - Enable Disable Input
  (cast `/Game/Blueprints/Enemy/BP_EnemyCharacter` OtherActor)
  (set `self.OpenMutex` false))

(event `Key|E`
  (params (Key :type "Key Structure" :default "AnyKey"))
  ;[1 1 1] Event Interaction - Open Close Door
)

(event `InputAction|Interact`
  (params (Key :type "Key Structure" :default "AnyKey"))
  ;[1 1 1] Set Door Interaction States
)

(event `OpenDoor_Mutex`
  (bind _isdooropen_ (`self.isDoorOpen?`))
  ;[1 1 1] Animating and Playing Sound on Door Opening
  (set `self.OpenMutex` true)
  (if (`self.isUnlocked`) :!label _label
    (if (`self.WasPreviouslyLocked`)
      (`GameplayStatics.PlaySound2D` "/Game/Audio/Sounds/Doors/Key_Wood_Door_A.Key_Wood_Door_A")
      (else
        (`GameplayStatics.PlaySound2D` "/Game/Audio/Sounds/Doors/Door_Medium_Open.Door_Medium_Open")))
    (else
      (`GameplayStatics.PlaySound2D` "/Game/Audio/Sounds/Doors/Door_Medium_Close.Door_Medium_Close") ; Door locked sound
    ))
  (if (`self.isAnimating?`)
    (set `self.isAnimating?` false)
    (`|ExecutionSequence`
      (:`then_0`
        (bind (_direction _door_yaw) (`Timeline|DoorOpenTimeline` :!via `Stop` :!label _label_2)
          (:`Update`
            (`SceneComponent.K2_SetRelativeRotation` (`self.Door`) (`KismetMathLibrary.MakeRotator` 0.0 0.0 (* _door_yaw (`self.YawNegator`))) false false)
            (set `self.isAnimating?` true))
          (:`Finished`
            (set `self.isAnimating?` false)
            (if (`self.isDoorOpen?`)
              (set `self.isDoorOpen?` false)
              (else
                (set `self.isDoorOpen?` true))))))
      (:`then_1`
        (set `self.isDoorOpen?` (not _isdooropen_))
        (if _isdooropen_
          (goto _label_2 :!via `Reverse`)
          (else
            (goto _label_2)))))
    (elif (`self.isDoorOpen?`)
      (goto _label_2 :!via `ReverseFromEnd`)
      (else
        (goto _label_2 :!via `PlayFromStart`)))))

(event `ToggleDoorSwing`
  ;[1 1 1] Animating and Playing Sound on Door Opening
  (if (not (`self.OpenMutex`))
    (goto _label)))

(fn `CloseDoor`
  (set `self.isDoorOpen?` false)
  (if (`self.Negate Swing`)
    (set `self.YawNegator` -1.0)
    (else
      (set `self.YawNegator` 1.0)))
  (`SceneComponent.K2_SetRelativeRotation` (`self.Door`) (`KismetMathLibrary.MakeRotator` 0.0) false false)
  (`KismetSystemLibrary.PrintString` "CLOSED DOOR"))

(fn `Interact`
  (params (ActorInstigator :type "Actor Object Reference"))
  (returns (ReturnValue :type Boolean))
  (`parent.Interact` ActorInstigator)
  (cast `EnemyCharacter` ActorInstigator
    (:`then`
      (`self.OpenDoor_Mutex`))
    (:`CastFailed`
      (`self.ToggleDoorSwing`)))
  (return true))

(fn `LockDoor`
  (set `self.isUnlocked` false))

(fn `OpenDoor`
  (set `self.isDoorOpen?` true)
  (if (`self.Negate Swing`)
    (set `self.YawNegator` -1.0)
    (else
      (set `self.YawNegator` 1.0)))
  (if (`self.isDoorOpen?`)
    (`SceneComponent.K2_SetRelativeRotation` (`self.Door`) (`KismetMathLibrary.MakeRotator` 0.0 0.0 (* (`self.YawNegator`) 90.0)) false false)))

(fn `UnlockDoor`
  (set `self.isUnlocked` true))

(fn `UserConstructionScript`
  (if (`self.Negate Swing`)
    (set `self.YawNegator` -1.0)
    (else
      (set `self.YawNegator` 1.0)))
  (if (`self.isDoorOpen?`)
    (`SceneComponent.K2_SetRelativeRotation` (`self.Door`) (`KismetMathLibrary.MakeRotator` 0.0 0.0 (* (`self.YawNegator`) 90.0)) false false)
    (`KismetSystemLibrary.PrintString` "Hello")))