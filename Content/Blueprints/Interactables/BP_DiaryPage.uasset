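; BP_DiaryPage is a collectible diary page interactable that the player picks up when inspection ends.
; It extends the parent's end-inspect event to notify the player, add itself to the inventory keyed by object name, and show diary pages on the HUD.
; Instead of being destroyed, the collected actor loses mesh collision, hides and moves below the world.
; BeginPlay resets the collected flag and finds the BP_HUD actor.
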(event `self.OnEndInspect`
  (bind _playerbindref (`self.PlayerBindRef`))
  (`PrimitiveComponent.SetCollisionEnabled` (`self.StaticMesh`) "NoCollision")
  (`parent.OnEndInspect`)
  (`/Game/Blueprints/FirstPersonCharacter/FirstPersonCharacter.CollectDiaryPage` _playerbindref)
  (`/Game/Blueprints/Components/BP_Inventory.Add Item` (`/Game/Blueprints/FirstPersonCharacter/FirstPersonCharacter.BP_Inventory` _playerbindref) (`KismetSystemLibrary.GetObjectName` self) self)
  (`self.SetActorHiddenInGame` true)
  (`self.K2_SetActorLocation` (0.0 0.0 -3000.0))
  (set `self.IsCollected` true)
  (`/Game/Blueprints/FirstPersonCharacter/BP_HUD.ShowDiaryPages` (`self.HUD_Ref`)))

(event `self.ReceiveBeginPlay`
  (set `self.IsCollected` false)
  (bind _outactors (`GameplayStatics.GetAllActorsOfClass` "/Game/Blueprints/FirstPersonCharacter/BP_HUD.BP_HUD_C"))
  (for _array_element _outactors
    (set `self.HUD_Ref` _array_element)))

(fn `UserConstructionScript`
  (`parent.UserConstructionScript`))