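; BP_Phonograph is an interactable that toggles a spatialized song on and off, playing a 2D eject sound when stopped.
; BeginPlay spawns a persistent, attenuated audio component at the actor's location, stops it immediately and caches the first-person player.
; Every Tick compares player and phonograph height, stepping volume down when they are over 350 units apart vertically and back up otherwise, so the fade speed depends on frame rate.
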(event `self.ReceiveTick`
  (params (DeltaSeconds :type "Float (single-precision)"))
  (`self.CheckZPlayer`))

(event `self.ReceiveBeginPlay`
  (bind _returnvalue (`GameplayStatics.SpawnSoundAtLocation` (`self.Song`) (`self.K2_GetActorLocation`) (struct) 1.0 1.0 0.0 (`self.Attenuation`) null false))
  (bind _output_get (set `self.AudioComponent` _returnvalue))
  (`AudioComponent.Stop` _output_get)
  (bind _asfirst_person_character (cast `/Game/Blueprints/FirstPersonCharacter/FirstPersonCharacter` (`GameplayStatics.GetPlayerPawn` 0)))
  (set `self.Player` _asfirst_person_character))

(fn `CheckZPlayer`
  (if (> (`KismetMathLibrary.Abs` (- (.z (`self.K2_GetActorLocation`)) (.z (`self.K2_GetActorLocation` (`self.Player`))))) 350.0)
    (if (> (`self.Volume`) 0.01)
      (set `self.Volume` (- (`self.Volume`) 0.005))
      (`AudioComponent.SetVolumeMultiplier` (`self.AudioComponent`) (`self.Volume`) :!label _label))
    (elif (< (`self.Volume`) 1.0)
      (set `self.Volume` (+ (`self.Volume`) 0.005))
      (goto _label))))

(fn `Interact`
  (params (ActorInstigator :type "Actor Object Reference"))
  (returns (ReturnValue :type Boolean))
  (bind _audiocomponent (`self.AudioComponent`))
  (bind _returnvalue (`parent.Interact` null))
  (if (`AudioComponent.IsPlaying` (`self.AudioComponent`))
    (`AudioComponent.Stop` _audiocomponent)
    (`GameplayStatics.PlaySound2D` "/Game/Audio/Sounds/Buttons/Others/Plastic_Eject_Empty.Plastic_Eject_Empty")
    (else
      (`AudioComponent.Play` _audiocomponent 0.0)))
  (return _returnvalue))

(fn `UserConstructionScript`
  (`parent.UserConstructionScript`))