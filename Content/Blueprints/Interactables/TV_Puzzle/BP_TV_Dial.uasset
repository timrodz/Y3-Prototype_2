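; TV puzzle dial that the player turns with vertical mouse input to change the texture mix on a linked TV.
; The input handler rotates the Cylinder by the look-up rate, combining rotators built from camera-derived axes.
; The resulting pitch, divided by 90 and clamped to 0–1, sets the TV's Mix and triggers its texture update.
; BeginPlay resets DialRotation; CustomEvent and the Round graph are unfinished.
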(event `self.ReceiveBeginPlay`
  (`parent.ReceiveBeginPlay`)
  (set `self.DialRotation` (`self.OriginalRotation`)))

(event `self.PlayerMouseInputHandler`
  (params (TurnRate :type "Float (single-precision)") (LookUpRate :type "Float (single-precision)"))
  (bind _tv_ref (`self.TV_Ref`))
  (bind (_returnvalue_roll _returnvalue_pitch) (`KismetMathLibrary.BreakRotator` (`SceneComponent.K2_GetComponentRotation` (`/Game/Blueprints/FirstPersonCharacter/FirstPersonCharacter.Camera` (`self.PlayerBindRef`)))))
  (bind _returnvalue (`KismetMathLibrary.ComposeRotators` (`KismetMathLibrary.RotatorFromAxisAndAngle` (`KismetMathLibrary.GetUpVector` (`KismetMathLibrary.MakeRotator` _returnvalue_roll))) (`KismetMathLibrary.ComposeRotators` (`SceneComponent.RelativeRotation` (`self.Cylinder`)) (`KismetMathLibrary.RotatorFromAxisAndAngle` (`KismetMathLibrary.GetRightVector` (`KismetMathLibrary.MakeRotator` 0.0 _returnvalue_pitch)) LookUpRate))))
  (`SceneComponent.K2_SetRelativeRotation` (`self.Cylinder`) _returnvalue false false)
  (set `/Game/Blueprints/Interactables/BP_TV_Interactable.Mix` (`KismetMathLibrary.FClamp` (/ (.pitch _returnvalue) 90.0)) _tv_ref)
  (`/Game/Blueprints/Interactables/BP_TV_Interactable.UpdateTextureMix` _tv_ref))

(event `CustomEvent`
  (params (TurnRate :type "Float (double-precision)") (LookUpRate :type "Float (double-precision)")))

(fn `UserConstructionScript`
  (`parent.UserConstructionScript`))