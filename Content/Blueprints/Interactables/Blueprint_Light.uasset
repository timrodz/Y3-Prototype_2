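; Interactable light actor that the player toggles on and off with the E key while inside its box trigger.
; Box overlap begin and end events enable and disable input for player controller 0, without checking which actor overlaps.
; Pressing E flips LightIsOff, which scales the point light's intensity between zero and the brightness cached at BeginPlay.
; The construction script applies the same intensity formula from LightIsOff and InitialBrightness.
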(event `self.ReceiveBeginPlay`
  (set `self.InitialBrightness` (`LightComponentBase.Intensity` (`self.PointLight`))))

(event `self.Box.OnComponentEndOverlap`
  (params (OverlappedComponent :type "PrimitiveComponent Object Reference") (OtherActor :type "Actor Object Reference") (OtherComp :type "PrimitiveComponent Object Reference") (OtherBodyIndex :type Integer))
  (`self.DisableInput` (`GameplayStatics.GetPlayerController` 0)))

(event `self.Box.OnComponentBeginOverlap`
  (params (OverlappedComponent :type "PrimitiveComponent Object Reference") (OtherActor :type "Actor Object Reference") (OtherComp :type "PrimitiveComponent Object Reference") (OtherBodyIndex :type Integer) (bFromSweep :type Boolean) (SweepResult :type "HitResult Structure (by ref)"))
  (`self.EnableInput` (`GameplayStatics.GetPlayerController` 0)))

(event `Key|E`
  (params (Key :type "Key Structure" :default "AnyKey"))
  (bind _lightisoff (`self.LightIsOff`))
  (:`Pressed`
    (if _lightisoff
      _
      (else
        _))
    (bind _output_get (set `self.LightIsOff` (not _lightisoff)))
    (`LightComponent.SetIntensity` (`self.PointLight`) (* (- 1.0 (`KismetMathLibrary.Conv_BoolToDouble` _output_get)) (`self.InitialBrightness`)))))

(fn `UserConstructionScript`
  (`LightComponent.SetIntensity` (`self.PointLight`) (* (- 1.0 (`KismetMathLibrary.Conv_BoolToDouble` (`self.LightIsOff`))) (`self.InitialBrightness`))))