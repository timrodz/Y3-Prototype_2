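; BP_DoorKey1 is a key pickup, an equippable interactable that unlocks a linked door.
; On Interact it runs the parent logic, adds itself to the first-person character's inventory under its item name and equips it.
; It then sets DoorToUnlock's unlocked flag directly on pickup and plays a pitched-up switch sound at the mesh.
; A custom event turns on physics simulation for the mesh.
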(event Custom|CustomEvent
  (Physics|SetSimulatePhysics (Variables|Default|GetEquipMesh) true))

(event EventBeginPlay)

(event Collision|EventActorBeginOverlap
  (params (OtherActor :type Actor%20Object%20Reference)))

(event EventTick
  (params (DeltaSeconds :type Float%20%28single-precision%29)))

(fn ConstructionScript
  (|CallParentFunction))

(fn Interact
  (params (ActorInstigator :type Actor%20Object%20Reference))
  (bind _itemname (Variables|Default|GetItemName))
  (|CallParentFunction 0)
  (bind _asfirst_person_character (Utilities|Casting|CastToFirstPersonCharacter ActorInstigator))
  (Default|AddItem (Variables|/Game/Blueprints/FirstPersonCharacter/FirstPersonCharacter.FirstPersonCharacter_C|GetBP_Inventory _asfirst_person_character) _itemname self)
  (Default|EquipItem (Variables|/Game/Blueprints/FirstPersonCharacter/FirstPersonCharacter.FirstPersonCharacter_C|GetBP_Inventory _asfirst_person_character) _itemname)
  (Variables|/Game/Blueprints/Interactables/Blueprint_Doorway.Blueprint_Doorway_C|SetisUnlocked (Variables|Default|GetDoorToUnlock) true)
  (Audio|PlaySoundatLocation "/Game/Audio/Sounds/Buttons/Others/Switch_Box_C.Switch_Box_C" (Transformation|GetWorldLocation (Variables|Default|GetEquipMesh)) "0, 0, 0" 1.0 1.5 0.0 0 "/Game/Audio/Sounds/SoundFX.SoundFX")
  (return (stale _returnvalue)))