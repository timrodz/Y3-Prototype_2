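; Equippable hammer pickup that joins the first-person character's inventory and can be swung.
; Interacting spawns a copy of itself, adds it to BPInventory under ItemName, equips it and destroys the original.
; ToggleMethodA alternates between playing and reversing the RotateHit timeline, which rolls the mesh on a sped-up swing.
; Sphere component hits or the Hit event stop the swing mid-motion, and Drop enables physics on the mesh.
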(event `self.Toggle_Method_A`
  (bind _equipmesh (`self.EquipMesh`))
  (`KismetSystemLibrary.PrintString` "Hit")
  (`/Engine/EditorBlueprintResources/StandardMacros.FlipFlop`
    (:`A`
      (`TimelineComponent.SetPlayRate` (`self.RotateHit`) 4.0)
      (bind (_direction _newtrack_0) (`Timeline|RotateHit` :!via `PlayFromStart` :!label _label)
        (:`Update`
          (`SceneComponent.K2_SetRelativeRotation` _equipmesh (`KismetMathLibrary.MakeRotator` _newtrack_0 (.pitch (`SceneComponent.RelativeRotation` _equipmesh)) (.yaw (`SceneComponent.RelativeRotation` _equipmesh))) false false))))
    (:`B`
      (goto _label :!via `Reverse`))))

(event `self.Drop`
  (`PrimitiveComponent.SetSimulatePhysics` (`self.EquipMesh`) true))

(event `self.ReceiveHit`
  (params (MyComp :type "PrimitiveComponent Object Reference") (Other :type "Actor Object Reference") (OtherComp :type "PrimitiveComponent Object Reference") (bSelfMoved :type Boolean) (HitLocation :type "Vector Structure") (HitNormal :type "Vector Structure") (NormalImpulse :type "Vector Structure") (Hit :type "HitResult Structure (by ref)"))
  (`TimelineComponent.Stop` (`self.RotateHit`) :!label _label_2))

(event `self.Sphere.OnComponentHit`
  (params (HitComponent :type "PrimitiveComponent Object Reference") (OtherActor :type "Actor Object Reference") (OtherComp :type "PrimitiveComponent Object Reference") (NormalImpulse :type "Vector Structure") (Hit :type "HitResult Structure (by ref)"))
  (goto _label_2))

(fn `Interact`
  (params (ActorInstigator :type "Actor Object Reference"))
  (returns (ReturnValue :type Boolean))
  (bind _itemname (`self.ItemName`))
  (`parent.Interact` null)
  (bind _asfirst_person_character (cast `/Game/Blueprints/FirstPersonCharacter/FirstPersonCharacter` ActorInstigator))
  (bind _returnvalue (`|SpawnActorFromClass` (`GameplayStatics.GetObjectClass` self) (`SceneComponent.K2_GetComponentToWorld` (`self.DefaultSceneRoot`)) "Undefined" "OverrideRootScale"))
  (bind _bp_inventory (`/Game/Blueprints/FirstPersonCharacter/FirstPersonCharacter.BP_Inventory` _asfirst_person_character))
  (`/Game/Blueprints/Components/BP_Inventory.Add Item` _bp_inventory _itemname _returnvalue)
  (`/Game/Blueprints/Components/BP_Inventory.Equip Item` _bp_inventory _itemname)
  (`self.K2_DestroyActor`)
  (return false))

(fn `UserConstructionScript`
  (`parent.UserConstructionScript`))