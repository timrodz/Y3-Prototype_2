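; Flashlight pickup that a FirstPersonCharacter can collect into its inventory and switch on and off.
; Interact spawns a copy of itself, toggles it if the original light is off, adds and equips it under ItemName, then destroys the original.
; ToggleMethodA flip-flops the spotlight between zero and the intensity cached in the construction script, with switch sounds.
; Drop turns on physics simulation for the equip mesh.
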(event `self.ReceiveBeginPlay`)

(event `self.Toggle_Method_A`
  (bind _spotlight (`self.SpotLight`))
  (bind _returnvalue (`SceneComponent.K2_GetComponentLocation` (`self.SpotLight`)))
  (`/Engine/EditorBlueprintResources/StandardMacros.FlipFlop`
    (:`A`
      (`LightComponent.SetIntensity` _spotlight 0.0)
      (`GameplayStatics.PlaySoundAtLocation` "/Game/Audio/Sounds/Buttons/Others/Switch_Toggle_A.Switch_Toggle_A" _returnvalue))
    (:`B`
      (`LightComponent.SetIntensity` _spotlight (`self.Intensity`))
      (`GameplayStatics.PlaySoundAtLocation` "/Game/Audio/Sounds/Buttons/Others/Switch_Toggle_D.Switch_Toggle_D" _returnvalue))))

(event `self.Drop`
  (`PrimitiveComponent.SetSimulatePhysics` (`self.EquipMesh`) true))

(fn `Interact`
  (params (ActorInstigator :type "Actor Object Reference"))
  (returns (ReturnValue :type Boolean))
  (bind _itemname (`self.ItemName`))
  (`parent.Interact` null)
  (bind _asfirst_person_character (cast `/Game/Blueprints/FirstPersonCharacter/FirstPersonCharacter` ActorInstigator))
  (bind _returnvalue (`|SpawnActorFromClass` (`GameplayStatics.GetObjectClass` self) (`SceneComponent.K2_GetComponentToWorld` (`self.DefaultSceneRoot`)) "Undefined" "OverrideRootScale"))
  (if (not (> (`LightComponentBase.Intensity` (`self.SpotLight`)) 0.0))
    (`self.Toggle_Method_A` _returnvalue))
  (bind _bp_inventory (`/Game/Blueprints/FirstPersonCharacter/FirstPersonCharacter.BP_Inventory` _asfirst_person_character))
  (`/Game/Blueprints/Components/BP_Inventory.Add Item` _bp_inventory _itemname _returnvalue)
  (`/Game/Blueprints/Components/BP_Inventory.Equip Item` _bp_inventory _itemname)
  (`GameplayStatics.PlaySoundAtLocation` "/Game/Audio/Sounds/Buttons/Others/Switch_Toggle_A.Switch_Toggle_A" (`SceneComponent.K2_GetComponentLocation` (`self.SpotLight`)))
  (`self.K2_DestroyActor`))

(fn `SpawnNew`)

(fn `UserConstructionScript`
  (`parent.UserConstructionScript`)
  (set `self.Intensity` (`LightComponentBase.Intensity` (`self.SpotLight`))))