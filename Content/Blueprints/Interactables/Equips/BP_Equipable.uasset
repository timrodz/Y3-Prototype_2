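; BP_Equipable is a base for equippable interactable items that the first-person character picks up.
; On BeginPlay it appends BaseInstances to ItemName, which serves as the inventory key.
; Interact calls the parent, adds itself to the character's BPInventory, equips by name, prints whether it was found and enables input for player 0.
; Drop, ToggleMethodA and ActiveMethodA are empty stubs.
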(event `self.ReceiveBeginPlay`
  (set `self.ItemName` (`KismetStringLibrary.Concat_StrStr` (`self.ItemName`) "_" (`KismetStringLibrary.Conv_IntToString` (`self.BaseInstances`)))))

(fn `Active_Method_A`)

(fn `Drop`)

(fn `Interact`
  (params (ActorInstigator :type "Actor Object Reference"))
  (returns (ReturnValue :type Boolean))
  (bind _itemname (`self.ItemName`))
  (bind _returnvalue (`parent.Interact` null))
  (bind _asfirst_person_character (cast `/Game/Blueprints/FirstPersonCharacter/FirstPersonCharacter` ActorInstigator))
  (bind _bp_inventory (`/Game/Blueprints/FirstPersonCharacter/FirstPersonCharacter.BP_Inventory` _asfirst_person_character))
  (`/Game/Blueprints/Components/BP_Inventory.Add Item` _bp_inventory _itemname self)
  (bind (_value _found) (`/Game/Blueprints/Components/BP_Inventory.Equip Item` _bp_inventory _itemname))
  (`KismetSystemLibrary.PrintString` (`KismetStringLibrary.Conv_BoolToString` _found) false)
  (`self.EnableInput` (`GameplayStatics.GetPlayerController` 0))
  (return _returnvalue))

(fn `Toggle_Method_A`)

(fn `UserConstructionScript`
  (`parent.UserConstructionScript`))