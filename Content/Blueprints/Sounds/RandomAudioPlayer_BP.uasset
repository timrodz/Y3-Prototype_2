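; Actor that plays randomly chosen sounds at random positions and random intervals.
; BeginPlay warns about empty arrays and picks the initial delay, then a Tick timer calls PlaySound and rerolls the delay from a separate range.
; Each sound plays at either a random preset actor's location or a random point inside a hardcoded world-space box, using configurable volume and attenuation plus a concurrency setting.
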(event `self.ReceiveBeginPlay`
  (if (== (`KismetArrayLibrary.Array_Length` (`self.Sounds`)) 0)
    (`KismetSystemLibrary.PrintString` "No Random Sounds Added!")
    (else
      (set `self.RandomTime` (`KismetMathLibrary.RandomFloatInRange` (`self.InitialTimeBeforeSoundMin`) (`self.InitialTimeBeforeSoundMax`)))
      (if (`self.UsingPresetLocations`)
        (if (== (`KismetArrayLibrary.Array_Length` (`self.SoundLocations`)) 0)
          (`KismetSystemLibrary.PrintString` "No Sound Locations Added!"))))))

(event `self.ReceiveTick`
  (params (DeltaSeconds :type "Float (single-precision)"))
  (bind _output_get (set `self.Timer` (+ DeltaSeconds (`self.Timer`))))
  (if (> _output_get (`self.RandomTime`))
    (`self.PlaySound`)
    (set `self.Timer` 0.0)
    (set `self.RandomTime` (`KismetMathLibrary.RandomFloatInRange` (`self.TimeBeforeSoundMin`) (`self.TimeBeforeSoundMax`)))))

(fn `GetRandomLocation`
  (returns (Location :type "Vector Structure"))
  (if (`self.UsingPresetLocations`)
    (set `self.LocationToUse` (`self.K2_GetActorLocation` (`|GetArrayItem` (`self.SoundLocations`) (`KismetMathLibrary.RandomIntegerInRange` 0 (- (`KismetArrayLibrary.Array_Length` (`self.SoundLocations`)) 1)))))
    (else
      (set `self.LocationToUse` (`KismetMathLibrary.MakeVector` (`KismetMathLibrary.RandomFloatInRange` -1000.0 5000.0) (`KismetMathLibrary.RandomFloatInRange` -1000.0 4000.0) (`KismetMathLibrary.RandomFloatInRange` 0.0 1000.0)))))
  (return (`self.LocationToUse`)))

(fn `GetRandomSound`
  (returns (Sound :type "SoundWave Object Reference"))
  (return (`|GetArrayItem` (`self.Sounds`) (`KismetMathLibrary.RandomIntegerInRange` 0 (- (`KismetArrayLibrary.Array_Length` (`self.Sounds`)) 1)))))

(fn `PlaySound`
  (bind _location (`self.GetRandomLocation`))
  (bind _sound (`self.GetRandomSound`))
  (`GameplayStatics.PlaySoundAtLocation` _sound _location (struct) (`self.VolumeMultiplier`) 1.0 0.0 (`self.Attenuation`) "/Game/Audio/Sounds/SoundFX.SoundFX"))

(fn `UserConstructionScript`)