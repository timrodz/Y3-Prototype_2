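; Candle actor whose flame starts hidden, is lit by a nearby player and put out by a nearby enemy.
; Collision sphere overlaps track the player and enemy, and Tick toggles flame visibility while either passes IsCloseToCandle.
; That check compares offset actor height with the candle's and requires world X beyond a hardcoded threshold.
; The enemy check runs last but is skipped when an overlapping player fails the closeness test.
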(event `self.ReceiveTick`
  (params (DeltaSeconds :type "Float (single-precision)"))
  (if (`self.IsOverlappingPlayer`)
    (bind _isclose (`self.IsCloseToCandle` (`self.K2_GetActorLocation` (`self.Player`))))
    (if _isclose
      (`SceneComponent.SetHiddenInGame` (`self.Flame`) false false)
      (if (`self.IsOverlappingEnemy`) :!label _label
        (bind _isclose_2 (`self.IsCloseToCandle` (`self.K2_GetActorLocation` (`self.Enemy`))))
        (if _isclose_2
          (`SceneComponent.SetHiddenInGame` (`self.Flame`) true false))))
    (else
      (goto _label))))

(event `self.ReceiveBeginPlay`
  (`SceneComponent.SetHiddenInGame` (`self.Flame`) true false))

(event `self.CollisionSphere.OnComponentBeginOverlap`
  (params (OverlappedComponent :type "PrimitiveComponent Object Reference") (OtherActor :type "Actor Object Reference") (OtherComp :type "PrimitiveComponent Object Reference") (OtherBodyIndex :type Integer) (bFromSweep :type Boolean) (SweepResult :type "HitResult Structure (by ref)"))
  (bind _asfirst_person_character (cast `/Game/Blueprints/FirstPersonCharacter/FirstPersonCharacter` OtherActor)
    (:`then`
      (set `self.Player` _asfirst_person_character)
      (set `self.IsOverlappingPlayer` true))
    (:`CastFailed`
      (bind _asenemy_character (cast `EnemyCharacter` OtherActor))
      (set `self.Enemy` _asenemy_character)
      (set `self.IsOverlappingEnemy` true))))

(event `self.CollisionSphere.OnComponentEndOverlap`
  (params (OverlappedComponent :type "PrimitiveComponent Object Reference") (OtherActor :type "Actor Object Reference") (OtherComp :type "PrimitiveComponent Object Reference") (OtherBodyIndex :type Integer))
  (bind _asfirst_person_character (cast `/Game/Blueprints/FirstPersonCharacter/FirstPersonCharacter` OtherActor)
    (:`then`
      (set `self.Player` _asfirst_person_character)
      (set `self.IsOverlappingPlayer` false))
    (:`CastFailed`
      (bind _asenemy_character (cast `EnemyCharacter` OtherActor))
      (set `self.Enemy` _asenemy_character)
      (set `self.IsOverlappingEnemy` false))))

(fn `IsCloseToCandle`
  (params (ActorLoc :type "Vector Structure"))
  (returns (IsClose :type Boolean))
  (return (and (< (`KismetMathLibrary.Abs` (- (.z (`self.K2_GetActorLocation`)) (- (.z ActorLoc) 90.0))) 130.0) (> (.x ActorLoc) 2500.0))))

(fn `UserConstructionScript`)