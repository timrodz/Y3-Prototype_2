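; Legacy box zone actor that groups lamps and keys and tracks whether an enemy is inside.
; On BeginPlay it collects overlapping BP_Lamp and BP_Key actors and sets itself as their Zone; actor overlaps maintain the enemy presence flag and reference.
; OLDUpdateZoneItems is an empty stub: its disconnected logic would flag lit lamps or taken keys and alert the enemy.
; A construction-script lamp scan is also disconnected.
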(event `self.ReceiveBeginPlay`
  (for _array_element (`PrimitiveComponent.GetOverlappingActors` (`self.Box`) null)
    (bind _asbp_lamp (cast `/Game/Blueprints/BP_Lamp` _array_element)
      (:`then`
        (`KismetArrayLibrary.Array_Add` (`self.Lamp_List`) _asbp_lamp)
        (set `/Game/Blueprints/BP_Lamp.Zone` self _asbp_lamp))
      (:`CastFailed`
        (bind _asbp_key (cast `/Game/Blueprints/BP_Key` _array_element))
        (`KismetArrayLibrary.Array_Add` (`self.Key_List`) _asbp_key)
        (set `/Game/Blueprints/BP_Key.Zone` self _asbp_key))))
  (`self.OLD_UpdateZoneItems`))

(event `self.ReceiveActorBeginOverlap`
  (params (OtherActor :type "Actor Object Reference"))
  (bind _asbp_enemy_character (cast `/Game/Blueprints/Enemy/BP_EnemyCharacter` OtherActor))
  (set `self.EnemyRef` _asbp_enemy_character)
  (set `self.EnemyInZone` true))

(event `self.ReceiveActorEndOverlap`
  (params (OtherActor :type "Actor Object Reference"))
  (cast `/Game/Blueprints/Enemy/BP_EnemyCharacter` OtherActor)
  (set `self.EnemyInZone` false))

(event `self.ReceiveTick`
  (params (DeltaSeconds :type "Float (single-precision)")))

(fn `OLD_UpdateZoneItems`)

(fn `UserConstructionScript`)