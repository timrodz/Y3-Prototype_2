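; BP_WallSpline is a construction-script tool that builds a straight wall or fence from a repeated mesh toward an EndPoint offset.
; It optionally derives segment width from the larger horizontal side of the mesh bounds, then rounds horizontal distance over width to get the segment count.
; Extra segments attach along local X to FenceStart, which is yawed toward the end point.
; Despite its name, it uses no spline component.
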(fn `UserConstructionScript`
  (bind _returnvalue (`self.K2_GetActorLocation`))
  (bind (_min _max) (break `Box` (`StaticMesh.GetBoundingBox` (`self.Mesh to spawn`))))
  (bind _x (.x (- _max _min)))
  (bind _y (.y (- _max _min)))
  (bind _returnvalue_2 (- (`KismetMathLibrary.Round` (/ (`KismetMathLibrary.VSize` (* (`self.End point`) (1.0 1.0 0.0))) (`self.Mesh width`))) 1))
  (if (`self.AutoWidth`)
    (if (> _x _y)
      (set `self.Mesh width` _x)
      (else
        (set `self.Mesh width` _y))))
  (`StaticMeshComponent.SetStaticMesh` (`self.Fence start`) (`self.Mesh to spawn`)) ; Change spawned mesh to the new type
  (if (> _returnvalue_2 0)
    (for _index (range 1 (+ _returnvalue_2 1))
      (bind _returnvalue_3 (`AddComponent|NODE_AddStaticMeshComponent-0` :`bManualAttachment` true))
      (`SceneComponent.K2_AttachTo` _returnvalue_3 (`self.Fence start`) "None" "KeepWorldPosition" true) ; Attach each segment to the initial mesh
      (`SceneComponent.K2_SetRelativeLocation` _returnvalue_3 (`KismetMathLibrary.MakeVector` (* _index (`self.Mesh width`))) false false)
      (`StaticMeshComponent.SetStaticMesh` _returnvalue_3 (`self.Mesh to spawn`)) ; Change spawned mesh to the new type
    ))
  (`SceneComponent.K2_SetWorldRotation` (`self.Fence start`) (`KismetMathLibrary.MakeRotator` 0.0 0.0 (.yaw (`KismetMathLibrary.FindLookAtRotation` _returnvalue (+ _returnvalue (`self.End point`))))) false false) ; Rotate the initial mesh to face the end point
)