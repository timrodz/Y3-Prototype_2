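; Actor that lays out a 3D inventory menu as a ring of item meshes, currently all the same FlashLight placeholder, viewed by a SceneCaptureComponent2D.
; The construction script places the capture outside the ring facing the actor, then spawns static mesh components at equal angles around it.
; SetWorldScale uniformly fits each mesh into a fixed extent and offsets it to compensate for off-center pivots.
; The event graph has no runtime logic.
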(fn `SetWorldScale`
  (params (StaticMesh1 :type "StaticMeshComponent Object Reference"))
  (locals (StaticMesh :type "StaticMeshComponent Object Reference") (NewLocalVar_0 :type "Vector Structure" :default (0.0 0.0 0.0)) (CurrentExtendMesh :type "Vector Structure"))
  (bind _staticmesh (`local.StaticMesh`))
  (set `local.StaticMesh` StaticMesh1)
  (set `local.CurrentExtendMesh` (`.BoxExtent` (`KismetSystemLibrary.GetComponentBounds` (`local.StaticMesh`))))
  (`SceneComponent.SetWorldScale3D` (`local.StaticMesh`) (* (`SceneComponent.K2_GetComponentScale` (`local.StaticMesh`)) (`KismetMathLibrary.FMin` (/ (.x (`KismetMathLibrary.MakeVector` 18.0 18.0 18.0)) (.x (`local.CurrentExtendMesh`))) (/ (.y (`KismetMathLibrary.MakeVector` 18.0 18.0 18.0)) (.y (`local.CurrentExtendMesh`))) (/ (.z (`KismetMathLibrary.MakeVector` 18.0 18.0 18.0)) (.z (`local.CurrentExtendMesh`))))))
  (`SceneComponent.K2_AddLocalOffset` (`local.StaticMesh`) (- (`SceneComponent.K2_GetComponentLocation` _staticmesh) (`KismetSystemLibrary.GetComponentBounds` _staticmesh)) false false))

(fn `UserConstructionScript`
  (bind _scenecapturecomponent2d (`self.SceneCaptureComponent2D`))
  (`SceneComponent.K2_SetRelativeLocation` (`self.SceneCaptureComponent2D`) (`KismetMathLibrary.MakeVector` (* (`self.RingSize`) 2.0)) false false)
  (`SceneComponent.K2_SetWorldRotation` _scenecapturecomponent2d (`KismetMathLibrary.FindLookAtRotation` (`SceneComponent.K2_GetComponentLocation` _scenecapturecomponent2d) (`self.K2_GetActorLocation`)) false false)
  (`KismetArrayLibrary.Array_Clear` (`self.Comps`))
  (for _index (range (+ (`self.NumItems`) 1))
    (bind _returnvalue (`AddComponent|NODE_AddStaticMeshComponent-0` :`RelativeTransform` (`KismetMathLibrary.MakeTransform` (`KismetMathLibrary.GreaterGreater_VectorRotator` (`KismetMathLibrary.MakeVector` (`self.RingSize`)) (`KismetMathLibrary.MakeRotator` 0.0 0.0 (* _index (/ 360.0 (`KismetMathLibrary.Conv_IntToDouble` (`self.NumItems`)))))))))
    (`StaticMeshComponent.SetStaticMesh` _returnvalue "/Game/Assets/Lights/FlashLight.FlashLight")
    (`self.SetWorldScale` _returnvalue)))