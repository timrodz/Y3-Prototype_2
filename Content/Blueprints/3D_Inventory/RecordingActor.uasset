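; 3D inventory carousel actor that shows copies of item actors in a ring in front of a SceneCaptureComponent2D.
; AddActor spawns and attaches each copy, fits it to DesiredExtend by bounds and spaces the items evenly around the ring.
; A and D change CurrentNum, and Tick eases the ring's yaw toward it.
; W reverses the Alpha timeline, which drives scale and player-camera depth of field and holds the inventory teardown.
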(event `self.ReceiveBeginPlay`
  (bind _scenecapturecomponent2d (`self.SceneCaptureComponent2D`))
  ;[1 1 1] Begin play
  (`self.EnableInput` (`GameplayStatics.GetPlayerController` 0))
  (`SceneComponent.K2_SetWorldRotation` _scenecapturecomponent2d (`KismetMathLibrary.FindLookAtRotation` (`SceneComponent.K2_GetComponentLocation` _scenecapturecomponent2d) (`SceneComponent.K2_GetComponentLocation` (`self.DefaultSceneRoot`))) false false))

(event `self.ReceiveTick`
  (params (DeltaSeconds :type "Float (single-precision)"))
  ;[1 1 1] Event Tick Rotation
  (`SceneComponent.K2_SetWorldRotation` (`self.Scene`) (`KismetMathLibrary.RInterpTo` (`SceneComponent.K2_GetComponentRotation` (`self.Scene`)) (`KismetMathLibrary.MakeRotator` 0.0 0.0 (* (`self.CurrentNum`) (/ 360.0 (`KismetMathLibrary.Conv_IntToDouble` (`KismetArrayLibrary.Array_Length` (`self.Actors`)))))) DeltaSeconds 4.0) false false))

(event `UpdateScale`
  ;[1 1 1] update Scale of all items in view
  (for (_array_element _array_index) (`self.Actors`)
    (set `self.CurrentExtendMesh` (`.BoxExtent` (`self.GetActorBounds` _array_element false)))
    (`self.SetActorScale3D` _array_element (* (1.0 1.0 1.0) (`KismetMathLibrary.FMin` (/ (.x (`self.DesiredExtend`)) (.x (`self.CurrentExtendMesh`))) (/ (.y (`self.DesiredExtend`)) (.y (`self.CurrentExtendMesh`))) (/ (.z (`self.DesiredExtend`)) (.z (`self.CurrentExtendMesh`))))))
    (`self.K2_SetActorRelativeLocation` _array_element (`KismetMathLibrary.GreaterGreater_VectorRotator` (`KismetMathLibrary.MakeVector` (`self.RingSize`)) (`KismetMathLibrary.MakeRotator` 0.0 0.0 (* _array_index (/ 360.0 (`KismetMathLibrary.Conv_IntToDouble` (`KismetArrayLibrary.Array_Length` (`self.Actors`))))))) false false)))

(event `Key|A`
  (params (Key :type "Key Structure" :default "AnyKey"))
  ;[1 1 1] Rotate Right - Left
  (:`Pressed`
    (bind _result (`/Engine/EditorBlueprintResources/StandardMacros.DecrementInt` (`self.CurrentNum`))
      (:`  `
        (if (< _result 1)
          (set `self.CurrentNum` (`KismetArrayLibrary.Array_Length` (`self.Actors`))))))))

(event `Key|D`
  (params (Key :type "Key Structure" :default "AnyKey"))
  ;[1 1 1] Rotate Right - Left
  (:`Pressed`
    (bind _result (`/Engine/EditorBlueprintResources/StandardMacros.IncrementInt` (`self.CurrentNum`))
      (:`  `
        (if (> _result (- (`KismetArrayLibrary.Array_Length` (`self.Actors`)) 1))
          (set `self.CurrentNum` 0))))))

(event `Key|W`
  (params (Key :type "Key Structure" :default "AnyKey"))
  (:`Pressed`
    (`TimelineComponent.ReverseFromEnd` (`self.Alpha`))))

(fn `AddActor`
  (params (Target :type "Actor Object Reference"))
  (bind _returnvalue (`MyFunctionLibrary.SpawnActorCopy` Target (make `_BP_ActorSpawnParameters` "None" Target null null null "AlwaysSpawn")))
  (`self.SetActorScale3D` _returnvalue (1.0 1.0 1.0))
  (`KismetArrayLibrary.Array_Add` (`self.Actors`) _returnvalue)
  (`self.SetActorHiddenInGame` _returnvalue false)
  (`self.K2_AttachToComponent` _returnvalue (`self.Scene`) "None" "KeepRelative" "KeepRelative" "SnapToTarget" false)
  (for (_array_element _array_index) (`self.Actors`)
    (set `self.CurrentExtendMesh` (`.BoxExtent` (`self.GetActorBounds` _returnvalue false)))
    (`self.SetActorScale3D` _array_element (* (`self.GetActorScale3D` _array_element) (`KismetMathLibrary.FMin` (/ (.x (`self.DesiredExtend`)) (.x (`self.CurrentExtendMesh`))) (/ (.y (`self.DesiredExtend`)) (.y (`self.CurrentExtendMesh`))) (/ (.z (`self.DesiredExtend`)) (.z (`self.CurrentExtendMesh`))))))
    (`self.K2_SetActorRelativeLocation` _array_element (`KismetMathLibrary.GreaterGreater_VectorRotator` (`KismetMathLibrary.MakeVector` (`self.RingSize`)) (`KismetMathLibrary.MakeRotator` 0.0 0.0 (* _array_index (/ 360.0 (`KismetMathLibrary.Conv_IntToDouble` (`KismetArrayLibrary.Array_Length` (`self.Actors`))))))) false false)))

(fn `SetNewMesh`
  (params (NewMesh :type "StaticMesh Object Reference")))

(fn `SetWorldScale`
  (params (StaticMesh :type "StaticMeshComponent Object Reference")))

(fn `UserConstructionScript`
  (bind _scenecapturecomponent2d (`self.SceneCaptureComponent2D`))
  (set `self.OriginalScale` (1.0 1.0 1.0))
  (`KismetArrayLibrary.Array_Clear` (`self.StaticMeshes`))
  (`SceneCaptureComponent.ShowOnlyActorComponents` (`self.SceneCaptureComponent2D`) self)
  (`SceneComponent.K2_SetRelativeLocation` (`self.SceneCaptureComponent2D`) (`KismetMathLibrary.MakeVector` (* (`self.RingSize`) 2.5) 0.0 25.0) false false)
  (`SceneComponent.K2_SetWorldRotation` _scenecapturecomponent2d (`KismetMathLibrary.FindLookAtRotation` (`SceneComponent.K2_GetComponentLocation` _scenecapturecomponent2d) (+ (`SceneComponent.K2_GetComponentLocation` (`self.DefaultSceneRoot`)) (0.0 0.0 50.0))) false false)
  (`self.UpdateScale`))