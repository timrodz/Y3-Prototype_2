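; Interactable lamp that the player toggles on and off, with its point light set dark at construction.
; Interact calls its parent, then branches by instigator: the first-person character toggles the light, while an enemy only gets the current on state back.
; Toggling flips intensity between zero and InitialBrightness, updates IsOn and ActiveState, then refreshes the Zone's items.
; The event graph holds only empty events and disconnected FlipFlop and input logic.
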(event `self.Box.OnComponentEndOverlap`
  (params (OverlappedComponent :type "PrimitiveComponent Object Reference") (OtherActor :type "Actor Object Reference") (OtherComp :type "PrimitiveComponent Object Reference") (OtherBodyIndex :type Integer)))

(event `self.Box.OnComponentBeginOverlap`
  (params (OverlappedComponent :type "PrimitiveComponent Object Reference") (OtherActor :type "Actor Object Reference") (OtherComp :type "PrimitiveComponent Object Reference") (OtherBodyIndex :type Integer) (bFromSweep :type Boolean) (SweepResult :type "HitResult Structure (by ref)")))

(event `Key|E`
  (params (Key :type "Key Structure" :default "AnyKey")))

(fn `EnemyInteraction`
  (returns (LightIsOn :type Boolean))
  (return (`self.IsOn`)))

(fn `Interact`
  (params (ActorInstigator :type "Actor Object Reference"))
  (returns (ReturnValue :type Boolean))
  (`parent.Interact` ActorInstigator)
  (cast `/Game/Blueprints/FirstPersonCharacter` ActorInstigator
    (:`then`
      (`self.PlayerInteraction`)
      (return true))
    (:`CastFailed`
      (cast `/Game/Blueprints/Enemy/BP_EnemyCharacter` ActorInstigator)
      (bind _lightison (`self.EnemyInteraction`))
      (return _lightison))))

(fn `PlayerInteraction`
  (bind _returnvalue (* (- 1.0 (`KismetMathLibrary.Conv_BoolToDouble` (`self.IsOn`))) (`self.InitialBrightness`)))
  (`KismetSystemLibrary.PrintString` "Player interaction function")
  (`LightComponent.SetIntensity` (`self.PointLight`) _returnvalue)
  (bind _output_get (set `self.IsOn` (> _returnvalue 0.0)))
  (set `self.ActiveState` _output_get)
  (`Zone.UpdateZoneItems` (`self.Zone`)))

(fn `UserConstructionScript`
  (`LightComponent.SetIntensity` (`self.PointLight`) 0.0))