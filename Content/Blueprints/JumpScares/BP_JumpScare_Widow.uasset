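; Widow jumpscare actor that fires on BeginPlay, hiding the actors in LightsAround and switching on its own spotlight.
; The Flicker timeline serves as a randomly paced timer, with a FlipFlop on Finished alternately showing and hiding the skeletal mesh.
; A counter replays the timeline through FlickerReplay until NumFlickers is reached, then restores the surrounding lights and turns off the spotlight.
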(event `self.ReceiveBeginPlay`
  (`self.Begin Jumpscare`))

(event `Begin Jumpscare`
  (bind _count (`self.Count`))
  (bind _skeletalmesh (`self.SkeletalMesh`))
  (for _array_element (`self.LightsAround`)
    (`self.SetActorHiddenInGame` _array_element true)
    (`SceneComponent.SetVisibility` (`self.SpotLight`) true false)
    (`TimelineComponent.SetPlayRate` (`self.Flicker`) (`KismetMathLibrary.RandomFloatInRange` (`self.RateMin`) (`self.RateMax`)) :!label _label)
    (`Timeline|Flicker` :!via `PlayFromStart`
      (:`Finished`
        (`/Engine/EditorBlueprintResources/StandardMacros.FlipFlop`
          (:`A`
            (`SceneComponent.SetVisibility` _skeletalmesh true false)
            (bind _result (`/Engine/EditorBlueprintResources/StandardMacros.IncrementInt` _count)
              (:`  `
                (if (<= _result (`self.NumFlickers`))
                  (`self.FlickerReplay` :!label _label_2)
                  (else
                    (for _array_element_2 (`self.LightsAround`) :!label _label_3
                      (`self.SetActorHiddenInGame` _array_element_2 false)
                      (`SceneComponent.SetVisibility` (`self.SpotLight`) false false)))))))
          (:`B`
            (`SceneComponent.SetVisibility` _skeletalmesh false false)
            (bind _result_2 (`/Engine/EditorBlueprintResources/StandardMacros.IncrementInt` _count)
              (:`  `
                (if (< _result_2 (`self.NumFlickers`))
                  (goto _label_2)
                  (else
                    (goto _label_3)))))))))))

(event `FlickerReplay`
  (goto _label))

(fn `UserConstructionScript`)