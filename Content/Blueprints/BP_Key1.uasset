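; BP_Key1 is an interactable key pickup that responds differently to the player and to enemies.
; Interact calls its parent, then casts the instigator to choose the player or enemy handler.
; A player pickup flags the key as taken, hides it, plays a sound and updates its Zone's items.
; The hidden actor persists until an enemy interacts, which destroys it and reports whether it was taken.
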(event `self.ReceiveBeginPlay`
  (set `self.HasBeenTaken` false))

(fn `EnemyInteraction`
  (params (Enemy :type "/Game/Blueprints/Enemy/BP_EnemyCharacter Object Reference"))
  (returns (HasBeenTaken :type Boolean))
  (bind _hasbeentaken (`self.HasBeenTaken`))
  (if _hasbeentaken
    (`self.K2_DestroyActor`))
  (return _hasbeentaken))

(fn `Interact`
  (params (Insitigator :type "Actor Object Reference"))
  (returns (Success :type Boolean))
  (`parent.Interact` null)
  (bind _asfirst_person_character (cast `/Game/Blueprints/FirstPersonCharacter` Insitigator)
    (:`then`
      (`self.PlayerInteraction` _asfirst_person_character)
      (return true))
    (:`CastFailed`
      (bind _asbp_enemy_character (cast `/Game/Blueprints/Enemy/BP_EnemyCharacter` Insitigator))
      (bind _hasbeentaken (`self.EnemyInteraction` _asbp_enemy_character))
      (return _hasbeentaken))))

(fn `PlayerInteraction`
  (params (Player :type "/Game/Blueprints/FirstPersonCharacter Object Reference"))
  (set `self.HasBeenTaken` true)
  (`self.SetActorHiddenInGame` true)
  (`GameplayStatics.PlaySound2D` "/Game/Audio/key_pick_up.key_pick_up")
  (`/Game/Blueprints/BP_Zone.UpdateZoneItems` (`self.Zone`))
  (`KismetSystemLibrary.PrintString` "Picked up key"))

(fn `UserConstructionScript`)