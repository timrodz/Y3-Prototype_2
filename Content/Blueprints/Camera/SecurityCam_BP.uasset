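; Security camera actor that sweeps its yaw around its starting angle with a timeline and raises an alarm when it spots the first-person player.
; While the player overlaps it, a per-tick Camera-channel line trace to above the player's origin checks line of sight.
; When the player is seen, the sweep stops, the spotlight turns red and a timer-throttled 2D alarm sound plays; otherwise it sweeps under white light.
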(event `self.ReceiveBeginPlay`
  (set `self.StartingAngle` (.yaw (`self.K2_GetActorRotation`))))

(event `self.ReceiveActorBeginOverlap`
  (params (OtherActor :type "Actor Object Reference"))
  (bind _asfirst_person_character (cast `/Game/Blueprints/FirstPersonCharacter/FirstPersonCharacter` OtherActor))
  (set `self.PlayerRef` _asfirst_person_character)
  (set `self.IsOveralapping` true))

(event `self.ReceiveActorEndOverlap`
  (params (OtherActor :type "Actor Object Reference"))
  (cast `/Game/Blueprints/FirstPersonCharacter/FirstPersonCharacter` OtherActor)
  (set `self.IsOveralapping` false)
  (set `self.PlayerSeen` false))

(event `self.ReceiveTick`
  (params (DeltaSeconds :type "Float (single-precision)"))
  (set `self.AlarmTimer` (+ DeltaSeconds (`self.AlarmTimer`)))
  (`|ExecutionSequence`
    (:`then_0`
      (`self.CheckRayCast`))
    (:`then_1`
      (if (`self.PlayerSeen`)
        (`self.CheckAlarmSound`)
        (`LightComponent.SetLightColor` (`self.SpotLight`) (struct :`R` 1.0 :`A` 1.0) true)
        (bind (_direction _floattrack) (`Timeline|CameraTimeline` :!via `Stop` :!label _label)
          (:`Update`
            (`self.K2_SetActorRotation` (`KismetMathLibrary.MakeRotator` (.roll (`self.K2_GetActorRotation`)) (.pitch (`self.K2_GetActorRotation`)) (+ (`self.StartingAngle`) _floattrack)))))
        (else
          (`LightComponent.SetLightColor` (`self.SpotLight`) (struct :`R` 1.0 :`G` 1.0 :`B` 1.0 :`A` 1.0) true)
          (goto _label))))))

(fn `CheckAlarmSound`
  (if (`self.AlarmSoundPlaying`)
    (if (> (`self.AlarmTimer`) 1.5)
      (set `self.AlarmSoundPlaying` false))
    (else
      (set `self.AlarmSoundPlaying` true)
      (`GameplayStatics.PlaySound2D` "/Game/Audio/Sounds/Bells/Arcade_Bells_Loop.Arcade_Bells_Loop")
      (set `self.AlarmTimer` 0.0))))

(fn `CheckRayCast`
  (if (`self.IsOveralapping`)
    (bind (_outhit _returnvalue) (`KismetSystemLibrary.LineTraceSingle` (`self.K2_GetActorLocation`) (+ (`self.K2_GetActorLocation` (`self.PlayerRef`)) (0.0 0.0 80.0)) "TraceTypeQuery2"))
    (if _returnvalue
      (cast `/Game/Blueprints/FirstPersonCharacter/FirstPersonCharacter` (`.HitActor` (`GameplayStatics.BreakHitResult` _outhit))
        (:`then`
          (set `self.PlayerSeen` true))
        (:`CastFailed`
          (set `self.PlayerSeen` false))))))

(fn `UserConstructionScript`)