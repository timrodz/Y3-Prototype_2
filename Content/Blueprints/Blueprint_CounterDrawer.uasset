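; Interactive counter drawer actor that the player slides open and closed with the E key.
; A box overlap enables and disables the actor's input from the first player controller.
; One timeline offsets the drawer along local Y from InitialLocation, playing forward to open and reversing from the end to close.
; An IsAnimating flag blocks presses mid-motion, and the timeline's finish toggles the open state.
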(event `self.Box.OnComponentBeginOverlap`
  (params (OverlappedComponent :type "PrimitiveComponent Object Reference") (OtherActor :type "Actor Object Reference") (OtherComp :type "PrimitiveComponent Object Reference") (OtherBodyIndex :type Integer) (bFromSweep :type Boolean) (SweepResult :type "HitResult Structure (by ref)"))
  ;[1 1 1] Input Overlap
  (`self.EnableInput` (`GameplayStatics.GetPlayerController` 0)))

(event `self.Box.OnComponentEndOverlap`
  (params (OverlappedComponent :type "PrimitiveComponent Object Reference") (OtherActor :type "Actor Object Reference") (OtherComp :type "PrimitiveComponent Object Reference") (OtherBodyIndex :type Integer))
  ;[1 1 1] Input Overlap
  (`self.DisableInput` (`GameplayStatics.GetPlayerController` 0)))

(event `Key|E`
  (params (Key :type "Key Structure" :default "AnyKey"))
  (:`Pressed`
    (if (not (`self.isAnimating?`))
      (if (`self.isDrawOpen?`)
        (set `self.OpenDraw?` true)
        (set `self.CloseDraw?` false)
        (`self.Close Drawer`)
        (else
          (set `self.CloseDraw?` true)
          (set `self.OpenDraw?` false)
          (`self.Open Drawer`)))
      (set `self.isAnimating?` true))))

(event `Open Drawer`
  (bind (_direction _draweroffset) (`Timeline|DrawerTimeline` :!label _label)
    (:`Update`
      (`SceneComponent.K2_SetRelativeLocation` (`self.Drawer`) (+ (`KismetMathLibrary.MakeVector` 0.0 _draweroffset) (`self.InitialLocation`)) false false))
    (:`Finished`
      (set `self.isAnimating?` false)
      (set `self.isDrawOpen?` (not (`self.isDrawOpen?`))))))

(event `Close Drawer`
  (goto _label :!via `ReverseFromEnd`))

(fn `UserConstructionScript`)