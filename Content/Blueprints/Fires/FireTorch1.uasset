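; FireTorch1 is an interactable torch that the first-person character can pick up and release.
; Interact runs the parent logic, snaps the torch to the character's HeldObjLoc, enables player input and calls EnableTorch, which is empty here.
; Left click then detaches it in place, keeping its world transform.
; Construction makes the Torch component the root, and GetTorch exposes that component.
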(event `self.ReceiveBeginPlay`)

(event `self.ReceiveTick`
  (params (DeltaSeconds :type "Float (single-precision)")))

(event `EnableTorch`)

(event `InputAction|LeftClick`
  (params (Key :type "Key Structure" :default "AnyKey"))
  (:`Pressed`
    (`self.K2_DetachFromActor` "KeepWorld" "KeepWorld" "KeepWorld")))

(fn `GetTorch`
  (returns (Torch :type "StaticMeshComponent Object Reference"))
  (return (`self.Torch`)))

(fn `Interact`
  (params (ActorInstigator :type "Actor Object Reference"))
  (returns (ReturnValue :type Boolean))
  (`parent.Interact` ActorInstigator)
  (bind _asfirst_person_character (cast `/Game/Blueprints/FirstPersonCharacter` ActorInstigator))
  (`self.K2_AttachToComponent` (`/Game/Blueprints/FirstPersonCharacter.HeldObjLoc` _asfirst_person_character) "None" "SnapToTarget" "SnapToTarget" "SnapToTarget")
  (`self.EnableTorch`)
  (`self.EnableInput` (`GameplayStatics.GetPlayerController` _asfirst_person_character))
  (return false))

(fn `UserConstructionScript`
  (set `self.DefaultSceneRoot` (`self.Torch`)))