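; BP_Log is a log pickup that adds to the first-person character's supply of burnable resources.
; Its Interact function casts the instigator to FirstPersonCharacter and looks up the "Burnable" key in that character's ResourceList map.
; An existing count is incremented and the log is destroyed.
; A missing key is added with a count of one, and that branch leaves the log in the world.
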(fn `Interact`
  (params (ActorInstigator :type "Actor Object Reference"))
  (returns (ReturnValue :type Boolean))
  (bind _asfirst_person_character (cast `/Game/Blueprints/FirstPersonCharacter` ActorInstigator))
  (bind _resourcelist (`/Game/Blueprints/FirstPersonCharacter.ResourceList` _asfirst_person_character))
  (bind (_value _returnvalue) (`BlueprintMapLibrary.Map_Find` _resourcelist "Burnable"))
  (if _returnvalue
    (`BlueprintMapLibrary.Map_Add` _resourcelist "Burnable" (+ _value 1))
    (`self.K2_DestroyActor`)
    (return false)
    (else
      (`BlueprintMapLibrary.Map_Add` _resourcelist "Burnable" 1))))

(fn `UserConstructionScript`
  (`parent.UserConstructionScript`))