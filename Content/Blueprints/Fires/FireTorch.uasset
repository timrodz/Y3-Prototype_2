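; Interactable torch that the first-person character picks up and carries, burning for a limited lifetime.
; Interact attaches it to the character's held-object location, spawns the fire emitter with a scaled light, resets the timer and enables input.
; Tick counts down while lit, then destroys the fire component.
; Left click detaches the torch, keeping its world transform.
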(event `self.ReceiveBeginPlay`
  (set `self.TimeLeft` (`self.Fire Lifetime`)))

(event `self.ReceiveTick`
  (params (DeltaSeconds :type "Float (single-precision)"))
  (if (`self.bIsLit`)
    (if (> (`self.TimeLeft`) 0.0)
      (set `self.TimeLeft` (- (`self.TimeLeft`) DeltaSeconds))
      (else
        (`ActorComponent.K2_DestroyComponent` (`self.TorchFire`))
        (set `self.bIsLit` false)))))

(event `EnableTorch`
  (bind _returnvalue (`GameplayStatics.SpawnEmitterAttached` "/Game/StarterContent/Particles/P_Fire1.P_Fire1" (`self.Scene`) "None" (0.0 0.0 0.0) (struct) "SnapToTargetIncludingScale" false))
  (bind _output_get (set `self.TorchFire` _returnvalue))
  (`ParticleSystemComponent.SetVectorParameter` _output_get "LightScale" (2.0 2.0 2.0))
  (set `self.bIsLit` true)
  (set `self.TimeLeft` (`self.Fire Lifetime`)))

(event `InputAction|LeftClick`
  (params (Key :type "Key Structure" :default "AnyKey"))
  (:`Pressed`
    (`self.K2_DetachFromActor` "KeepWorld" "KeepWorld" "KeepWorld")))

(fn `GetTorch`
  (returns (Torch :type "StaticMeshComponent Object Reference"))
  (return (`self.Torch`)))

(fn `Interact`
  (params (ActorInstigator :type "Actor Object Reference"))
  (returns (ReturnValue :type Boolean))
  (`parent.Interact` ActorInstigator)
  (bind _asfirst_person_character (cast `/Game/Blueprints/FirstPersonCharacter` ActorInstigator))
  (`self.K2_AttachToComponent` (`/Game/Blueprints/FirstPersonCharacter.HeldObjLoc` _asfirst_person_character) "None" "SnapToTarget" "SnapToTarget" "SnapToTarget")
  (`self.EnableTorch`)
  (`self.EnableInput` (`GameplayStatics.GetPlayerController` _asfirst_person_character))
  (return false))

(fn `UserConstructionScript`
  (set `self.DefaultSceneRoot` (`self.Torch`)))