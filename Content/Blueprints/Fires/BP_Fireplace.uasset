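; Fireplace actor that a first-person character can feed with burnable resources through an Interact event.
; When the interactor's ResourceList holds a positive "Burnable" count, it increments Stack and scales the particle system's LightScale vector parameter by that Stack.
; The decremented count is written to the misspelled key "Brunable", so the "Burnable" count itself stays unchanged.
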(event `self.Interact`
  (params (Insitigator :type "Actor Object Reference"))
  (bind _asfirst_person_character (cast `/Game/Blueprints/FirstPersonCharacter` Insitigator))
  (bind _resourcelist (`/Game/Blueprints/FirstPersonCharacter.ResourceList` _asfirst_person_character))
  (bind (_value _returnvalue) (`BlueprintMapLibrary.Map_Find` _resourcelist "Burnable"))
  (if _returnvalue
    (if (> _value 0)
      (`BlueprintMapLibrary.Map_Add` _resourcelist "Brunable" (- _value 1))
      (`/Engine/EditorBlueprintResources/StandardMacros.IncrementInt` (`self.Stack`)
        (:`  `
          (`ParticleSystemComponent.SetVectorParameter` (`self.ParticleSystem`) "LightScale" (* (1.0 1.0 1.0) (`self.Stack`))))))))

(fn `UserConstructionScript`)