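; Menu camera controller that makes a Camera actor the first player's view and pans it.
; BeginPlay sets the view target and starts the CameraPan timeline.
; The timeline's Pan track drives the camera's relative yaw with pitch and roll held at zero, and its Finished output restarts it from the start for a continuous loop.
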(event `self.ReceiveBeginPlay`
  (`PlayerController.SetViewTargetWithBlend` (`GameplayStatics.GetPlayerController` 0) (`self.Camera`) 0.0 "VTBlend_Linear" 0.0 false)
  (`TimelineComponent.PlayFromStart` (`self.CameraPan`)))

(fn `UserConstructionScript`)