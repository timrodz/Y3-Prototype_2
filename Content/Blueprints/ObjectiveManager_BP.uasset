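; Objective manager that shows and updates on-screen objectives as the player collects postcards.
; On BeginPlay it creates the objectives widget and binds to the end-inspect event of every BP_DiaryPage in the level.
; A collection counter switches the objective from finding the remaining postcards on the first pickup to finding a way out on the fourth.
; Objective changes play widget fade animations, with a short delay before the final one.
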(event `self.ReceiveBeginPlay`
  (bind _returnvalue (`|CreateWidget` "/Game/Blueprints/Widgets/UMG/Widgets/WidgetBP_Objectives.WidgetBP_Objectives_C" (`GameplayStatics.GetPlayerController` 0)))
  (bind _output_get (set `self.ObjectiveWidget` _returnvalue))
  (`UserWidget.AddToViewport` _output_get 0)
  (bind _outactors (`GameplayStatics.GetAllActorsOfClass` "/Game/Blueprints/Interactables/BP_DiaryPage.BP_DiaryPage_C"))
  (for _array_element _outactors
    (add `/Game/Blueprints/Interactables/Inspectable/BP_Inspectable_Base_BP.Event_OnEndInspect` _array_element (`|CreateDelegate` :!event `On_Collect_PostCard`))
    (set `self.NumberOfPostCardsCollected` 0)))

(event `On_Collect_PostCard`
  (bind _numberofpostcardscollected (`self.NumberOfPostCardsCollected`))
  (if (== _numberofpostcardscollected 0)
    (`self.AddNewObjective` "Find the remaining postcards")
    (elif (== _numberofpostcardscollected 3)
      (`self.Remove`)
      (`KismetSystemLibrary.Delay` 3.0)
      (`self.AddNewObjective` "Find a way out")))
  (bind _result (`/Engine/EditorBlueprintResources/StandardMacros.IncrementInt` (`self.NumberOfPostCardsCollected`))
    (:`  `
      (set `self.NumberOfPostCardsCollected` _result))))

(fn `AddNewObjective`
  (params (NewObjective :type Text))
  (bind _objectivewidget (`self.ObjectiveWidget`))
  (bind _output_get (set `self.CurrentObjective` NewObjective))
  (`/Game/Blueprints/Widgets/UMG/Widgets/WidgetBP_Objectives.SetText` (`self.ObjectiveWidget`) _output_get)
  (`UserWidget.PlayAnimation` _objectivewidget (`/Game/Blueprints/Widgets/UMG/Widgets/WidgetBP_Objectives.FadeInandOut` _objectivewidget) 0.0 1 "Forward" 1.0))

(fn `Remove`
  (bind _objectivewidget (`self.ObjectiveWidget`))
  (`UserWidget.PlayAnimation` _objectivewidget (`/Game/Blueprints/Widgets/UMG/Widgets/WidgetBP_Objectives.FadeOut` _objectivewidget) 0.0 1 "Forward" 1.0))

(fn `UserConstructionScript`)