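; Light prop Blueprint with a point light and optional spotlight that can start on or off, blink, and be switched via TurnON and TurnOFF.
; BeginPlay applies the default state and cancels blinking if off.
; While blinking, Tick accumulates time and uses a random sub-second Delay before ToggleLights, creating irregular flicker.
; Blinking ends with both lights visible after TotalBlinkDuration, or runs indefinitely at -1.
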(event `self.ReceiveBeginPlay`
  (bind _turnedonbydefault_ (`self.TurnedOnByDefault?`))
  (`SceneComponent.SetVisibility` (`self.SpotLight`) _turnedonbydefault_ false)
  (`SceneComponent.SetVisibility` (`self.PointLight`) _turnedonbydefault_ false)
  (if (not _turnedonbydefault_)
    (set `self.IsBlinking?` false)))

(event `self.ReceiveTick`
  (params (DeltaSeconds :type "Float (single-precision)"))
  (if (`self.IsBlinking?`)
    (set `self.CurrentBlinkTime` (+ (`self.CurrentBlinkTime`) DeltaSeconds))
    (`KismetSystemLibrary.Delay` (`KismetMathLibrary.RandomFloat`))
    (`self.ToggleLights`)
    (if (!= (`self.TotalBlinkDuration`) -1.0)
      (if (>= (`self.CurrentBlinkTime`) (`self.TotalBlinkDuration`))
        (set `self.IsBlinking?` false)
        (set `self.CurrentBlinkTime` 0.0)
        (`SceneComponent.SetVisibility` (`self.SpotLight`) true false)
        (`SceneComponent.SetVisibility` (`self.PointLight`) true false)))))

(fn `ToggleLights`
  (`SceneComponent.ToggleVisibility` (`self.PointLight`) false)
  (if (`self.HasSpotlight?`)
    (`SceneComponent.ToggleVisibility` (`self.SpotLight`) false)))

(fn `TurnOFF`
  (`SceneComponent.SetVisibility` (`self.PointLight`) false false)
  (if (`self.HasSpotlight?`)
    (`SceneComponent.SetVisibility` (`self.SpotLight`) false false)))

(fn `TurnON`
  (`SceneComponent.SetVisibility` (`self.PointLight`) true false)
  (if (`self.HasSpotlight?`)
    (`SceneComponent.SetVisibility` (`self.SpotLight`) true false)))

(fn `UserConstructionScript`)