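; Ceiling light prop that can be on, off or blinking, and tells the first-person character whether they stand under it.
; TurnON and TurnOFF set the point and spot lights plus the dynamic bulb material's emissive.
; While blinking, Tick toggles them after random delays with flicker sounds, ending visible after any finite duration.
; A trigger box sets UnderCeilingLight from light visibility on entry and clears it on exit.
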(event `self.ReceiveBeginPlay`
  (if (`self.TurnedOnByDefault?`)
    (`self.TurnON`)
    (else
      (set `self.IsBlinking?` false)
      (`self.TurnOFF`))))

(event `self.ReceiveTick`
  (params (DeltaSeconds :type "Float (single-precision)"))
  (if (`self.IsBlinking?`)
    (set `self.CurrentBlinkTime` (+ (`self.CurrentBlinkTime`) DeltaSeconds))
    (`KismetSystemLibrary.Delay` (`KismetMathLibrary.RandomFloat`))
    (`self.ToggleLights`)
    (if (!= (`self.TotalBlinkDuration`) -1.0)
      (if (>= (`self.CurrentBlinkTime`) (`self.TotalBlinkDuration`))
        (set `self.IsBlinking?` false)
        (set `self.CurrentBlinkTime` 0.0)
        (`SceneComponent.SetVisibility` (`self.SpotLight`) true false)
        (`SceneComponent.SetVisibility` (`self.PointLight`) true false)))))

(event `self.TriggerBox.OnComponentBeginOverlap`
  (params (OverlappedComponent :type "PrimitiveComponent Object Reference") (OtherActor :type "Actor Object Reference") (OtherComp :type "PrimitiveComponent Object Reference") (OtherBodyIndex :type Integer) (bFromSweep :type Boolean) (SweepResult :type "HitResult Structure (by ref)"))
  (bind _asfirst_person_character (cast `/Game/Blueprints/FirstPersonCharacter/FirstPersonCharacter` OtherActor))
  (set `/Game/Blueprints/FirstPersonCharacter/FirstPersonCharacter.UnderCeilingLight` (`SceneComponent.bVisible` (`self.PointLight`)) _asfirst_person_character))

(event `self.TriggerBox.OnComponentEndOverlap`
  (params (OverlappedComponent :type "PrimitiveComponent Object Reference") (OtherActor :type "Actor Object Reference") (OtherComp :type "PrimitiveComponent Object Reference") (OtherBodyIndex :type Integer))
  (bind _asfirst_person_character (cast `/Game/Blueprints/FirstPersonCharacter/FirstPersonCharacter` OtherActor))
  (set `/Game/Blueprints/FirstPersonCharacter/FirstPersonCharacter.UnderCeilingLight` false _asfirst_person_character))

(fn `ToggleLights`
  (bind _lightbulbmaterial (`self.LightBulbMaterial`))
  (`SceneComponent.ToggleVisibility` (`self.PointLight`) false)
  (`SceneComponent.ToggleVisibility` (`self.SpotLight`) false)
  (if (`SceneComponent.bVisible` (`self.SpotLight`))
    (`MaterialInstanceDynamic.SetScalarParameterValue` _lightbulbmaterial "EmissiveIntensity" (`self.EmmisiveIntensityMax`))
    (`GameplayStatics.PlaySoundAtLocation` "/Game/Audio/Sounds/Static/LightFlickerShorter.LightFlickerShorter" (`SceneComponent.K2_GetComponentLocation` (`self.PointLight`)) (struct) 0.25 (`KismetMathLibrary.RandomFloatInRange` 1.0 1.1) 0.0 "/Game/Audio/Attenuation/Phonograph_Attenuation.Phonograph_Attenuation")
    (else
      (`MaterialInstanceDynamic.SetScalarParameterValue` _lightbulbmaterial "EmissiveIntensity" (`self.EmmisiveIntensityMin`)))))

(fn `TurnOFF`
  (`SceneComponent.SetVisibility` (`self.PointLight`) false false)
  (`SceneComponent.SetVisibility` (`self.SpotLight`) false false)
  (`MaterialInstanceDynamic.SetScalarParameterValue` (`self.LightBulbMaterial`) "EmissiveIntensity" (`self.EmmisiveIntensityMin`)))

(fn `TurnON`
  (`SceneComponent.SetVisibility` (`self.PointLight`) true false)
  (`SceneComponent.SetVisibility` (`self.SpotLight`) true false)
  (`MaterialInstanceDynamic.SetScalarParameterValue` (`self.LightBulbMaterial`) "EmissiveIntensity" (`self.EmmisiveIntensityMax`)))

(fn `UserConstructionScript`
  (bind _returnvalue (`PrimitiveComponent.CreateDynamicMaterialInstance` (`self.StaticMesh`) 0 "/Game/Assets/Furniture/LightBulber.LightBulber"))
  (set `self.LightBulbMaterial` _returnvalue)
  (if (`self.TurnedOnByDefault?`)
    (`self.TurnON`)
    (else
      (`self.TurnOFF`))))