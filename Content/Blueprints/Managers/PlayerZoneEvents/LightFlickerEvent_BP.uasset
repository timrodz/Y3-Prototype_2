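; Zone event manager Blueprint that flickers a set of lights, starting on BeginPlay or through TriggerEve.
; Construction script caches each light's original intensity by index.
; A timeline lerps intensities down to a randomly divided, near-dark fraction, while a FlipFlop alternates forward and reverse playback, randomizing play rate before reversing.
; Timeline completion re-enters the cycle indefinitely; the random loop count is set but never checked.
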(event `self.ReceiveBeginPlay`
  (if (`self.TriggerOnPlay`)
    (`self.TriggerEve`)
    (`KismetSystemLibrary.Delay` 5.3)))

(event `TriggerIt`
  (set `self.NumLoops` (`KismetMathLibrary.RandomIntegerInRange` 0 (`self.RandLoopRange`)))
  (bind _output_get (set `self.RandomPercent` (`KismetMathLibrary.RandomFloatInRange` 80.0 100.0) :!label _label))
  (`/Engine/EditorBlueprintResources/StandardMacros.FlipFlop`
    (:`A`
      (bind (_direction _newtrack_1) (`Timeline|Timeline_0` :!via `PlayFromStart` :!label _label_2)
        (:`Update`
          (for (_array_element _array_index) (`self.Lights`)
            (bind _value (`BlueprintMapLibrary.Map_Find` (`self.OriginalIntensities`) _array_index))
            (`LightComponent.SetIntensity` (`Light.LightComponent` _array_element) (`KismetMathLibrary.Lerp` _value (/ _value _output_get) _newtrack_1))))
        (:`Finished`
          (goto _label))))
    (:`B`
      (`TimelineComponent.SetPlayRate` (`self.Timeline_0`) (`KismetMathLibrary.RandomFloatInRange` 0.5 5.0))
      (goto _label_2 :!via `ReverseFromEnd`))))

(fn `TriggerEve`
  (`self.TriggerIt`))

(fn `UserConstructionScript`
  (`parent.UserConstructionScript`)
  (for (_array_element _array_index) (`self.Lights`)
    (bind _aslight (cast `Light` _array_element))
    (`BlueprintMapLibrary.Map_Add` (`self.OriginalIntensities`) _array_index (`LightComponentBase.Intensity` (`Light.LightComponent` _aslight)))))