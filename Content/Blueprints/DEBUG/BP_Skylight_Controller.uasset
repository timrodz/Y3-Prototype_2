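; Debug actor that adjusts a referenced skylight's intensity at runtime from the keyboard.
; On BeginPlay it enables input from the first player controller.
; Page Up and Page Down then raise or lower the Skylight's light component intensity in small fixed steps, with no clamping.
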(event `self.ReceiveBeginPlay`
  (`self.EnableInput` (`GameplayStatics.GetPlayerController` 0)))

(event `Key|PageUp`
  (params (Key :type "Key Structure" :default "AnyKey"))
  (bind _lightcomponent (`SkyLight.LightComponent` (`self.Skylight`)))
  (:`Pressed`
    (`SkyLightComponent.SetIntensity` _lightcomponent (+ (`LightComponentBase.Intensity` _lightcomponent) 0.1))))

(event `Key|PageDown`
  (params (Key :type "Key Structure" :default "AnyKey"))
  (bind _lightcomponent (`SkyLight.LightComponent` (`self.Skylight`)))
  (:`Pressed`
    (`SkyLightComponent.SetIntensity` _lightcomponent (- (`LightComponentBase.Intensity` _lightcomponent) 0.1))))

(fn `UserConstructionScript`)