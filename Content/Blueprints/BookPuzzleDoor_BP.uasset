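; Puzzle door Blueprint that unlocks and opens once all of its linked door lights are on.
; Interacting runs the parent behaviour, then checks every valid entry in DoorLights while the puzzle is unsolved.
; On success it calls UnlockAndOpen, destroys the lights, disables collision on the linked book meshes and plays a bell sound at the door.
; A PuzzleComplete flag, reset on BeginPlay, keeps the solve from repeating.
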(event `self.ReceiveBeginPlay`
  (`parent.ReceiveBeginPlay`)
  (set `self.PuzzleComplete` false))

(fn `CheckLightsAreOn`
  (if (not (`self.PuzzleComplete`))
    (set `self.AllOn` true)
    (for _array_element (`self.DoorLights`)
      (`/Engine/EditorBlueprintResources/StandardMacros.IsValid` _array_element
        (:`Is Valid`
          (if (not (`/Game/Blueprints/DoorLight_BP.IsOn` _array_element))
            (set `self.AllOn` false)))))
    (if (`self.AllOn`)
      (`self.UnlockAndOpen`)
      (for _array_element_2 (`self.DoorLights`)
        (`self.K2_DestroyActor` _array_element_2))
      (for _array_element_3 (`self.Books`)
        (`PrimitiveComponent.SetCollisionEnabled` (`/Game/Blueprints/BookButton_BP.BookMesh` _array_element_3) "NoCollision"))
      (set `self.PuzzleComplete` true)
      (`GameplayStatics.PlaySoundAtLocation` "/Game/Audio/Sounds/Bells/Bell_Door_Camel.Bell_Door_Camel" (`self.K2_GetActorLocation`)))))

(fn `Interact`
  (params (ActorInstigator :type "Actor Object Reference"))
  (returns (ReturnValue :type Boolean))
  (bind _returnvalue (`parent.Interact` null))
  (`self.CheckLightsAreOn`)
  (return _returnvalue))

(fn `UserConstructionScript`
  (`parent.UserConstructionScript`))