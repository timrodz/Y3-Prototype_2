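; Interactable padlock puzzle controller that opens a chained doorway once the padlock is solved.
; It creates the padlock widget at BeginPlay and shows it on interact with UI-only input and a visible cursor, unless already solved.
; The widget's exit callback reports the result: success adds a subtitle, plays a sound, destroys the chains and unlocks the door after a delay.
; Either outcome then closes the widget and restores game input.
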(event `self.ReceiveBeginPlay`
  (bind _returnvalue (`|CreateWidget` "/Game/Blueprints/Widgets/Padlock_WidgetBP.Padlock_WidgetBP_C" (`GameplayStatics.GetPlayerController` 0)))
  (bind _output_get (set `self.Padlock_Widget` _returnvalue))
  (`/Engine/EditorBlueprintResources/StandardMacros.IsValid` _output_get
    (:`Is Valid`
      (add `/Game/Blueprints/Widgets/Padlock_WidgetBP.Exit_Button_OnClick` _output_get (delegate `OnExitButtonClick`)))))

(event `OnExitButtonClick`
  (params (`SolvedPuzzle?` :type Boolean))
  (if `SolvedPuzzle?`
    (bind _asfirst_person_character (cast `/Game/Blueprints/FirstPersonCharacter/FirstPersonCharacter` (`GameplayStatics.GetPlayerPawn` 0)))
    (`/Game/Blueprints/FirstPersonCharacter/FirstPersonCharacter.AddSubtitle` _asfirst_person_character "I got it!" 3.0 0.5)
    (`GameplayStatics.PlaySound2D` "/Game/Audio/Sounds/Horror/dark_slam.dark_slam")
    (`self.K2_DestroyActor` (`self.Chains`))
    (`KismetSystemLibrary.Delay` 2.5)
    (`/Game/Blueprints/Interactables/Blueprint_Doorway.UnlockDoor` (`self.Doorway`))
    (set `self.Solved` true))
  (`self.DisableWidget`))

(fn `DisableWidget`
  (bind _returnvalue (`GameplayStatics.GetPlayerController` 0))
  ;[1 1 1] Remove the widget from the viewport and set input mode to Game Only
  (`Widget.RemoveFromParent` (`self.Padlock_Widget`))
  (`WidgetBlueprintLibrary.SetInputMode_GameOnly` _returnvalue)
  (set `PlayerController.bShowMouseCursor` false _returnvalue)
  (set `self.IsPadlockVisible?` false))

(fn `EnableWidget`
  (bind _returnvalue (`GameplayStatics.GetPlayerController` 0))
  (bind _padlock_widget (`self.Padlock_Widget`))
  ;[1 1 1] Add the widget to the viewport and set the input mode to UI only
  (if (not (`self.Solved`))
    (`UserWidget.AddToViewport` _padlock_widget 0)
    (`WidgetBlueprintLibrary.SetInputMode_UIOnlyEx` _returnvalue null "LockOnCapture")
    (set `PlayerController.bShowMouseCursor` true _returnvalue)
    (set `self.IsPadlockVisible?` true)
    (`Widget.SetKeyboardFocus` _padlock_widget)))

(fn `Interact`
  (params (ActorInstigator :type "Actor Object Reference"))
  (returns (ReturnValue :type Boolean))
  (bind _returnvalue (`parent.Interact` null))
  (`self.EnableWidget`)
  (return _returnvalue))

(fn `UserConstructionScript`)