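; Controller for a lever puzzle that traps a gate shut on trigger overlap and reopens it once solved.
; Entering the initial box lowers the gate by timeline, destroys the box and reveals the levers, which start at zero scale.
; Lever interactions update a state array compared against the solution, currently all false despite a comment about random values.
; A separate check lever raises the gate if solved, with sounds marking each stage.
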(event `self.ReceiveBeginPlay`
  (bind _solved_lever_states (`self.Solved Lever States`))
  ;[1 1 1] Initialise the solved states to random values (All true for testing)
  (for (_ _array_index) _solved_lever_states
    (`KismetArrayLibrary.Array_Set` _solved_lever_states _array_index)
    (for _array_element (`self.Lever Array`)
      (add `/Game/Blueprints/Interactables/BP_Lever.Interacted` _array_element (delegate `Listen_Interact`))
      (`self.SetActorScale3D` _array_element (0.0 0.0 0.0)))
    (add `/Game/Blueprints/Interactables/BP_Lever.Interacted` (`self.Lever to Check Solution`) (delegate `Listen_Interact`))
    (set `self.Start Position` (`self.K2_GetActorLocation` (`self.Gate`)))))

(event `Listen_Interact`
  (params (Instigator :type "/Game/Blueprints/Interactables/BP_Lever Object Reference") (Value :type Boolean))
  ;[1 0.3482 0.0546] Player interacts with gate opening lever
  (if (== Instigator (`self.Lever to Check Solution`))
    ;[1 0.8987 0.3411] Puzzle is solved and door is opened
    (if (`self.Solved`)
      (set `self.Phase` 2)
      (`GameplayStatics.PlaySound2D` null) ; Play GATE_OPENING sound
      (bind (_direction _gate_lerp) (`Timeline|Open Gate`)
        (:`Update`
          (`self.K2_SetActorLocation` (`self.Gate`) (+ (`KismetMathLibrary.MakeVector` 0.0 0.0 (* _gate_lerp 300.0)) (`self.Start Position`)) false false))
        (:`Finished`
          (`GameplayStatics.PlaySound2D` null) ; Play GATE_OPENED sound
        )))
    (else
      (`KismetArrayLibrary.Array_Set` (`self.Current Lever States`) (`KismetArrayLibrary.Array_Find` (`self.Lever Array`) Instigator) Value)
      (bind _solved (`self.CheckSolution`))
      (bind _output_get (set `self.Solved` _solved))
      (if _output_get
        (`GameplayStatics.PlaySound2D` null) ; Play GATE_UNLOCKED sound
      ))))

(event `self.Initial_State_Box.OnComponentBeginOverlap`
  (params (OverlappedComponent :type "PrimitiveComponent Object Reference") (OtherActor :type "Actor Object Reference") (OtherComp :type "PrimitiveComponent Object Reference") (OtherBodyIndex :type Integer) (bFromSweep :type Boolean) (SweepResult :type "HitResult Structure (by ref)"))
  ;[0.4144 1 0.2316] Interacting with initial state box
  (`GameplayStatics.PlaySound2D` null) ; Play GATE_CLOSING sound
  (bind (_direction _gate_lerp) (`Timeline|Gate Close`)
    (:`Update`
      (`self.K2_SetActorLocation` (`self.Gate`) (+ (`KismetMathLibrary.MakeVector` 0.0 0.0 (* _gate_lerp -300.0)) (`self.Start Position`)) false false))
    (:`Finished`
      (set `self.Start Position` (`self.K2_GetActorLocation` (`self.Gate`)))
      (set `self.Phase` 1)
      (`GameplayStatics.PlaySound2D` null) ; Play GATE_CLOSED sound
      (`ActorComponent.K2_DestroyComponent` (`self.Initial_State_Box`))
      (for _array_element (`self.Lever Array`)
        (`self.SetActorScale3D` _array_element (1.0 1.0 1.0))))))

(fn `CheckSolution`
  (returns (Solved :type Boolean))
  (locals (NewLocalVar_0 :type "Vector Structure" :default (0.0 0.0 0.0)))
  (set `self.Is Puzzle Solved` true)
  (for (_array_element _array_index) (`self.Current Lever States`)
    ;[1 1 1] If one lever does not share the state of the solved one - Return
    (if (not (== _array_element (`|GetArrayItem` (`self.Solved Lever States`) _array_index)))
      (`KismetSystemLibrary.PrintString` "Not Solved")
      (return false)))
  (if (`self.Is Puzzle Solved`)
    (`KismetSystemLibrary.PrintString` "Solved")
    (return true)))

(fn `UserConstructionScript`)