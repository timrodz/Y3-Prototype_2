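; Door controller trigger volume that locks or unlocks a referenced door when the first-person character enters its box.
; ShouldUnlock picks the action.
; Locking turns off the door's subtitles, optionally plays a knock sound, then briefly speeds up the door's timeline around an OpenDoorMutex call before restoring speed and clearing the mutex.
; DestroyAfterAction makes the trigger destroy itself afterwards.
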(event `self.Box.OnComponentBeginOverlap`
  (params (OverlappedComponent :type "PrimitiveComponent Object Reference") (OtherActor :type "Actor Object Reference") (OtherComp :type "PrimitiveComponent Object Reference") (OtherBodyIndex :type Integer) (bFromSweep :type Boolean) (SweepResult :type "HitResult Structure (by ref)"))
  (bind _doortolock (`self.DoorToLock`))
  (bind _dooropentimeline (`/Game/Blueprints/Interactables/Blueprint_Doorway.DoorOpenTimeline` _doortolock))
  ;[1 0.481 0.8139] Box collider overlap event
  (cast `/Game/Blueprints/FirstPersonCharacter/FirstPersonCharacter` OtherActor)
  (if (`self.ShouldUnlock?`)
    (`self.UnlockDoor`)
    (else
      (`self.LockDoor`)
      (`TimelineComponent.SetPlayRate` _dooropentimeline 3.5)
      (`/Game/Blueprints/Interactables/Blueprint_Doorway.OpenDoor_Mutex` _doortolock)
      (`KismetSystemLibrary.Delay` 0.75)
      (`TimelineComponent.SetPlayRate` _dooropentimeline 1.0)
      (set `/Game/Blueprints/Interactables/Blueprint_Doorway.OpenMutex` false _doortolock)))
  (if (`self.DestroyAfterAction`)
    (`KismetSystemLibrary.PrintString` "Hello")
    (`self.K2_DestroyActor`)))

(fn `LockDoor`
  (bind _doortolock (`self.DoorToLock`))
  (set `/Game/Blueprints/Interactables/Blueprint_Doorway.ShowSubtitles?` false _doortolock)
  (`/Game/Blueprints/Interactables/Blueprint_Doorway.LockDoor` _doortolock)
  (if (`self.PlayKnockSound?`)
    (`GameplayStatics.PlaySoundAtLocation` null)))

(fn `UnlockDoor`
  (`/Game/Blueprints/Interactables/Blueprint_Doorway.UnlockDoor` (`self.DoorToLock`))
  (if (`self.DestroyAfterAction`)
    (`self.K2_DestroyActor`)))

(fn `UserConstructionScript`)