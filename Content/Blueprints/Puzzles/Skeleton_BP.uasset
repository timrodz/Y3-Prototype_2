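; Skeleton assembly puzzle that serves as the game's finale, where the player returns bones to free the widow.
; Overlapping items are matched to hidden bone slots by the first four characters of their object names, then released, destroyed and shown on the skeleton.
; Completing it resets the objective, fades in the widow, raises her on a timeline, removes the enemy and shows the end-of-game widget.
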(event `self.ReceiveTick`
  (params (DeltaSeconds :type "Float (single-precision)")))

(event `self.ReceiveBeginPlay`
  (bind _childactorarray (`self.ChildActorArray`))
  (bind _finalwidow (`self.FinalWidow`))
  (bind _staticmesh (`/Game/Blueprints/FinalWIdow_BP.StaticMesh` _finalwidow))
  (`KismetArrayLibrary.Array_Add` _childactorarray (`self.Head`))
  (`KismetArrayLibrary.Array_Add` _childactorarray (`self.RightFoot`))
  (`KismetArrayLibrary.Array_Add` _childactorarray (`self.LeftArm`))
  (`KismetArrayLibrary.Array_Add` _childactorarray (`self.Sternum`))
  (set `self.TotalNumberOfItems` (`KismetArrayLibrary.Array_Length` (`self.ChildActorArray`)))
  (for _array_element (`self.ChildActorArray`)
    (`SceneComponent.SetVisibility` (`SceneComponent.GetChildComponent` _array_element 0) false false)
    (`/Engine/EditorBlueprintResources/StandardMacros.IsValid` (`self.FinalWidow`)
      (:`Is Valid`
        (set `self.Widow Original Location` (`self.K2_GetActorLocation` _finalwidow))
        (`ActorComponent.SetActive` _staticmesh false false)
        (`SceneComponent.SetVisibility` _staticmesh false false))
      (:`Is Not Valid`
        (`KismetSystemLibrary.PrintString` "No Widow assigned to skeleton!")))))

(event `self.ReceiveActorBeginOverlap`
  (params (OtherActor :type "Actor Object Reference"))
  (bind _finalwidow (`self.FinalWidow`))
  (bind _staticmesh (`/Game/Blueprints/FinalWIdow_BP.StaticMesh` _finalwidow))
  (for _array_element (`self.ChildActorArray`)
    (if (`KismetStringLibrary.EqualEqual_StrStr` (`KismetStringLibrary.GetSubstring` (`KismetSystemLibrary.GetObjectName` _array_element) 0 4) (`KismetStringLibrary.GetSubstring` (`KismetSystemLibrary.GetObjectName` OtherActor) 0 4))
      (`SceneComponent.SetVisibility` (`SceneComponent.GetChildComponent` _array_element 0) true false)
      (bind _asfirst_person_character (cast `/Game/Blueprints/FirstPersonCharacter/FirstPersonCharacter` (`GameplayStatics.GetPlayerPawn` 0)))
      (`Grabber.Release` (`self.GetComponentByClass` _asfirst_person_character "/Game/Blueprints/Components/BP_GrabberComponent.BP_GrabberComponent_C"))
      (`self.K2_DestroyActor` OtherActor)
      (`GameplayStatics.PlaySound2D` "/Game/Audio/Sounds/Impacts/Bone_Crack.Bone_Crack" 0.4)
      (bind _result (`/Engine/EditorBlueprintResources/StandardMacros.IncrementInt` (`self.CurrentItemsAdded`))
        (:`  `
          (set `self.CurrentItemsAdded` _result)
          (if (== (`self.TotalNumberOfItems`) (`self.CurrentItemsAdded`))
            (bind _asfirst_person_character_2 (cast `/Game/Blueprints/FirstPersonCharacter/FirstPersonCharacter` (`GameplayStatics.GetPlayerPawn` 0))
              (:`then`
                (`/Game/Blueprints/FirstPersonCharacter/FirstPersonCharacter.ResetCurrentObjective` _asfirst_person_character_2))
              (:`CastFailed`
                _))
            (`/Engine/EditorBlueprintResources/StandardMacros.IsValid` _finalwidow
              (:`Is Valid`
                (`ActorComponent.SetActive` _staticmesh true false)
                (`SceneComponent.SetVisibility` _staticmesh true false)
                (`/Game/Blueprints/FinalWIdow_BP.FadeIn` _finalwidow)
                (`self.Widow Event`)
                (`/Game/Blueprints/Enemy/BP_EnemyCharacter.FadeOut` (`self.Enemy`))
                (bind _asfirst_person_character_3 (cast `/Game/Blueprints/FirstPersonCharacter/FirstPersonCharacter` (`GameplayStatics.GetPlayerPawn` 0)))
                (`/Game/Blueprints/FirstPersonCharacter/FirstPersonCharacter.AddSubtitle` _asfirst_person_character_3 "That's the last one. My work here is done." 3.0 1.0 1.0)
                (`KismetSystemLibrary.Delay` 2.0)
                (`self.K2_DestroyActor` (`self.Enemy`))
                (`KismetSystemLibrary.Delay` 8.0)
                (bind _returnvalue (`|CreateWidget` "/Game/Blueprints/Widgets/EndOfGame_WidgetBP.EndOfGame_WidgetBP_C"))
                (`/Game/Blueprints/Widgets/EndOfGame_WidgetBP.Show` _returnvalue))
              (:`Is Not Valid`
                (`KismetSystemLibrary.PrintString` "Skeleton Widow Not Valid")))
            (elif (== (- (`self.TotalNumberOfItems`) 1) (`self.CurrentItemsAdded`))
              (bind _asfirst_person_character_4 (cast `/Game/Blueprints/FirstPersonCharacter/FirstPersonCharacter` (`GameplayStatics.GetPlayerPawn` 0)))
              (`/Game/Blueprints/FirstPersonCharacter/FirstPersonCharacter.AddSubtitle` _asfirst_person_character_4 "One more bone to add. Then she can finally be free." 5.0 1.0 0.0))))))))

(event `Widow Event`
  (bind _finalwidow (`self.FinalWidow`))
  (`/Engine/EditorBlueprintResources/StandardMacros.IsValid` _finalwidow
    (:`Is Valid`
      (`GameplayStatics.PlaySoundAtLocation` "/Game/Audio/Sounds/Horror/supernatural.supernatural" (`self.K2_GetActorLocation` _finalwidow))
      (bind (_direction _float) (`Timeline|Widow Rise` :!via `PlayFromStart`)
        (:`Update`
          (`self.K2_SetActorLocation` (`self.FinalWidow`) (`KismetMathLibrary.MakeVector` (.x (`self.Widow Original Location`)) (.y (`self.Widow Original Location`)) (+ _float (.z (`self.Widow Original Location`)))) false false))
        (:`Finished`
          (`self.K2_DestroyActor` (`self.FinalWidow`)))))))

(fn `UserConstructionScript`)