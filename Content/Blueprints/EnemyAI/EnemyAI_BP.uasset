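; EnemyAI_BP is the AI controller for Enemy_BP, driving guard points and noise response through a behavior tree.
; On BeginPlay it runs the tree and copies the pawn's four guard points into the Blackboard, leaving their order to the tree.
; When PawnSensing hears a noise, the location is stored on the pawn and written to the TargetLocation key.
; An older random-wander loop and a debug print remain disconnected.
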(event `self.ReceiveBeginPlay`
  (`self.RunBehaviorTree` (`self.BehaviourTree`))
  ;[1 1 1] For setting 4 target points for the enemy - sequence order can be changed in behaviour tree
  (bind _asenemy_bp (cast `/Game/Blueprints/EnemyAI/Enemy_BP` (`self.K2_GetPawn`)))
  (`BlackboardComponent.SetValueAsObject` (`AIBlueprintHelperLibrary.GetBlackboard` self) "GuardPoint1" (`/Game/Blueprints/EnemyAI/Enemy_BP.GuardPoint1` _asenemy_bp))
  (`BlackboardComponent.SetValueAsObject` (`AIBlueprintHelperLibrary.GetBlackboard` self) "GuardPoint2" (`/Game/Blueprints/EnemyAI/Enemy_BP.GuardPoint2` _asenemy_bp))
  (`BlackboardComponent.SetValueAsObject` (`AIBlueprintHelperLibrary.GetBlackboard` self) "GuardPoint3" (`/Game/Blueprints/EnemyAI/Enemy_BP.GuardPoint3` _asenemy_bp))
  (`BlackboardComponent.SetValueAsObject` (`AIBlueprintHelperLibrary.GetBlackboard` self) "GuardPoint4" (`/Game/Blueprints/EnemyAI/Enemy_BP.GuardPoint4` _asenemy_bp)))

(event `self.PawnSensing.OnHearNoise`
  (params (Instigator :type "Pawn Object Reference") (Location :type "Vector Structure (by ref)") (Volume :type "Float (single-precision)"))
  (bind _asenemy_bp (cast `/Game/Blueprints/EnemyAI/Enemy_BP` (`self.K2_GetPawn`)))
  (bind _output_get (set `/Game/Blueprints/EnemyAI/Enemy_BP.CurrentTargetLocation` Location _asenemy_bp))
  (`BlackboardComponent.SetValueAsVector` (`AIBlueprintHelperLibrary.GetBlackboard` self) "TargetLocation" _output_get))

(fn `UserConstructionScript`)