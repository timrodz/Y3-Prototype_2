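; Key_BP is a key pickup the player collects by pressing E while standing in its trigger.
; The KeyTrigger overlap stores the FirstPersonCharacter reference and enables the actor's input, and leaving the trigger disables it.
; Pressing E destroys the key, sets HasKey on the stored player and plays a pickup sound.
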(event `self.KeyTrigger.OnComponentBeginOverlap`
  (params (OverlappedComponent :type "PrimitiveComponent Object Reference") (OtherActor :type "Actor Object Reference") (OtherComp :type "PrimitiveComponent Object Reference") (OtherBodyIndex :type Integer) (bFromSweep :type Boolean) (SweepResult :type "HitResult Structure (by ref)"))
  ;[1 1 1] Event Overlap - Enable Disable Input
  (bind _asfirst_person_character (cast `/Game/Blueprints/FirstPersonCharacter` OtherActor))
  (set `self.PlayerRef` _asfirst_person_character)
  (`self.EnableInput` (`GameplayStatics.GetPlayerController` 0)))

(event `self.KeyTrigger.OnComponentEndOverlap`
  (params (OverlappedComponent :type "PrimitiveComponent Object Reference") (OtherActor :type "Actor Object Reference") (OtherComp :type "PrimitiveComponent Object Reference") (OtherBodyIndex :type Integer))
  ;[1 1 1] Event Overlap - Enable Disable Input
  (cast `/Game/Blueprints/FirstPersonCharacter` OtherActor)
  (`self.DisableInput` (`GameplayStatics.GetPlayerController` 0)))

(event `Key|E`
  (params (Key :type "Key Structure" :default "AnyKey"))
  ;[1 1 1] Event Interaction - Open Close Door
  (:`Pressed`
    (`self.K2_DestroyActor`)
    (set `/Game/Blueprints/FirstPersonCharacter.hasKey` true (`self.PlayerRef`))
    (`GameplayStatics.PlaySound2D` "/Game/Audio/key_pick_up.key_pick_up")))

(fn `UserConstructionScript`)