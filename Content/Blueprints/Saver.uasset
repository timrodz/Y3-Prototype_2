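; Saver is an actor Blueprint that writes and reads a list of actors through a CheckPointSystem SaveGame in a debug slot.
; Save creates the save object, copies ActorsToSave into it and writes it to the slot.
; Load reads the slot and loops over the saved array, but the loop body is empty, so nothing is restored.
; The default events are unused.
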(fn `Load`
  (bind _returnvalue (`GameplayStatics.LoadGameFromSlot` "DebugSave"))
  (bind _output_get (set `self.SaveGameInstance` _returnvalue))
  (bind _ascheck_point_system (cast `/Game/Blueprints/CheckPointSystem` _output_get))
  (for (_ _array_index) (`/Game/Blueprints/CheckPointSystem.ActorsToSave` _ascheck_point_system)
    _))

(fn `Save`
  (bind _returnvalue (`GameplayStatics.CreateSaveGameObject` "/Game/Blueprints/CheckPointSystem.CheckPointSystem_C"))
  (bind _output_get (set `self.SaveGameInstance` _returnvalue))
  (bind _ascheck_point_system (cast `/Game/Blueprints/CheckPointSystem` _output_get))
  (set `/Game/Blueprints/CheckPointSystem.ActorsToSave` (`self.ActorsToSave`) _ascheck_point_system)
  (`GameplayStatics.SaveGameToSlot` _ascheck_point_system "DebugSave"))

(fn `UserConstructionScript`)