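; A one-shot trigger actor that moves an existing enemy, presumably the first one, to a spawn location when overlapped.
; On any actor overlap, it validates the enemy and location references, teleports the enemy to the location's transform without sweep, then destroys itself.
; An invalid reference only prints an error and leaves the trigger in place.
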(event `self.ReceiveActorBeginOverlap`
  (params (OtherActor :type "Actor Object Reference"))
  (`/Engine/EditorBlueprintResources/StandardMacros.IsValid` (`self.EnemyRef`)
    (:`Is Valid`
      (`/Engine/EditorBlueprintResources/StandardMacros.IsValid` (`self.EnemySpawnLocation`)
        (:`Is Valid`
          (`self.K2_SetActorTransform` (`self.EnemyRef`) (`self.GetTransform` (`self.EnemySpawnLocation`)) false true)
          (`self.K2_DestroyActor`))
        (:`Is Not Valid`
          (`KismetSystemLibrary.PrintString` "Enemy spawn location not valid"))))
    (:`Is Not Valid`
      (`KismetSystemLibrary.PrintString` "Enemy ref in spawner not valid!"))))

(fn `UserConstructionScript`)