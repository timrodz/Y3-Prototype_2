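; Enemy character that stalks first-person players, raising their awareness value when they are within range and lowering it when they hold their breath or move away.
; Each tick drives that awareness per player, scaled by delta time.
; Overlaps track the current zone and let the enemy switch off lamps or interact with keys, completing zone events and rechecking for active ones.
; Pawn sensing by sight or sound runs a target check and plays a scream with a cooldown.
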(event `self.ReceiveBeginPlay`
  (`self.GetAllPlayers`))

(event `self.ReceiveTick`
  (params (DeltaSeconds :type "Float (single-precision)"))
  (set `self.Delta` DeltaSeconds)
  (for _array_element (`self.Players`)
    (if (<= (`KismetMathLibrary.VSize` (- (`self.K2_GetActorLocation`) (`self.K2_GetActorLocation` _array_element))) 600.0)
      (if (`BreatheMechanic.IsHoldingBreath` (`/Game/Blueprints/FirstPersonCharacter.BP_BreatheMechanic` _array_element))
        (`self.DecreaseAwarenessOfPlayer` _array_element :!label _label)
        (else
          (`self.IncreaseAwarenessOfPlayer` _array_element)))
      (else
        (goto _label)))))

(event `self.ReceiveActorBeginOverlap`
  (params (OtherActor :type "Actor Object Reference"))
  (bind _currentzone (`self.CurrentZone`))
  (bind _asbp_zone (cast `/Game/Blueprints/BP_Zone` OtherActor)
    (:`then`
      (set `self.CurrentZone` _asbp_zone)
      (`KismetSystemLibrary.Delay` 0.2 :!label _label_2)
      (`self.CheckForActiveZoneEvents`)
      (`KismetSystemLibrary.PrintString` "Hello"))
    (:`CastFailed`
      (bind _asbp_lamp (cast `/Game/Blueprints/BP_Lamp` OtherActor)
        (:`then`
          (bind _returnvalue (`TrackedObject.Interact` _asbp_lamp self))
          (if _returnvalue
            (`self.TurnOffLamp` _asbp_lamp)
            (`/Engine/EditorBlueprintResources/StandardMacros.IsValid` _currentzone :!label _label_3
              (:`Is Valid`
                (`self.SetZoneEventComplete`)
                (`Zone.UpdateZoneItems` _currentzone)
                (goto _label_2)))))
        (:`CastFailed`
          (bind _asbp_key (cast `/Game/Blueprints/BP_Key` OtherActor))
          (bind _returnvalue_2 (`TrackedObject.Interact` _asbp_key self))
          (if _returnvalue_2
            (`KismetSystemLibrary.PrintString` "Key is missing....")
            (`KismetSystemLibrary.Delay` 3.0)
            (goto _label_3)))))))

(event `self.PawnSensingComp.OnSeePawn`
  (params (Pawn :type "Pawn Object Reference"))
  (bind _returnvalue (`self.HasSeenTarget` :!label _label_4))
  (if _returnvalue
    (if (`self.ShouldPlaySenseNoise`)
      (`GameplayStatics.PlaySound2D` "/Game/Audio/Scream2.Scream2")
      (set `self.ShouldPlaySenseNoise` false)
      (`KismetSystemLibrary.Delay` 10.0)
      (set `self.ShouldPlaySenseNoise` true))))

(event `self.PawnSensingComp.OnHearNoise`
  (params (Instigator :type "Pawn Object Reference") (Location :type "Vector Structure (by ref)") (Volume :type "Float (single-precision)"))
  (goto _label_4))

(fn `DecreaseAwarenessOfPlayer`
  (params (Player :type "/Game/Blueprints/FirstPersonCharacter Object Reference"))
  (`/Game/Blueprints/FirstPersonCharacter.DecreaseAwareness` Player (* (`self.Delta`) 10.0)))

(fn `GetAllPlayers`
  (bind _outactors (`GameplayStatics.GetAllActorsOfClass` "/Game/Blueprints/FirstPersonCharacter.FirstPersonCharacter_C"))
  (set `self.Players` _outactors))

(fn `IncreaseAwarenessOfPlayer`
  (params (Player :type "/Game/Blueprints/FirstPersonCharacter Object Reference"))
  (`/Game/Blueprints/FirstPersonCharacter.IncreaseAwareness` Player (* (`self.Delta`) 10.0) self))

(fn `SetDebugRenderOutline`
  (bind _mesh (`self.Mesh`))
  (if (`self.DebugMode`)
    (`PrimitiveComponent.SetRenderCustomDepth` _mesh true)
    (`PrimitiveComponent.SetCustomDepthStencilValue` _mesh 255)))

(fn `TurnOffLamp`
  (params (Lamp :type "/Game/Blueprints/BP_Lamp Object Reference"))
  (`LightComponent.SetIntensity` (`/Game/Blueprints/BP_Lamp.PointLight` Lamp) 0.0)
  (set `/Game/Blueprints/BP_Lamp.IsOn` false Lamp))

(fn `UserConstructionScript`
  (`self.GetAllPlayers`))