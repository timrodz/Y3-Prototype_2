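; Trigger actor that relocates the enemy to a random spawn location when the player overlaps it.
; BeginPlay caches a BP_EnemyCharacter; on overlap, it teleports only if that enemy is patrolling and far from the trigger.
; AI wandering pauses briefly after the teleport.
; The coin-flip compare gates nothing, and the validity check and destination use separate random picks.
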(event `self.ReceiveBeginPlay`
  (bind _outactors (`GameplayStatics.GetAllActorsOfClass` "/Game/Blueprints/Enemy/BP_EnemyCharacter.BP_EnemyCharacter_C"))
  (for _array_element _outactors
    (set `self.EnemyRef` _array_element)))

(event `self.ReceiveActorBeginOverlap`
  (params (OtherActor :type "Actor Object Reference"))
  (bind _enemyref (`self.EnemyRef`))
  (bind _output (`|GetArrayItem` (`self.Spawn_Locations`) (`KismetMathLibrary.RandomIntegerInRange` 0 (- (`KismetArrayLibrary.Array_Length` (`self.Spawn_Locations`)) 1))))
  (cast `/Game/Blueprints/FirstPersonCharacter/FirstPersonCharacter` OtherActor)
  (`/Engine/EditorBlueprintResources/StandardMacros.IsValid` _enemyref
    (:`Is Valid`
      (bind _returnvalue (`EnemyCharacter.IsEnemyPatrolling` _enemyref))
      (if (and (> (`self.GetDistanceTo` _enemyref) 2500.0) _returnvalue)
        (`/Engine/EditorBlueprintResources/StandardMacros.CompareInt` (`KismetMathLibrary.RandomIntegerInRange` 0 1)
          (:`>`
            _)
          (:`==`
            _)
          (:`<`
            _))
        (`/Engine/EditorBlueprintResources/StandardMacros.IsValid` _output
          (:`Is Valid`
            (`self.K2_TeleportTo` :`self` (`self.EnemyRef`) :`DestLocation` (`self.K2_GetActorLocation` _output))
            (`self.SetWanderFalse`)
            (`KismetSystemLibrary.Delay` 0.5)
            (`self.SetWanderTrue`)))))))

(fn `SetWanderFalse`
  (bind _asbp_enemy_aicontroller (cast `/Game/Blueprints/Enemy/BP_EnemyAIController` (`AIBlueprintHelperLibrary.GetAIController` (`self.EnemyRef`))))
  (`EnemyAIController.SetShouldWander` _asbp_enemy_aicontroller false))

(fn `SetWanderTrue`
  (bind _asbp_enemy_aicontroller (cast `/Game/Blueprints/Enemy/BP_EnemyAIController` (`AIBlueprintHelperLibrary.GetAIController` (`self.EnemyRef`))))
  (`EnemyAIController.SetShouldWander` _asbp_enemy_aicontroller true))

(fn `UserConstructionScript`)