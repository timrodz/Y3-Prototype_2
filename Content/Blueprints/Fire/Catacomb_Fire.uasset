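; Catacomb fire actor that can start hidden and plays flame sounds when enabled or disabled.
; On BeginPlay it hides itself in game if HideBeginPlay is set.
; Enable unhides it and plays a quieter, lower-pitched whoosh with Catacombes attenuation at its location.
; Disable plays a poof at its location but also sets the actor visible rather than hiding it.
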(event `self.ReceiveBeginPlay`
  (if (`self.bHideBeginPlay`)
    (`self.SetActorHiddenInGame` true)))

(event `Enable`
  (`self.SetActorHiddenInGame` false)
  (`GameplayStatics.PlaySoundAtLocation` "/Game/Audio/Sounds/Fire/Flame_Whoosh_By.Flame_Whoosh_By" (`self.K2_GetActorLocation`) (struct) 0.2 0.8 0.1 "/Game/Audio/Attenuation/Catacombes.Catacombes"))

(event `Disable`
  (`self.SetActorHiddenInGame` false)
  (`GameplayStatics.PlaySoundAtLocation` "/Game/Audio/Sounds/Fire/Flame_Poof_Whoosh.Flame_Poof_Whoosh" (`self.K2_GetActorLocation`)))

(fn `UserConstructionScript`)