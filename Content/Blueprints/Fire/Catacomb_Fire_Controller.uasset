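; Catacomb fire controller that lights an array of fires in sequence after a start delay.
; A timeline, with play rate set by a speed multiplier, fires an event track that enables the next two fires through a running counter.
; The timeline restarts itself from that event until the counter reaches the end of the array.
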(event `self.ReceiveBeginPlay`
  (bind _fires (`self.Fires`))
  (bind _count (`self.Count`))
  (`KismetSystemLibrary.Delay` (`self.StartDelay`))
  (`TimelineComponent.SetPlayRate` (`self.Event`) (`self.SpeedMultiplier`))
  (`Timeline|Event` :!via `PlayFromStart` :!label _label
    (:`NewTrack_0`
      (if (< _count (`KismetArrayLibrary.Array_Length` _fires))
        (`/Game/Blueprints/Fire/Catacomb_Fire.Enable` (`|GetArrayItem` _fires _count))
        (bind _result (`/Engine/EditorBlueprintResources/StandardMacros.IncrementInt` _count)
          (:`  `
            (if (< (`self.Count`) (`KismetArrayLibrary.Array_Length` (`self.Fires`)))
              (`/Game/Blueprints/Fire/Catacomb_Fire.Enable` (`|GetArrayItem` (`self.Fires`) _result))
              (`/Engine/EditorBlueprintResources/StandardMacros.IncrementInt` (`self.Count`)
                (:`  `
                  (if (< (`self.Count`) (`KismetArrayLibrary.Array_Length` (`self.Fires`)))
                    (goto _label :!via `PlayFromStart`)))))))))))

(fn `UserConstructionScript`)