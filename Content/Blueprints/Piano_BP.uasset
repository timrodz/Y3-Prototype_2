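; Piano Blueprint, an interactable actor that plays a single low piano note when used.
; It overrides Interact to call the parent implementation, play the sound at its own location, and return the parent's result.
; GetInteractLocation returns the world position of its InteractLocation component, and the event graph holds no active logic.
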(fn `GetInteractLocation`
  (returns (ReturnValue :type "Vector Structure"))
  (`parent.GetInteractLocation`)
  (return (`SceneComponent.K2_GetComponentLocation` (`self.InteractLocation`))))

(fn `Interact`
  (params (ActorInstigator :type "Actor Object Reference"))
  (returns (ReturnValue :type Boolean))
  (bind _returnvalue (`parent.Interact` null))
  (`GameplayStatics.PlaySoundAtLocation` "/Game/Audio/Sounds/Piano/PianoSingleNoteLow.PianoSingleNoteLow" (`self.K2_GetActorLocation`))
  (return _returnvalue))

(fn `UserConstructionScript`
  (`parent.UserConstructionScript`))