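; BookButton_BP is an interactable book that acts as a button in a book puzzle door.
; Interacting plays a latch sound and runs the BookMovement timeline, which animates the book's roll to tilt it.
; If its DoorLight is valid, it turns that light on and tells the BookPuzzleDoor_BP, cached at BeginPlay via GetAllActorsOfClass, to check whether the lights are on.
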(event `self.ReceiveBeginPlay`
  (set `self.OriginalLocation` (`self.K2_GetActorLocation`))
  (bind _outactors (`GameplayStatics.GetAllActorsOfClass` "/Game/Blueprints/BookPuzzleDoor_BP.BookPuzzleDoor_BP_C"))
  (for _array_element _outactors
    (set `self.BookPuzzleDoor` _array_element)))

(event `PushBook`
  (`GameplayStatics.PlaySoundAtLocation` "/Game/Audio/Sounds/Buttons/Latches/Latch_Slide_3.Latch_Slide_3" (`self.K2_GetActorLocation`))
  (bind (_direction _rotation) (`Timeline|BookMovement` :!via `PlayFromStart`)
    (:`Update`
      (`self.K2_SetActorRotation` (`KismetMathLibrary.MakeRotator` _rotation (.pitch (`self.K2_GetActorRotation`)) (.yaw (`self.K2_GetActorRotation`)))))))

(fn `Interact`
  (params (ActorInstigator :type "Actor Object Reference"))
  (returns (ReturnValue :type Boolean))
  (bind _doorlight (`self.DoorLight`))
  (bind _returnvalue (`parent.Interact` null))
  (`self.PushBook`)
  (`/Engine/EditorBlueprintResources/StandardMacros.IsValid` _doorlight
    (:`Is Valid`
      (`/Game/Blueprints/DoorLight_BP.Turn On` _doorlight)
      (`/Game/Blueprints/BookPuzzleDoor_BP.CheckLightsAreOn` (`self.BookPuzzleDoor`))
      (return _returnvalue))))

(fn `UserConstructionScript`
  (`parent.UserConstructionScript`))