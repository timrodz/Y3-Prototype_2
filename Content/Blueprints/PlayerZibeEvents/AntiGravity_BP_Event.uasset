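; Anti-gravity event volume that makes nearby physics props float when the first-person character enters its box.
; Overlapping simulating static mesh actors lose gravity, receive an upward acceleration in a random cone, and join FloatingMeshes.
; A delayed reset restores gravity on every stored mesh after a few seconds; the array is never cleared.
; Debug print strings remain in the overlap and float logic.
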(event `self.Box.OnComponentBeginOverlap`
  (params (OverlappedComponent :type "PrimitiveComponent Object Reference") (OtherActor :type "Actor Object Reference") (OtherComp :type "PrimitiveComponent Object Reference") (OtherBodyIndex :type Integer) (bFromSweep :type Boolean) (SweepResult :type "HitResult Structure (by ref)"))
  (cast `/Game/Blueprints/FirstPersonCharacter` OtherActor)
  (`self.MakeItemsFloat` (`self.Box`))
  (`KismetSystemLibrary.PrintString` "213"))

(event `Delayed_Reset`
  (params (Duration :type "Float (double-precision)"))
  (`KismetSystemLibrary.Delay` Duration)
  (for _array_element (`self.FloatingMeshes`)
    (`PrimitiveComponent.SetEnableGravity` (`StaticMeshActor.StaticMeshComponent` _array_element) true)))

(fn `MakeItemsFloat`
  (params (BoxCollision :type "BoxComponent Object Reference"))
  (for _array_element (`PrimitiveComponent.GetOverlappingActors` BoxCollision "/Script/Engine.StaticMeshActor")
    (`KismetSystemLibrary.PrintString` "1")
    (bind _asstatic_mesh_actor (cast `StaticMeshActor` _array_element :!pure true))
    (if (`SceneComponent.IsAnySimulatingPhysics` (`StaticMeshActor.StaticMeshComponent` _asstatic_mesh_actor))
      (`KismetArrayLibrary.Array_Add` (`self.FloatingMeshes`) _asstatic_mesh_actor)
      (bind _staticmeshcomponent (`StaticMeshActor.StaticMeshComponent` _asstatic_mesh_actor))
      (`PrimitiveComponent.SetEnableGravity` _staticmeshcomponent false)
      (`PrimitiveComponent.AddForce` _staticmeshcomponent (* (`KismetMathLibrary.RandomUnitVectorInCone` (0.0 0.0 1.0) 40.0) 1000.0) "None" true)
      (`self.Delayed_Reset` 5.0))))

(fn `UserConstructionScript`
  (`parent.UserConstructionScript`))