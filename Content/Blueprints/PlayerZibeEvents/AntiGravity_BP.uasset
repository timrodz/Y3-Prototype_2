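; AntiGravity_BP is an anti-gravity effect that makes physics props inside a box volume float.
; MakeItemsFloat takes a box collision and finds overlapping StaticMeshActors that simulate physics.
; It records each in FloatingMeshes, disables its gravity and applies one small upward force as an acceleration change.
; The event graph holds only disabled stubs, and nothing here calls the function or restores gravity.
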(fn `MakeItemsFloat`
  (params (BoxCollision :type "BoxComponent Object Reference"))
  (for _array_element (`PrimitiveComponent.GetOverlappingActors` BoxCollision "/Script/Engine.StaticMeshActor")
    (bind _asstatic_mesh_actor (cast `StaticMeshActor` _array_element :!pure true))
    (if (`SceneComponent.IsAnySimulatingPhysics` (`StaticMeshActor.StaticMeshComponent` _asstatic_mesh_actor))
      (`KismetArrayLibrary.Array_Add` (`self.FloatingMeshes`) _asstatic_mesh_actor)
      (bind _staticmeshcomponent (`StaticMeshActor.StaticMeshComponent` _asstatic_mesh_actor))
      (`PrimitiveComponent.SetEnableGravity` _staticmeshcomponent false)
      (`PrimitiveComponent.AddForce` _staticmeshcomponent (0.0 0.0 10.0) "None" true))))

(fn `UserConstructionScript`
  (`parent.UserConstructionScript`))