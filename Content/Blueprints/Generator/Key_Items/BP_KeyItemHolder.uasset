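; BP_KeyItemHolder is a generator Blueprint that references a key item and visualizes that link with a debug line.
; Both the Construction Script and Tick draw a long-lived line from the holder's location to KeyItemReference's location, colored by DebugColor.
; It contains no other active logic, and neither graph checks that the reference is valid before drawing.
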(event `self.ReceiveTick`
  (params (DeltaSeconds :type "Float (single-precision)"))
  (`KismetSystemLibrary.DrawDebugLine` (`self.K2_GetActorLocation`) (`self.K2_GetActorLocation` (`self.KeyItem_Reference`)) (`KismetMathLibrary.Conv_VectorToLinearColor` (`self.Debug_Color`)) 125.0 1.0))

(fn `UserConstructionScript`
  (`KismetSystemLibrary.DrawDebugLine` (`self.K2_GetActorLocation`) (`self.K2_GetActorLocation` (`self.KeyItem_Reference`)) (`KismetMathLibrary.Conv_VectorToLinearColor` (`self.Debug_Color`)) 125.0 1.0))