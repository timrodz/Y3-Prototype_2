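; Vignette controller that fades a post-process effect in and out with the player's awareness level.
; BeginPlay caches the FirstPersonCharacter, and Tick sets the PostProcess blend weight to its AwarenessOf value divided by 100.
; A breath-mechanic air ratio is left unconnected, and GetPlayerValues is empty apart from unreachable nodes for setting vignette and chromatic aberration.
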(event `self.ReceiveBeginPlay`
  (set `self.Player` (cast `/Game/Blueprints/FirstPersonCharacter/FirstPersonCharacter` (`GameplayStatics.GetPlayerPawn` 0) :!pure true)))

(event `self.ReceiveTick`
  (params (DeltaSeconds :type "Float (single-precision)"))
  (set `PostProcessComponent.BlendWeight` (/ (`/Game/Blueprints/FirstPersonCharacter/FirstPersonCharacter.AwarenessOf` (`self.Player`)) 100.0) (`self.PostProcess`)))

(fn `GetPlayerValues`)

(fn `UserConstructionScript`)