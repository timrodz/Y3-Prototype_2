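; Actor that drives heartbeat audio and a post-process effect from the first-person player's AwarenessOf value.
; Each tick it sets the post-process blend weight proportional to awareness.
; When neither heartbeat sound is playing, it starts the normal or high one by awareness threshold; otherwise it scales both pitches with awareness.
; GetPlayerValues is empty, with unconnected leftover post-process setup.
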(event `self.ReceiveBeginPlay`
  (set `self.Player` (cast `/Game/Blueprints/FirstPersonCharacter/FirstPersonCharacter` (`GameplayStatics.GetPlayerPawn` 0) :!pure true)))

(event `self.ReceiveTick`
  (params (DeltaSeconds :type "Float (single-precision)"))
  (bind _awarenessof (`/Game/Blueprints/FirstPersonCharacter/FirstPersonCharacter.AwarenessOf` (`self.Player`)))
  (`self.VignetteEffect`)
  (if (and (not (`AudioComponent.IsPlaying` (`self.HeatBeat`))) (not (`AudioComponent.IsPlaying` (`self.HeatBeat_High`))))
    (if (>= _awarenessof 75.0)
      (`AudioComponent.Play` (`self.HeatBeat_High`) 0.0)
      (elif (>= _awarenessof 1.0)
        (`AudioComponent.Play` (`self.HeatBeat`) 0.0)))
    (else
      (`AudioComponent.SetPitchMultiplier` (`self.HeatBeat`) (+ 0.8 (* (/ _awarenessof 75.0) 0.25)))
      (`AudioComponent.SetPitchMultiplier` (`self.HeatBeat_High`) (/ _awarenessof 100.0)))))

(fn `GetPlayerValues`)

(fn `UserConstructionScript`)

(fn `VignetteEffect`
  (set `PostProcessComponent.BlendWeight` (/ (`/Game/Blueprints/FirstPersonCharacter/FirstPersonCharacter.AwarenessOf` (`self.Player`)) 100.0) (`self.PostProcess`)))