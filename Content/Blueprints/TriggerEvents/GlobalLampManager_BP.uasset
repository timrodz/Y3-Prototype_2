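; Manager actor that flickers level Lights and BP_Lamp_B lamps to simulate power fluctuations and outages.
; It caches base intensities of lights gathered from its Box at BeginPlay or level-wide in the construction script.
; FluctuatePower loops a randomly paced timeline dimming and restoring lights, skipping switched-off lamps.
; FluctuatePowerOff flickers similarly, then can fade to near black with a zero-volume power-down sound, leaving RunningTimeline set, blocking further fluctuations.
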(event `self.ReceiveBeginPlay`
  (if (`self.bAutoFetchBox`)
    (for _array_element (`PrimitiveComponent.GetOverlappingActors` (`self.Box`) "/Script/Engine.Light")
      (bind _aslight (cast `Light` _array_element))
      (bind _returnvalue (`KismetArrayLibrary.Array_Add` (`self.Lights`) _aslight))
      (`BlueprintMapLibrary.Map_Add` (`self.Light_Intensities`) _returnvalue (`LightComponentBase.Intensity` (`Light.LightComponent` _aslight))))
    (for _array_element_2 (`PrimitiveComponent.GetOverlappingActors` (`self.Box`) "/Game/Blueprints/Interactables/BP_Lamp_B.BP_Lamp_B_C")
      (bind _asbp_lamp_b (cast `/Game/Blueprints/Interactables/BP_Lamp_B` _array_element_2))
      (bind _returnvalue_2 (`KismetArrayLibrary.Array_Add` (`self.Lamps`) _asbp_lamp_b))
      (`BlueprintMapLibrary.Map_Add` (`self.Lamp_Intensities`) _returnvalue_2 (`LightComponentBase.Intensity` (`/Game/Blueprints/Interactables/BP_Lamp_B.PointLight` _asbp_lamp_b))))))

(event `FluctuatePower`
  (if (not (`self.RunningTimeline`))
    (set `self.RunningTimeline` true)
    (set `self.NumLoops` (`KismetMathLibrary.RandomIntegerInRange` (`self.MinLoopRange`) (`self.RandLoopRange`)))
    (bind _output_get (set `self.RandomPercent` (`KismetMathLibrary.RandomFloatInRange` 1.0 10.0) :!label _label))
    (`/Engine/EditorBlueprintResources/StandardMacros.FlipFlop`
      (:`A`
        (`TimelineComponent.SetPlayRate` (`self.Timeline_0`) (`KismetMathLibrary.RandomFloatInRange` 1.0 5.0))
        (bind (_direction _newtrack_1) (`Timeline|Timeline_0` :!label _label_2)
          (:`Update`
            (for (_array_element _array_index) (`self.Lights`)
              (bind _value (`BlueprintMapLibrary.Map_Find` (`self.Light_Intensities`) _array_index))
              (`LightComponent.SetIntensity` (`Light.LightComponent` _array_element) (`KismetMathLibrary.Lerp` _value (/ _value _output_get) _newtrack_1)))
            (for (_array_element_2 _array_index_2) (`self.Lamps`)
              (if (`/Game/Blueprints/Interactables/BP_Lamp_B.IsOn` _array_element_2)
                (bind _value_2 (`BlueprintMapLibrary.Map_Find` (`self.Lamp_Intensities`) _array_index_2))
                (`LightComponent.SetIntensity` (`/Game/Blueprints/Interactables/BP_Lamp_B.PointLight` _array_element_2) (`KismetMathLibrary.Lerp` _value_2 (/ _value_2 _output_get) _newtrack_1)))))
          (:`Finished`
            (`/Engine/EditorBlueprintResources/StandardMacros.FlipFlop`
              (:`A`
                (goto _label_2 :!via `ReverseFromEnd`))
              (:`B`
                (bind _result (`/Engine/EditorBlueprintResources/StandardMacros.DecrementInt` (`self.NumLoops`))
                  (:`  `
                    (if (> _result 0)
                      (goto _label)
                      (else
                        (set `self.RunningTimeline` false))))))))))
      (:`B`
        (`TimelineComponent.SetPlayRate` (`self.Timeline_0`) (`KismetMathLibrary.RandomFloatInRange` 1.0 5.0))
        (goto _label_2)))))

(event `FluctuatePowerOff`
  (if (not (`self.RunningTimeline`))
    (set `self.RunningTimeline` true)
    (set `self.NumLoops` (`KismetMathLibrary.RandomIntegerInRange` (`self.MinLoopRange`) (`self.RandLoopRange`)))
    (bind _output_get (set `self.RandomPercent` (`KismetMathLibrary.RandomFloatInRange` 0.1 1.0) :!label _label_3))
    (`TimelineComponent.SetPlayRate` (`self.Timeline_1`) (`KismetMathLibrary.RandomFloatInRange` 3.0 8.0) :!label _label_4)
    (bind (_direction _newtrack_1) (`Timeline|Timeline_1` :!label _label_5)
      (:`Update`
        (for (_array_element _array_index) (`self.Lights`)
          (bind _value (`BlueprintMapLibrary.Map_Find` (`self.Light_Intensities`) _array_index))
          (`LightComponent.SetIntensity` (`Light.LightComponent` _array_element) (`KismetMathLibrary.Lerp` _value (* _value _output_get) _newtrack_1)))
        (for (_array_element_2 _array_index_2) (`self.Lamps`)
          (if (`/Game/Blueprints/Interactables/BP_Lamp_B.IsOn` _array_element_2)
            (bind _value_2 (`BlueprintMapLibrary.Map_Find` (`self.Lamp_Intensities`) _array_index_2))
            (`LightComponent.SetIntensity` (`/Game/Blueprints/Interactables/BP_Lamp_B.PointLight` _array_element_2) (`KismetMathLibrary.Lerp` _value_2 (* _value_2 _output_get) _newtrack_1)))))
      (:`Finished`
        (if (not (`KismetMathLibrary.NearlyEqual_FloatFloat` (stale _output_get_2) 1e-06))
          (`/Engine/EditorBlueprintResources/StandardMacros.FlipFlop`
            (:`A`
              (goto _label_5 :!via `ReverseFromEnd`))
            (:`B`
              (bind _result (`/Engine/EditorBlueprintResources/StandardMacros.DecrementInt` (`self.NumLoops`))
                (:`  `
                  (if (> _result 1)
                    (goto _label_3)
                    (elif (> (`self.NumLoops`) 0)
                      (`GameplayStatics.PlaySoundAtLocation` (`self.EnginePowerDown`) (`KismetMathLibrary.MakeVector` 262.0 384.0 37.0) (struct) 0.0 0.8 0.0 "/Game/Audio/Attenuation/Engine_Atten.Engine_Atten")
                      (bind _output_get_2 (set `self.RandomPercent` 1e-06))
                      (goto _label_4)
                      (else
                        (set `self.RunningTimeline` false)))))))))))))

(fn `ClearArrays`
  (`KismetArrayLibrary.Array_Clear` (`self.Lights`))
  (`KismetArrayLibrary.Array_Clear` (`self.Lamps`)))

(fn `GetLampClasses`
  (bind _outactors (`GameplayStatics.GetAllActorsOfClass` "/Game/Blueprints/Interactables/BP_Lamp_B.BP_Lamp_B_C"))
  (bind _output_get (set `self.Lamps` _outactors))
  (for (_array_element _array_index) _output_get
    (`BlueprintMapLibrary.Map_Add` (`self.Lamp_Intensities`) _array_index (`LightComponentBase.Intensity` (`/Game/Blueprints/Interactables/BP_Lamp_B.PointLight` _array_element)))))

(fn `GetLightClasses`
  (bind _outactors (`GameplayStatics.GetAllActorsOfClass` "/Script/Engine.Light"))
  (bind _output_get (set `self.Lights` _outactors))
  (for (_array_element _array_index) _output_get
    (`BlueprintMapLibrary.Map_Add` (`self.Light_Intensities`) _array_index (`LightComponentBase.Intensity` (`Light.LightComponent` _array_element)))))

(fn `UserConstructionScript`
  (if (`self.bFetchAll`)
    (set `self.bAutoFetchBox` false)
    (`self.ClearArrays`)
    (`self.GetLightClasses`)
    (`self.GetLampClasses`)))