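; Trigger volume actor that switches blinking on or off for a set of lights when the first-person player walks into it.
; On Box overlap by a FirstPersonCharacter, it sets IsBlinking on every entry in the Lights array according to the MakeLightsBlink flag.
; An optional DestroyAfterBeginOverlap flag destroys the trigger afterwards, making it one-shot.
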(event `self.Box.OnComponentBeginOverlap`
  (params (OverlappedComponent :type "PrimitiveComponent Object Reference") (OtherActor :type "Actor Object Reference") (OtherComp :type "PrimitiveComponent Object Reference") (OtherBodyIndex :type Integer) (bFromSweep :type Boolean) (SweepResult :type "HitResult Structure (by ref)"))
  (bind _lights (`self.Lights`))
  (cast `/Game/Blueprints/FirstPersonCharacter/FirstPersonCharacter` OtherActor)
  (if (`self.MakeLightsBlink?`)
    (for _array_element _lights
      (set `/Game/Blueprints/Props/Ceiling_Light_BP.IsBlinking?` true _array_element))
    (else
      (for _array_element_2 _lights
        (set `/Game/Blueprints/Props/Ceiling_Light_BP.IsBlinking?` false _array_element_2))))
  (if (`self.DestroyAfterBeginOverlap?`)
    (`self.K2_DestroyActor`)))

(fn `UserConstructionScript`)