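; Hallway trigger-event Blueprint that hides a doorway behind a wall until the Polaroid's end-inspect event reveals it.
; Shortly after BeginPlay, one static mesh becomes a wall plane at the blocker location and scale.
; When inspection ends, that same mesh swaps to a door frame and moves to the door transform.
; Editor-named functions toggle the open and closed states.
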(event `self.ReceiveBeginPlay`
  (bind _staticmesh (`self.StaticMesh`))
  (add `/Game/Blueprints/Interactables/Inspectable/BP_Inspectable_Base_BP.Event_OnEndInspect` (`self.Polaroid`) (delegate `OpenHiddenDoor`))
  (`KismetSystemLibrary.Delay` 0.2)
  (`StaticMeshComponent.SetStaticMesh` _staticmesh "/Game/NewHouse/Architecture/Plane_Wall.Plane_Wall")
  (`SceneComponent.K2_SetWorldLocation` _staticmesh (`self.BlockerLocation`) false false)
  (`SceneComponent.SetWorldScale3D` _staticmesh (`self.BlockerScale`)))

(event `OpenHiddenDoor`
  (bind _staticmesh (`self.StaticMesh`))
  (`StaticMeshComponent.SetStaticMesh` _staticmesh "/Game/NewHouse/Architecture/Door_Frame.Door_Frame")
  (`SceneComponent.SetWorldScale3D` _staticmesh (`self.DoorScale`))
  (`SceneComponent.K2_SetWorldLocation` _staticmesh (`self.DoorLocation`) false true))

(fn `Editor_CloseHiddenDoor`
  (bind _staticmesh (`self.StaticMesh`))
  (`StaticMeshComponent.SetStaticMesh` _staticmesh "/Game/NewHouse/Architecture/Plane_Wall.Plane_Wall")
  (`SceneComponent.K2_SetWorldLocation` _staticmesh (`self.BlockerLocation`) false false)
  (`SceneComponent.SetWorldScale3D` _staticmesh (`self.BlockerScale`)))

(fn `Editor_OpenHiddenDoor`
  (`self.OpenHiddenDoor`))

(fn `UserConstructionScript`)