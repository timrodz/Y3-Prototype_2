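; LerpEvent_BP is a level event actor that sets static mesh props adrift in zero gravity, then eases them back to their starting transforms.
; On BeginPlay it gathers movable StaticMeshActors inside its Box, saves their transforms, and enables gravity-free physics with a random push.
; The Revert event stops simulation, records the drifted transforms, and plays a slowed timeline that lerps each actor back to its original transform.
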(event `self.ReceiveBeginPlay`
  (bind _actors (`self.Actors`))
  (bind _overlappingactors (`PrimitiveComponent.GetOverlappingActors` (`self.Box`) "/Script/Engine.StaticMeshActor"))
  (`KismetSystemLibrary.PrintString` (`KismetStringLibrary.Conv_IntToString` (`KismetArrayLibrary.Array_Length` _overlappingactors)))
  (for _array_element _overlappingactors
    (bind _asstatic_mesh_actor (cast `StaticMeshActor` _array_element :!pure true))
    (if (`|EnumEquality` (`SceneComponent.Mobility` (`self.K2_GetRootComponent` _asstatic_mesh_actor)) "Movable")
      (`KismetArrayLibrary.Array_AddUnique` _actors _asstatic_mesh_actor)))
  (for _array_element_2 _actors
    (bind (_returnvalue_location _returnvalue_rotation _returnvalue_scale) (`KismetMathLibrary.BreakTransform` (`self.GetTransform` _array_element_2)))
    (`KismetArrayLibrary.Array_Add` (`self.OriginalTransforms`) (`KismetMathLibrary.MakeTransform` _returnvalue_location _returnvalue_rotation _returnvalue_scale))
    (bind _asstatic_mesh_actor_2 (cast `StaticMeshActor` _array_element_2 :!pure true))
    (`PrimitiveComponent.SetSimulatePhysics` (`StaticMeshActor.StaticMeshComponent` _asstatic_mesh_actor_2) true)
    (bind _staticmeshcomponent (`StaticMeshActor.StaticMeshComponent` _asstatic_mesh_actor_2))
    (`PrimitiveComponent.SetMassOverrideInKg` _staticmeshcomponent "None" 2.5 true)
    (`PrimitiveComponent.SetAngularDamping` _staticmeshcomponent 0.25)
    (`PrimitiveComponent.SetLinearDamping` _staticmeshcomponent 0.1)
    (`PrimitiveComponent.SetEnableGravity` (`StaticMeshActor.StaticMeshComponent` _asstatic_mesh_actor_2) false)
    (`PrimitiveComponent.AddForce` (`StaticMeshActor.StaticMeshComponent` _asstatic_mesh_actor_2) (* (`KismetMathLibrary.RandomUnitVector`) 10000.0) "None" false)))

(event `Revert`
  (for _array_element (`self.Actors`)
    (`PrimitiveComponent.SetSimulatePhysics` (`StaticMeshActor.StaticMeshComponent` _array_element) false)
    (bind (_returnvalue_location _returnvalue_rotation _returnvalue_scale) (`KismetMathLibrary.BreakTransform` (`self.GetTransform` _array_element)))
    (`KismetArrayLibrary.Array_Add` (`self.FinalTransforms`) (`KismetMathLibrary.MakeTransform` _returnvalue_location _returnvalue_rotation _returnvalue_scale))
    (`TimelineComponent.SetPlayRate` (`self.Lerp`) 0.25)
    (bind (_direction _newtrack_0) (`Timeline|Lerp`)
      (:`Update`
        (for (_array_element_2 _array_index) (`self.Actors`)
          (`self.K2_SetActorTransform` _array_element_2 (`KismetMathLibrary.TLerp` (`|GetArrayItem` (`self.FinalTransforms`) _array_index) (`|GetArrayItem` (`self.OriginalTransforms`) _array_index) _newtrack_0) false false))))))

(fn `UserConstructionScript`
  (`parent.UserConstructionScript`))