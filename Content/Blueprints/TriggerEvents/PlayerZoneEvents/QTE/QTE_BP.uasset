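; Quick-time-event trigger zone that launches a physics mesh and changes global time dilation when the first-person character enters its box.
; On overlap it pushes the mesh along an arrow, optionally tags it Highlightable, and restores normal time after a short dilation-affected delay.
; Flags block re-entry during the event and limit it to one firing unless Retriggerable.
; Empty OnBeginTrigger and OnEndTrigger functions serve as hooks around the event.
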(event `self.ReceiveBeginPlay`)

(event `self.Box.OnComponentBeginOverlap`
  (params (OverlappedComponent :type "PrimitiveComponent Object Reference") (OtherActor :type "Actor Object Reference") (OtherComp :type "PrimitiveComponent Object Reference") (OtherBodyIndex :type Integer) (bFromSweep :type Boolean) (SweepResult :type "HitResult Structure (by ref)"))
  (cast `/Game/Blueprints/FirstPersonCharacter/FirstPersonCharacter` OtherActor)
  (if (`self.Triggered`)
    (if (`self.Retriggerable`)
      (if (not (`self.InTriggered`)) :!label _label
        (set `self.InTriggered` true)
        (set `self.Triggered` true)
        (`self.SimulateAndAddForce`)
        (`self.OnBeginTrigger`)
        (`GameplayStatics.SetGlobalTimeDilation` (`self.TimeDilation`))
        (`KismetSystemLibrary.Delay` 0.5)
        (`self.onEndTrigger`)
        (`GameplayStatics.SetGlobalTimeDilation` 1.0)
        (set `self.InTriggered` false)))
    (else
      (goto _label))))

(fn `OnBeginTrigger`)

(fn `onEndTrigger`)

(fn `SimulateAndAddForce`
  (bind _mesh (`self.Mesh`))
  (`PrimitiveComponent.SetSimulatePhysics` _mesh true)
  (`PrimitiveComponent.AddForce` _mesh (* (`SceneComponent.GetForwardVector` (`self.Arrow`)) (`self.Force`)) "None" true)
  (if (`self.Highlight`)
    (set `ActorComponent.ComponentTags` (`|MakeArray` "Highlightable" :!type "Name") (`self.Mesh`))))

(fn `UserConstructionScript`
  (`parent.UserConstructionScript`))