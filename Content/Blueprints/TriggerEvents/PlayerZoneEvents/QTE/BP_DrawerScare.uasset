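; BP_DrawerScare is a scare event Blueprint that makes its mesh rattle and jump, apparently as a haunted drawer.
; On Tick, while Jump is set and Triggered is not, it applies a random-strength force in a narrow upward cone to the mesh.
; Neither flag is set in this graph, and the construction script only calls its parent.
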(event `self.ReceiveTick`
  (params (DeltaSeconds :type "Float (single-precision)"))
  (if (`self.Jump`)
    (if (not (`self.Triggered`))
      (`PrimitiveComponent.AddForce` (`self.Mesh`) (* (`KismetMathLibrary.RandomUnitVectorInCone` (0.0 0.0 1.0) 10.0) (`KismetMathLibrary.RandomFloatInRange` 0.0 100000.0)) "None" false))))

(fn `UserConstructionScript`
  (`parent.UserConstructionScript`))