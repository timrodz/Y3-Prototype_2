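; One-shot player zone trigger for a Widow window scare event.
; When the first-person character overlaps the box, it fluctuates power through a linked light flicker Blueprint, if valid, then pauses briefly.
; It spawns the WidowWindow actor at a spawn point and writes a target actor's location into its enemy AI blackboard.
; The trigger destroys itself after that handoff, with debug prints left in.
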(event `self.ReceiveBeginPlay`
  (`/Engine/EditorBlueprintResources/StandardMacros.IsValid` null
    (:`Is Valid`
      (`self.SetActorScale3D` (0.0 0.0 0.0)))))

(event `self.Box.OnComponentBeginOverlap`
  (params (OverlappedComponent :type "PrimitiveComponent Object Reference") (OtherActor :type "Actor Object Reference") (OtherComp :type "PrimitiveComponent Object Reference") (OtherBodyIndex :type Integer) (bFromSweep :type Boolean) (SweepResult :type "HitResult Structure (by ref)"))
  (bind _lightflicker_bp (`self.LightFlicker_BP`))
  (cast `/Game/Blueprints/FirstPersonCharacter/FirstPersonCharacter` OtherActor)
  (if (not (`self.bTriggered`))
    (set `self.bTriggered` true)
    (`/Engine/EditorBlueprintResources/StandardMacros.IsValid` _lightflicker_bp
      (:`Is Valid`
        (`/Game/Blueprints/TriggerEvents/GlobalLampManager_BP.FluctuatePower` _lightflicker_bp)
        (`KismetSystemLibrary.Delay` 1.0))
      (:`Is Not Valid`
        _))
    (bind _returnvalue (`|SpawnActorFromClass` (`self.WidowWindow`) (`KismetMathLibrary.MakeTransform` (`self.K2_GetActorLocation` (`self.SpawnPos`))) "AlwaysSpawn" "OverrideRootScale"))
    (`KismetSystemLibrary.PrintString` "Hello")
    (bind _asbp_enemy_aicontroller (cast `/Game/Blueprints/Enemy/BP_EnemyAIController` (`AIBlueprintHelperLibrary.GetAIController` _returnvalue))
      (:`then`
        (`BlackboardComponent.SetValueAsVector` (`AIBlueprintHelperLibrary.GetBlackboard` _asbp_enemy_aicontroller) "TargetLocation" (`self.K2_GetActorLocation` (`self.Target`)))
        (`self.K2_DestroyActor`))
      (:`CastFailed`
        (`KismetSystemLibrary.PrintString` "fail")))))

(fn `UserConstructionScript`)