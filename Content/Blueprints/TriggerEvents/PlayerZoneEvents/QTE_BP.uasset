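; Player zone trigger that launches a book in brief slow motion when the first-person character enters its box, apparently as a quick-time event.
; On overlap it enables physics on BookSolo, tags it Highlightable and pushes it along the Arrow's forward vector.
; Global time dilation drops, then restores after a Delay, which is itself stretched by the slowdown.
; No input handling or one-shot guard is present.
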(event `self.ReceiveBeginPlay`)

(event `self.Box.OnComponentBeginOverlap`
  (params (OverlappedComponent :type "PrimitiveComponent Object Reference") (OtherActor :type "Actor Object Reference") (OtherComp :type "PrimitiveComponent Object Reference") (OtherBodyIndex :type Integer) (bFromSweep :type Boolean) (SweepResult :type "HitResult Structure (by ref)"))
  (bind _book_solo (`self.Book_Solo`))
  (cast `/Game/Blueprints/FirstPersonCharacter/FirstPersonCharacter` OtherActor)
  (`PrimitiveComponent.SetSimulatePhysics` _book_solo true)
  (set `ActorComponent.ComponentTags` (`|MakeArray` "Highlightable" :!type "Name") _book_solo)
  (`PrimitiveComponent.AddForce` _book_solo (* (`SceneComponent.GetForwardVector` (`self.Arrow`)) 1000.0) "None" true)
  (`GameplayStatics.SetGlobalTimeDilation` 0.25)
  (`KismetSystemLibrary.Delay` 0.5)
  (`GameplayStatics.SetGlobalTimeDilation` 1.0))

(fn `UserConstructionScript`
  (`parent.UserConstructionScript`))