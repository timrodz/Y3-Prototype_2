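; Blueprint that models a breath-holding air meter, draining CurrentAir each tick while IsHoldingBreath is set.
; Both a HoldBreath custom event and an EnableHoldBreath function set the flag, each printing which path was called.
; RestoreBreath refills air toward MaxAir at BreathRechargeRate, but nothing in the file calls it or clears the flag.
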(event `self.ReceiveTick`
  (params (DeltaSeconds :type "Float (single-precision)"))
  ;[1 1 1] Tick Air
  (if (`self.isHoldingBreath?`)
    (`self.TickBreath` DeltaSeconds)))

(event `HoldBreath`
  ;[1 1 1] Custom Event - HoldBreath
  (`KismetSystemLibrary.PrintString` "Calling from custom event")
  (set `self.isHoldingBreath?` true))

(fn `EnableHoldBreath`
  (`KismetSystemLibrary.PrintString` "Calling from Function")
  (set `self.isHoldingBreath?` true))

(fn `RestoreBreath`
  (params (DeltaTime :type "Float (double-precision)"))
  (if (< (`self.CurrentAir`) (`self.MaxAir`))
    (set `self.CurrentAir` (+ (`self.CurrentAir`) (* DeltaTime (`self.BreathRechargeRate`))))))

(fn `TickBreath`
  (params (DeltaTime :type "Float (double-precision)"))
  (if (> (`self.CurrentAir`) 0.0)
    (set `self.CurrentAir` (- (`self.CurrentAir`) DeltaTime))))