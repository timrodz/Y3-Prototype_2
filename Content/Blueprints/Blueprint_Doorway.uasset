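; Interactive door that starts locked until a player with a key enters its trigger, then can be opened and closed.
; Overlapping players gain Interact input, while enemies snap an unlocked door open and shut as they enter and leave.
; Press and release drive the player's BP_DoorInteraction, whose returned value inversely sets the timeline swing rate and sound volume and pitch.
; Low values also trigger player noise.
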(event `self.DoorTrigger.OnComponentBeginOverlap`
  (params (OverlappedComponent :type "PrimitiveComponent Object Reference") (OtherActor :type "Actor Object Reference") (OtherComp :type "PrimitiveComponent Object Reference") (OtherBodyIndex :type Integer) (bFromSweep :type Boolean) (SweepResult :type "HitResult Structure (by ref)"))
  ;[1 1 1] Event Overlap - Enable Disable Input
  (if (`self.isUnlocked`)
    (cast `/Game/Blueprints/EnemyAI/Enemy_BP` OtherActor
      (:`then`
        (`SceneComponent.K2_SetRelativeRotation` (`self.Door`) (struct :`Yaw` 90.0) false false)
        (set `self.isDoorOpen?` true))
      (:`CastFailed`
        (bind _asfirst_person_character (cast `/Game/Blueprints/FirstPersonCharacter` OtherActor :!label _label))
        (set `self.PlayerRef` _asfirst_person_character)
        (`self.EnableInput` (`GameplayStatics.GetPlayerController` 0))))
    (else
      (bind _asfirst_person_character_2 (cast `/Game/Blueprints/FirstPersonCharacter` OtherActor))
      (if (`/Game/Blueprints/FirstPersonCharacter.hasKey` _asfirst_person_character_2)
        (set `self.isUnlocked` true)
        (goto _label)))))

(event `self.DoorTrigger.OnComponentEndOverlap`
  (params (OverlappedComponent :type "PrimitiveComponent Object Reference") (OtherActor :type "Actor Object Reference") (OtherComp :type "PrimitiveComponent Object Reference") (OtherBodyIndex :type Integer))
  ;[1 1 1] Event Overlap - Enable Disable Input
  (if (`self.isUnlocked`)
    (cast `/Game/Blueprints/EnemyAI/Enemy_BP` OtherActor
      (:`then`
        (`SceneComponent.K2_SetRelativeRotation` (`self.Door`) (struct) false false)
        (set `self.isDoorOpen?` false))
      (:`CastFailed`
        (cast `/Game/Blueprints/FirstPersonCharacter` OtherActor)
        (`self.DisableInput` (`GameplayStatics.GetPlayerController` 0))
        (`/Game/Blueprints/BP_DoorInteraction.StopInteracting` (`self.GetComponentByClass` (`self.PlayerRef`) "/Game/Blueprints/BP_DoorInteraction.BP_DoorInteraction_C"))
        (set `self.PlayerRef` null)))))

(event `Key|E`
  (params (Key :type "Key Structure" :default "AnyKey"))
  ;[1 1 1] Event Interaction - Open Close Door
)

(event `InputAction|Interact`
  (params (Key :type "Key Structure" :default "AnyKey"))
  (bind _returnvalue (`self.GetComponentByClass` (`self.PlayerRef`) "/Game/Blueprints/BP_DoorInteraction.BP_DoorInteraction_C"))
  ;[1 1 1] Set Door Interaction States
  (:`Pressed`
    (if (not (`self.isAnimating?`))
      (`/Game/Blueprints/BP_DoorInteraction.StartInteracting` _returnvalue self)))
  (:`Released`
    (bind _openspeed (`/Game/Blueprints/BP_DoorInteraction.StopInteracting` _returnvalue))
    (`self.OpenDoorAnim` _openspeed)))

(event `OpenDoorAnim`
  (params (OpenSpeed :type "Float (double-precision)"))
  (bind _returnvalue (- 1.0 OpenSpeed))
  ;[1 1 1] Animating and Playing Sound on Door Opening
  (`/Engine/EditorBlueprintResources/StandardMacros.CompareFloat` OpenSpeed 0.6
    (:`>`
      _)
    (:`==`
      _)
    (:`<`
      ;[1 1 1] Set Door Interaction States
      (`/Game/Blueprints/FirstPersonCharacter.PlayerMakeNoise` (`self.PlayerRef`))))
  (`GameplayStatics.PlaySoundAtLocation` (`self.SlowDoorSound`) (`SceneComponent.K2_GetComponentLocation` (`self.Door`)) (struct) _returnvalue _returnvalue)
  (`TimelineComponent.SetPlayRate` (`self.DoorOpenTimeline`) (`KismetMathLibrary.FClamp` _returnvalue 0.4))
  (if (`self.isDoorOpen?`)
    (bind (_direction _1) (`Timeline|DoorOpenTimeline` :!via `ReverseFromEnd` :!label _label_2)
      (:`Update`
        (`SceneComponent.K2_SetRelativeRotation` (`self.Door`) (`KismetMathLibrary.MakeRotator` 0.0 0.0 _1) false false)
        (set `self.isAnimating?` true))
      (:`Finished`
        (set `self.isAnimating?` false)
        (if (`self.isDoorOpen?`)
          (set `self.isDoorOpen?` false)
          (else
            (set `self.isDoorOpen?` true)))))
    (else
      (goto _label_2 :!via `PlayFromStart`))))

(fn `CloseDoor`)

(fn `OpenDoor`)

(fn `UserConstructionScript`)