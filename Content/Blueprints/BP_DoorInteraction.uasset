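; Door interaction Blueprint that times how long an interaction has been held as a fraction of the total time to operate.
; Starting an interaction sets a flag and resets the timer, which Tick advances while the flag is set.
; Stopping clears the flag and returns the elapsed fraction, also available through a getter.
; The fraction is not clamped, and nothing here moves a door or acts on completion.
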(event `self.ReceiveTick`
  (params (DeltaSeconds :type "Float (single-precision)"))
  (if (`self.isInteracting?`)
    (set `self.TimeSinceInteraction` (+ DeltaSeconds (`self.TimeSinceInteraction`)))))

(fn `GetNormalisedTime`
  (returns (`Normalised Time` :type "Float (double-precision)"))
  (return (/ (`self.TimeSinceInteraction`) (`self.TotalTimeToOperate`))))

(fn `StartInteracting`
  (set `self.isInteracting?` true)
  (set `self.TimeSinceInteraction` 0.0))

(fn `StopInteracting`
  (returns (OpenSpeed :type "Float (double-precision)"))
  (set `self.isInteracting?` false)
  (return (/ (`self.TimeSinceInteraction`) (`self.TotalTimeToOperate`))))