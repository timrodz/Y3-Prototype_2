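; BP_BreathController manages a player's breath-holding, tracking an air intake value that starts full.
; Each tick it drains air while breath is held, and otherwise recharges it up to the maximum threshold, using separate rate multipliers.
; A toggle event switches holding on or off when allowed.
; Running out of air triggers a reset that stops holding and blocks it for a delay, with debug prints reporting state changes.
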(event `self.ReceiveBeginPlay`
  ;[1 1 1] Set the starting air intake to be the maximum air treshold
  (set `self.CurrentAirIntake` (`self.MaxAirTreshold`)))

(event `self.ReceiveTick`
  (params (DeltaSeconds :type "Float (single-precision)"))
  ;[1 1 1] Determine if the player should be decreasing or restoring breath
  (if (`self.CanHoldBreath`)
    (if (`self.IsHoldingBreath`)
      (`self.DecreaseBreath` DeltaSeconds)
      (else
        (`self.RestoreBreath` DeltaSeconds :!label _label)))
    (else
      (goto _label))))

(event `ToggleBreathState`
  ;[1 1 1] Toggle breath states
  (if (`self.CanHoldBreath`)
    (if (`self.IsHoldingBreath`)
      (set `self.IsHoldingBreath` false)
      (`KismetSystemLibrary.PrintString` "Holding breath: false")
      (else
        (set `self.IsHoldingBreath` true)
        (`KismetSystemLibrary.PrintString` "Holding breath: true")))
    (else
      (`KismetSystemLibrary.PrintString` "Can not hold breath"))))

(event `ResetBreathState`
  (set `self.CurrentAirIntake` 0.0)
  (set `self.IsHoldingBreath` false)
  (set `self.CanHoldBreath` false)
  (`KismetSystemLibrary.PrintString` "Breath treshold reached - Resetting")
  (`KismetSystemLibrary.Delay` (`self.BreathResetDelay`))
  (set `self.CanHoldBreath` true)
  (`KismetSystemLibrary.PrintString` "Can breath again"))

(fn `DecreaseBreath`
  (params (DeltaTime :type "Float (double-precision)"))
  (if (> (`self.CurrentAirIntake`) 0.0)
    (set `self.CurrentAirIntake` (- (`self.CurrentAirIntake`) (* DeltaTime (`self.BreathDecreaseMultiplier`))))
    (else
      (`self.ResetBreathState`))))

(fn `RestoreBreath`
  (params (DeltaTime :type "Float (double-precision)"))
  (if (< (`self.CurrentAirIntake`) (`self.MaxAirTreshold`))
    (set `self.CurrentAirIntake` (+ (`self.CurrentAirIntake`) (* DeltaTime (`self.BreathRechargeMultiplier`))))))