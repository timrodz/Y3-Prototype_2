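; SlidingDoor_BP is a sliding door actor that moves along the world X axis when its IsOpening flag is true.
; BeginPlay stores the start location, and Tick calls Play on a timeline while the flag is set.
; The timeline track sets X as an absolute value, keeping the starting Y and Z, and clears the flag on finish.
; Nothing in this file sets the flag to true or closes the door.
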(event `self.ReceiveBeginPlay`
  (set `self.StartPosition` (`self.K2_GetActorLocation`)))

(event `self.ReceiveTick`
  (params (DeltaSeconds :type "Float (single-precision)"))
  (if (`self.IsOpening`)
    (bind (_direction _newtrack_0) (`Timeline|SlidingDoorTimelIne`)
      (:`Update`
        (`self.K2_SetActorLocation` (`KismetMathLibrary.MakeVector` _newtrack_0 (.y (`self.StartPosition`)) (.z (`self.StartPosition`)))))
      (:`Finished`
        (set `self.IsOpening` false)))))

(fn `UserConstructionScript`)