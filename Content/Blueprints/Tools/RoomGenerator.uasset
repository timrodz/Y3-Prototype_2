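; RoomGenerator builds a rectangular room shell in the construction script from a MaxX by MaxY grid sized to the wall mesh.
; It resizes and raises a Box, then rebuilds four rotated, origin-centred walls as mesh instances.
; Helpers for floor tiles, random props on those tiles and swapping a random wall for an access point exist but are not called here.
; BeginPlay and GenerateMeshStructs do nothing.
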(event `self.ReceiveBeginPlay`)

(fn `AddAccessPoint`
  (locals (Index :type Integer))
  (bind _instancedstaticmesh (`self.InstancedStaticMesh`))
  (`/Engine/EditorBlueprintResources/StandardMacros.IsValid` (`self.AcessSpawn`)
    (:`Is Not Valid`
      (if (`KismetSystemLibrary.IsValidClass` (`self.AcessType`))
        (`KismetSystemLibrary.PrintString` "Valid")
        (bind _output_get (set `local.Index` (`KismetMathLibrary.RandomInteger` (`InstancedStaticMeshComponent.GetInstanceCount` _instancedstaticmesh))))
        (`InstancedStaticMeshComponent.AddInstance` (`self.AccessPoint`) (`InstancedStaticMeshComponent.GetInstanceTransform` (`self.InstancedStaticMesh`) _output_get false))
        (bind _output_get_2 (set `self.AcessSpawn` null))
        (`self.K2_AttachToComponent` _output_get_2 (`self.Box`) "None" "KeepRelative" "KeepRelative" "KeepRelative" false)
        (`InstancedStaticMeshComponent.RemoveInstance` _instancedstaticmesh _output_get)
        (else
          (`KismetSystemLibrary.PrintString` "Invalid"))))))

(fn `AddRandomMesh`
  (params (Mesh :type "StaticMesh Object Reference"))
  (locals (VectorOffset :type "Vector Structure") (Index :type Integer))
  (bind _tempfloortiles (`self.TempFloorTiles`))
  (bind _output_get (set `local.Index` (`KismetMathLibrary.RandomInteger` (`InstancedStaticMeshComponent.GetInstanceCount` _tempfloortiles))))
  (bind _outinstancetransform (`InstancedStaticMeshComponent.GetInstanceTransform` _tempfloortiles _output_get false))
  (bind _returnvalue (`AddComponent|NODE_AddStaticMeshComponent-0` :`RelativeTransform` (`KismetMathLibrary.MakeTransform` (.location _outinstancetransform) (.rotation _outinstancetransform))))
  (`StaticMeshComponent.SetStaticMesh` _returnvalue Mesh)
  (`InstancedStaticMeshComponent.RemoveInstance` (`self.TempFloorTiles`) (`local.Index`)))

(fn `AddStaticMeshToRoot`
  (params (RelativeTransform :type "Transform Structure"))
  (bind _returnvalue (`AddComponent|NODE_AddStaticMeshComponent-4` :`bManualAttachment` true :`RelativeTransform` RelativeTransform))
  (`StaticMeshComponent.SetStaticMesh` _returnvalue (`StaticMeshComponent.StaticMesh` (`self.InstancedStaticMesh`)))
  (`SceneComponent.K2_AttachToComponent` _returnvalue (`self.Scene`) "None" "KeepRelative" "KeepRelative" "KeepRelative" false))

(fn `CreateBoundingWalls`
  (bind _returnvalue (`self.GetBoundingXVector`))
  (bind _returnvalue_2 (`self.GetBoundingXVector`))
  (bind _returnvalue_3 (`self.GetBoundingXVector`))
  (bind _returnvalue_4 (`self.GetBoundingXVector`))
  ;[1 1 1] First Run Through - West Wall
  (for _index (range (`self.MaxX`))
    (`InstancedStaticMeshComponent.AddInstance` (`self.InstancedStaticMesh`) (`KismetMathLibrary.MakeTransform` (- (- (* _returnvalue _index) (* _returnvalue (/ (`KismetMathLibrary.Conv_IntToDouble` (`self.MaxX`)) 2.0))) (* (`KismetMathLibrary.GreaterGreater_VectorRotator` _returnvalue (struct :`Yaw` 90.0)) (/ (`KismetMathLibrary.Conv_IntToDouble` (`self.MaxY`)) 2.0))))))
  ;[1 1 1] Second Run Through - South Wall
  (for _index_2 (range (`self.MaxY`))
    (`InstancedStaticMeshComponent.AddInstance` (`self.InstancedStaticMesh`) (`KismetMathLibrary.MakeTransform` (- (- (* (`KismetMathLibrary.GreaterGreater_VectorRotator` (`self.GetBoundingXVector`) (struct :`Yaw` 90.0)) _index_2) (* _returnvalue_3 (/ (`KismetMathLibrary.Conv_IntToDouble` (`self.MaxX`)) 2.0))) (* (`KismetMathLibrary.GreaterGreater_VectorRotator` _returnvalue_3 (struct :`Yaw` 90.0)) (/ (`KismetMathLibrary.Conv_IntToDouble` (`self.MaxY`)) 2.0))) (struct :`Yaw` 90.0))))
  ;[1 1 1] Third Run Through - North Wall
  (for _index_3 (range (`self.MaxY`))
    (`InstancedStaticMeshComponent.AddInstance` (`self.InstancedStaticMesh`) (`KismetMathLibrary.MakeTransform` (- (+ (* (`KismetMathLibrary.GreaterGreater_VectorRotator` (`self.GetBoundingXVector`) (struct :`Yaw` 90.0)) (+ _index_3 1)) (* _returnvalue_2 (/ (`KismetMathLibrary.Conv_IntToDouble` (`self.MaxX`)) 2.0))) (* (`KismetMathLibrary.GreaterGreater_VectorRotator` _returnvalue_2 (struct :`Yaw` 90.0)) (/ (`KismetMathLibrary.Conv_IntToDouble` (`self.MaxY`)) 2.0))) (struct :`Yaw` -90.0))))
  (for _index_4 (range (`self.MaxX`))
    (`InstancedStaticMeshComponent.AddInstance` (`self.InstancedStaticMesh`) (`KismetMathLibrary.MakeTransform` (- (+ (* (`self.GetBoundingXVector`) (+ _index_4 1)) (* (`KismetMathLibrary.GreaterGreater_VectorRotator` _returnvalue_4 (struct :`Yaw` 90.0)) (/ (`KismetMathLibrary.Conv_IntToDouble` (`self.MaxY`)) 2.0))) (* _returnvalue_4 (/ (`KismetMathLibrary.Conv_IntToDouble` (`self.MaxX`)) 2.0))) (struct :`Yaw` 180.0)))))

(fn `CreateFloorTiles`
  (bind _returnvalue_x (`KismetMathLibrary.BreakVector` (`self.GetBoundingXVector`)))
  (bind _returnvalue (`KismetMathLibrary.MakeVector` _returnvalue_x _returnvalue_x))
  (for _index (range (`self.MaxX`))
    (for _index_2 (range (`self.MaxY`))
      (`InstancedStaticMeshComponent.AddInstance` (`self.TempFloorTiles`) (`KismetMathLibrary.MakeTransform` (- (- (+ (`KismetMathLibrary.MakeVector` (* _index _returnvalue_x) (* _index_2 _returnvalue_x)) (/ _returnvalue 2.0)) (* (`KismetMathLibrary.MakeVector` _returnvalue_x) (/ (`KismetMathLibrary.Conv_IntToDouble` (`self.MaxX`)) 2.0))) (* (`KismetMathLibrary.MakeVector` 0.0 _returnvalue_x) (/ (`KismetMathLibrary.Conv_IntToDouble` (`self.MaxY`)) 2.0))) (struct) _returnvalue)))))

(fn `GenerateMeshStructs`
  (locals (Range :type Integer)))

(fn `UserConstructionScript`
  (bind _returnvalue (`self.GenerateBoxExtents`))
  (bind _box (`self.Box`))
  (`BoxComponent.SetBoxExtent` _box _returnvalue true)
  (`SceneComponent.K2_AddLocalOffset` _box (`KismetMathLibrary.MakeVector` 0.0 0.0 (/ (.z _returnvalue) 1.0)) false false)
  (`InstancedStaticMeshComponent.ClearInstances` (`self.InstancedStaticMesh`))
  (`self.CreateBoundingWalls`))