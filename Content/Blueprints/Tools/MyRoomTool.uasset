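; Room-building tool actor that generates walls, extensions, doors and optional corner pieces from mesh info, using instanced static meshes.
; Edit functions swap wall or corner instances for attached StaticMeshActors so pieces can be adjusted individually, one set at a time.
; Save functions fold valid actors with a matching mesh back into instances and destroy them.
; ReplaceDoorsWithActors turns door instances into attached Blueprint_Doorway actors, removing the instances.
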(fn `Edit Corner Pieces`
  (bind _cornerpieceinstances (`self.CornerPieceInstances`))
  (if (not (`self.bEditingInstances`))
    (set `self.bEditingInstances` true)
    (set `self.EditingPieces` true)
    (`KismetArrayLibrary.Array_Clear` (`self.StaticMesh`))
    (for _index (range (`InstancedStaticMeshComponent.GetInstanceCount` (`self.CornerPieceInstances`)))
      (bind _outinstancetransform (`InstancedStaticMeshComponent.GetInstanceTransform` _cornerpieceinstances _index true))
      (bind _returnvalue (`|SpawnActorFromClass` "/Script/Engine.StaticMeshActor" (`KismetMathLibrary.MakeTransform` (.location _outinstancetransform) (.rotation _outinstancetransform) (.scale _outinstancetransform)) "Undefined" "OverrideRootScale" self))
      (`StaticMeshComponent.SetStaticMesh` (`StaticMeshActor.StaticMeshComponent` _returnvalue) (`StaticMeshComponent.StaticMesh` _cornerpieceinstances))
      (`KismetArrayLibrary.Array_Add` (`self.StaticMesh`) _returnvalue)
      (`SceneComponent.K2_AttachToComponent` (`StaticMeshActor.StaticMeshComponent` _returnvalue) (`self.RootComponent`) "None" "KeepRelative" "KeepRelative" "KeepRelative" true))
    (while (`self.RemoveInstances`)
      (bind _returnvalue_2 (`InstancedStaticMeshComponent.RemoveInstance` _cornerpieceinstances 0))
      (set `self.RemoveInstances` _returnvalue_2))
    (set `self.RemoveInstances` true)))

(fn `Edit Walls`
  (bind _wallinstances (`self.WallInstances`))
  (if (not (`self.bEditingInstances`))
    (set `self.bEditingInstances` true)
    (set `self.EditingWalls` true)
    (`KismetArrayLibrary.Array_Clear` (`self.StaticMesh`))
    (for _index (range (`InstancedStaticMeshComponent.GetInstanceCount` (`self.WallInstances`)))
      (bind _outinstancetransform (`InstancedStaticMeshComponent.GetInstanceTransform` _wallinstances _index true))
      (bind _returnvalue (`|SpawnActorFromClass` "/Script/Engine.StaticMeshActor" (`KismetMathLibrary.MakeTransform` (.location _outinstancetransform) (.rotation _outinstancetransform) (.scale _outinstancetransform)) "Undefined" "OverrideRootScale" self))
      (`StaticMeshComponent.SetStaticMesh` (`StaticMeshActor.StaticMeshComponent` _returnvalue) (`StaticMeshComponent.StaticMesh` _wallinstances))
      (`KismetArrayLibrary.Array_Add` (`self.StaticMesh`) _returnvalue)
      (`SceneComponent.K2_AttachToComponent` (`StaticMeshActor.StaticMeshComponent` _returnvalue) (`self.RootComponent`) "None" "KeepRelative" "KeepRelative" "KeepRelative" true))
    (while (`self.RemoveInstances`)
      (bind _returnvalue_2 (`InstancedStaticMeshComponent.RemoveInstance` _wallinstances 0))
      (set `self.RemoveInstances` _returnvalue_2))
    (set `self.RemoveInstances` true)))

(fn `Generate`
  (`self.GenerateWallInfo`)
  (`self.AddWall`)
  (`self.AddExtentions`)
  (`self.AddDoors`)
  (if (`self.bUseCornerPieces`)
    (`self.AddCornerPieces`)))

(fn `GenerateDoorInfo`
  (bind _mesh (break `MeshInfo` (`self.DoorwayInfo`)))
  (`/Engine/EditorBlueprintResources/StandardMacros.IsValid` _mesh
    (:`Is Valid`
      (bind _returnvalue (`self.GenerateMeshInfo` _mesh))
      (set `self.DoorwayInfo` _returnvalue))))

(fn `GenerateWallInfo`
  (bind _mesh (break `MeshInfo` (`self.WallInfo`)))
  (`/Engine/EditorBlueprintResources/StandardMacros.IsValid` _mesh
    (:`Is Valid`
      (bind _returnvalue (`self.GenerateMeshInfo` _mesh))
      (set `self.WallInfo` _returnvalue))))

(fn `ReplaceDoorsWithActors`
  (for _index (range (`InstancedStaticMeshComponent.GetInstanceCount` (`self.DoorInstances`)))
    (bind _outinstancetransform (`InstancedStaticMeshComponent.GetInstanceTransform` (`self.DoorInstances`) _index true))
    (bind _returnvalue (`|SpawnActorFromClass` "/Game/Blueprints/Interactables/Blueprint_Doorway.Blueprint_Doorway_C" (`KismetMathLibrary.MakeTransform` (.location _outinstancetransform) (.rotation _outinstancetransform) (.scale _outinstancetransform)) "Undefined" "OverrideRootScale"))
    (`self.K2_AttachToActor` _returnvalue self "None" "KeepWorld" "KeepWorld" "KeepWorld" true)
    (bind _returnvalue_2 (`InstancedStaticMeshComponent.RemoveInstance` (`self.DoorInstances`) 0 :!label _label))
    (while _returnvalue_2
      (goto _label))))

(fn `Save Corner Pieces`
  (bind _cornerpieceinstances (`self.CornerPieceInstances`))
  (if (`self.EditingPieces`)
    (if (`self.bEditingInstances`)
      (set `self.EditingPieces` false)
      (set `self.bEditingInstances` false)
      (for _array_element (`self.StaticMesh`)
        (`/Engine/EditorBlueprintResources/StandardMacros.IsValid` _array_element
          (:`Is Valid`
            (if (== (`StaticMeshComponent.StaticMesh` (`StaticMeshActor.StaticMeshComponent` _array_element)) (`StaticMeshComponent.StaticMesh` _cornerpieceinstances))
              (`InstancedStaticMeshComponent.AddInstance` _cornerpieceinstances (`KismetMathLibrary.ConvertTransformToRelative` (`SceneComponent.K2_GetComponentToWorld` _cornerpieceinstances) (`SceneComponent.K2_GetComponentToWorld` (`StaticMeshActor.StaticMeshComponent` _array_element))))
              (`self.K2_DestroyActor` _array_element)))))
      (`KismetArrayLibrary.Array_Clear` (`self.StaticMesh`)))))

(fn `Save Walls`
  (bind _wallinstances (`self.WallInstances`))
  (if (`self.EditingWalls`)
    (if (`self.bEditingInstances`)
      (set `self.bEditingInstances` false)
      (set `self.EditingWalls` false)
      (for _array_element (`self.StaticMesh`)
        (`/Engine/EditorBlueprintResources/StandardMacros.IsValid` _array_element
          (:`Is Valid`
            (if (== (`StaticMeshComponent.StaticMesh` (`StaticMeshActor.StaticMeshComponent` _array_element)) (`StaticMeshComponent.StaticMesh` _wallinstances))
              (`InstancedStaticMeshComponent.AddInstance` _wallinstances (`KismetMathLibrary.ConvertTransformToRelative` (`SceneComponent.K2_GetComponentToWorld` _wallinstances) (`SceneComponent.K2_GetComponentToWorld` (`StaticMeshActor.StaticMeshComponent` _array_element))))
              (`self.K2_DestroyActor` _array_element)))))
      (`KismetArrayLibrary.Array_Clear` (`self.StaticMesh`)))))

(fn `UserConstructionScript`)