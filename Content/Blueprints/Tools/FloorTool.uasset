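; Editor-style floor tool that fills an X by Y grid with Floormesh as instanced static meshes.
; The construction script and Generate build the grid, spacing both axes by the mesh's X bounds and duplicating the first tile of each row.
; Unconvert swaps instances for attached StaticMeshActors.
; Convert folds those still using the same mesh back into instances and sets Saved, which stops the construction script from rebuilding.
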(fn `Convert`
  (bind _instancedstaticmesh (`self.InstancedStaticMesh`))
  (set `self.Saved` true)
  (for _array_element (`self.StaticMesh`)
    (`/Engine/EditorBlueprintResources/StandardMacros.IsValid` _array_element
      (:`Is Valid`
        (if (== (`StaticMeshComponent.StaticMesh` (`StaticMeshActor.StaticMeshComponent` _array_element)) (`StaticMeshComponent.StaticMesh` _instancedstaticmesh))
          (`InstancedStaticMeshComponent.AddInstance` _instancedstaticmesh (`KismetMathLibrary.ConvertTransformToRelative` (`SceneComponent.K2_GetComponentToWorld` _instancedstaticmesh) (`SceneComponent.K2_GetComponentToWorld` (`StaticMeshActor.StaticMeshComponent` _array_element))))
          (`self.K2_DestroyActor` _array_element)))))
  (`KismetArrayLibrary.Array_Clear` (`self.StaticMesh`)))

(fn `Generate`
  (bind _floormesh (`self.Floormesh`))
  (bind _instancedstaticmesh (`self.InstancedStaticMesh`))
  (bind _returnvalue (`StaticMesh.GetBoundingBox` _floormesh))
  (bind _returnvalue_2 (+ (`KismetMathLibrary.Abs` (.x (break `Box` _returnvalue))) (`KismetMathLibrary.Abs` (.x (`.Max` (break `Box` _returnvalue))))))
  (`InstancedStaticMeshComponent.ClearInstances` _instancedstaticmesh)
  (`StaticMeshComponent.SetStaticMesh` _instancedstaticmesh _floormesh)
  (for _index (range (`self.X`))
    (bind _returnvalue_3 (* _index _returnvalue_2))
    (`InstancedStaticMeshComponent.AddInstance` (`self.InstancedStaticMesh`) (`KismetMathLibrary.MakeTransform` (`KismetMathLibrary.MakeVector` _returnvalue_3)))
    (for _index_2 (range (`self.Y`))
      (`InstancedStaticMeshComponent.AddInstance` (`self.InstancedStaticMesh`) (`KismetMathLibrary.MakeTransform` (`KismetMathLibrary.MakeVector` _returnvalue_3 (* _index_2 _returnvalue_2)))))))

(fn `Unconvert`
  (bind _instancedstaticmesh (`self.InstancedStaticMesh`))
  (`KismetArrayLibrary.Array_Clear` (`self.StaticMesh`))
  (for _index (range (`InstancedStaticMeshComponent.GetInstanceCount` (`self.InstancedStaticMesh`)))
    (bind _returnvalue (`|SpawnActorFromClass` "/Script/Engine.StaticMeshActor" (`InstancedStaticMeshComponent.GetInstanceTransform` _instancedstaticmesh _index true) "Undefined" "OverrideRootScale" self))
    (`StaticMeshComponent.SetStaticMesh` (`StaticMeshActor.StaticMeshComponent` _returnvalue) (`StaticMeshComponent.StaticMesh` _instancedstaticmesh))
    (`KismetArrayLibrary.Array_Add` (`self.StaticMesh`) _returnvalue)
    (`SceneComponent.K2_AttachToComponent` (`StaticMeshActor.StaticMeshComponent` _returnvalue) (`self.RootComponent`) "None" "KeepRelative" "KeepRelative" "KeepRelative" true))
  (while (`self.RemoveInstances`)
    (bind _returnvalue_2 (`InstancedStaticMeshComponent.RemoveInstance` _instancedstaticmesh 0))
    (set `self.RemoveInstances` _returnvalue_2)))

(fn `UserConstructionScript`
  (bind _floormesh (`self.Floormesh`))
  (bind _instancedstaticmesh (`self.InstancedStaticMesh`))
  (bind _returnvalue (`StaticMesh.GetBoundingBox` _floormesh))
  (bind _returnvalue_2 (+ (`KismetMathLibrary.Abs` (.x (break `Box` _returnvalue))) (`KismetMathLibrary.Abs` (.x (`.Max` (break `Box` _returnvalue))))))
  (if (not (`self.Saved`))
    (`InstancedStaticMeshComponent.ClearInstances` _instancedstaticmesh)
    (`StaticMeshComponent.SetStaticMesh` _instancedstaticmesh _floormesh)
    (for _index (range (`self.X`))
      (bind _returnvalue_3 (* _index _returnvalue_2))
      (`InstancedStaticMeshComponent.AddInstance` (`self.InstancedStaticMesh`) (`KismetMathLibrary.MakeTransform` (`KismetMathLibrary.MakeVector` _returnvalue_3)))
      (for _index_2 (range (`self.Y`))
        (`InstancedStaticMeshComponent.AddInstance` (`self.InstancedStaticMesh`) (`KismetMathLibrary.MakeTransform` (`KismetMathLibrary.MakeVector` _returnvalue_3 (* _index_2 _returnvalue_2))))))))