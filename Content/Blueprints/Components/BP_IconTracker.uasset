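; Player component that tracks nearby interactable objects and shows an on-screen icon over the best candidate.
; A spawned sphere attached to the pawn collects overlapping InteractableObjects, and Tick picks the one nearest a point along the camera's forward vector.
; The icon animates between targets and follows the projected screen position.
; Within close range and a narrow view cone, it shows the interact texture and enables custom depth highlighting.
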(event `self.ReceiveBeginPlay`
  (bind _returnvalue (`GameplayStatics.GetPlayerPawn` 0))
  (bind (_returnvalue_location _returnvalue_rotation _returnvalue_scale) (`KismetMathLibrary.BreakTransform` (`Actor.GetTransform` _returnvalue)))
  (bind _returnvalue_2 (`|CreateWidget` "/Game/Blueprints/Widgets/Subtitle/BP_Icon.BP_Icon_C" (`GameplayStatics.GetPlayerController` 0)))
  (bind _output_get (set `self.IconWidget` _returnvalue_2))
  (`UserWidget.AddToViewport` _output_get 0)
  (bind _returnvalue_3 (`|SpawnActorFromClass` "/Script/Engine.TriggerSphere" (`KismetMathLibrary.MakeTransform` (+ _returnvalue_location (0.0 0.0 0.0)) _returnvalue_rotation _returnvalue_scale) "Undefined" "OverrideRootScale" _returnvalue _returnvalue))
  (bind _collisioncomponent (`TriggerBase.CollisionComponent` _returnvalue_3))
  (set `self.TriggerSphere` _collisioncomponent)
  (`SceneComponent.SetRelativeScale3D` _collisioncomponent (`KismetMathLibrary.Conv_DoubleToVector` (/ (`self.Size`) 32.0)))
  (`Actor.K2_AttachToActor` _returnvalue_3 (`GameplayStatics.GetPlayerPawn` 0) "None" "SnapToTarget" "SnapToTarget" "KeepWorld" true)
  (add `PrimitiveComponent.OnComponentBeginOverlap` _collisioncomponent (`|CreateDelegate` :!event `OnComponentBeginOverlap`))
  (add `PrimitiveComponent.OnComponentEndOverlap` _collisioncomponent (`|CreateDelegate` :!event `OnComponentEndOverlap`))
  (bind _asfirst_person_character (cast `/Game/Blueprints/FirstPersonCharacter/FirstPersonCharacter` (`self.GetOwner`)))
  (set `self.Player` _asfirst_person_character))

(event `self.ReceiveTick`
  (params (DeltaSeconds :type "Float (single-precision)"))
  (bind _output (`self.GetLowest`))
  (set `self.LowestLength` 999999999.0)
  (set `self.Lowest` -99999)
  (for (_array_element _array_index) (`self.Actors`)
    (bind (_returnvalue _returnvalue2) (`self.isCloser` _array_element))
    (if _returnvalue
      (set `self.Lowest` _array_index)
      (set `self.LowestLength` _returnvalue2)))
  (if (>= (`self.Lowest`) 0)
    (if (== _output (`self.CurrentActor`))
      (`/Engine/EditorBlueprintResources/StandardMacros.IsValid` (`self.IconWidget`)
        (:`Is Valid`
          _))
      (else
        (bind _output_get (`self.AnimateIn` _output))))
    (bind _returnvalue_2 (`MyFunctionLibrary.GetLastRenderedTime` _output_get 0.2))
    (if _returnvalue_2
      (`self.UpdateViewportPosition`))
    (else
      (`self.AnimateOut`))))

(event `OnComponentBeginOverlap`
  (params (OverlappedComponent :type "PrimitiveComponent Object Reference") (OtherActor :type "Actor Object Reference") (OtherComp :type "PrimitiveComponent Object Reference") (OtherBodyIndex :type Integer) (bFromSweep :type Boolean) (SweepResult :type "HitResult Structure (by ref)"))
  (bind _asinteractable_object (cast `InteractableObject` OtherActor))
  (`KismetArrayLibrary.Array_Add` (`self.Actors`) _asinteractable_object))

(event `OnComponentEndOverlap`
  (params (OverlappedComponent :type "PrimitiveComponent Object Reference") (OtherActor :type "Actor Object Reference") (OtherComp :type "PrimitiveComponent Object Reference") (OtherBodyIndex :type Integer))
  (bind _asinteractable_object (cast `InteractableObject` OtherActor))
  (`KismetArrayLibrary.Array_RemoveItem` (`self.Actors`) _asinteractable_object))

(fn `AnimateIn`
  (params (CurrentActor :type "Actor Object Reference"))
  (returns (Output_Get :type "Actor Object Reference"))
  (bind _currentactor (`self.CurrentActor`))
  (`/Engine/EditorBlueprintResources/StandardMacros.IsValid` _currentactor
    (:`Is Valid`
      (bind _asstatic_mesh_component (cast `StaticMeshComponent` (`Actor.GetComponentByClass` _currentactor "/Script/Engine.PrimitiveComponent"))
        (:`then`
          (`PrimitiveComponent.SetRenderCustomDepth` _asstatic_mesh_component false))
        (:`CastFailed`
          _)))
    (:`Is Not Valid`
      _))
  (bind _output_get (set `self.CurrentActor` CurrentActor))
  (`/Engine/EditorBlueprintResources/StandardMacros.IsValid` _output_get
    (:`Is Valid`
      (bind _returnvalue (`Actor.GetComponentByClass` _output_get "/Script/Engine.PrimitiveComponent"))
      (`/Engine/EditorBlueprintResources/StandardMacros.IsValid` _returnvalue
        (:`Is Valid`
          (`PrimitiveComponent.SetRenderCustomDepth` _returnvalue true))
        (:`Is Not Valid`
          _)))
    (:`Is Not Valid`
      _))
  (`/Game/Blueprints/Widgets/Subtitle/BP_Icon.Animate` (`self.IconWidget`))
  (return (`self.CurrentActor`)))

(fn `AnimateOut`
  (bind _currentactor (`self.CurrentActor`))
  (bind _returnvalue (`Actor.GetComponentByClass` _currentactor "/Script/Engine.PrimitiveComponent"))
  (`/Engine/EditorBlueprintResources/StandardMacros.IsValid` _currentactor
    (:`Is Valid`
      (`/Engine/EditorBlueprintResources/StandardMacros.IsValid` _returnvalue
        (:`Is Valid`
          (`PrimitiveComponent.SetRenderCustomDepth` _returnvalue false))))
    (:`Is Not Valid`
      _))
  (set `self.CurrentActor` null)
  (`/Game/Blueprints/Widgets/Subtitle/BP_Icon.AnimateOut` (`self.IconWidget`)))

(fn `NewFunction_0`
  (bind _widgets (`self.Widgets`))
  (set `self.LowestLength` 999.0)
  (set `self.Lowest` -999)
  (for (_array_element _array_index) (`self.Widgets`)
    (bind _returnvalue (`KismetMathLibrary.VSize2D` (`.Translation` (break `WidgetTransform` (`Widget.RenderTransform` _array_element)))))
    (if (<= _returnvalue (`self.LowestLength`))
      (set `self.Lowest` _array_index)
      (set `self.LowestLength` _returnvalue)
      (else
        (`Widget.RemoveFromParent` _array_element))))
  (if (>= (`self.Lowest`) 0)
    (if (not (`Widget.IsInViewport` _array_element))
      (bind _output_get (set `self.IconWidget` (`|GetArrayItem` _widgets (`self.Lowest`))))
      (`UserWidget.AddToViewport` _output_get 0)
      (`KismetSystemLibrary.PrintString` (`KismetStringLibrary.Conv_IntToString` (`KismetArrayLibrary.Array_Length` (`self.Widgets`))))
      (`KismetArrayLibrary.Array_Clear` _widgets))))

(fn `NewFunction_1`
  (params (Object :type "Object Object Reference") (LocatorRef :type "Actor Object Reference") (self2 :type "Actor Object Reference") (Object2 :type "Object Object Reference"))
  (bind _returnvalue (`GameplayStatics.GetPlayerController` 0))
  (cast `/Game/Blueprints/BaseClasses/BP_InteractableObject` Object
    (:`then`
      _)
    (:`CastFailed`
      (cast `/Game/Blueprints/Interactables/Equips/BP_Equipable` Object2)))
  (bind _returnvalue_2 (`|CreateWidget` "/Game/Blueprints/Widgets/Subtitle/BP_Icon.BP_Icon_C" _returnvalue))
  (set `/Game/Blueprints/Widgets/Subtitle/BP_Icon.LocatorRef` LocatorRef _returnvalue_2)
  (`KismetArrayLibrary.Array_Add` (`self.Widgets`) _returnvalue_2)
  (`UserWidget.AddToViewport` _returnvalue_2 0)
  (if true
    (`UserWidget.SetPositionInViewport` _returnvalue_2 (`WidgetLayoutLibrary.ProjectWorldLocationToWidgetPosition` _returnvalue (`Actor.K2_GetActorLocation` self2)) true)))

(fn `ReturnCurrentActor`
  (returns (AtInteractDistance :type Boolean) (CurrentActor :type "Actor Object Reference"))
  (bind _camera (`/Game/Blueprints/FirstPersonCharacter/FirstPersonCharacter.Camera` (`self.Player`)))
  (return (and (< (`KismetMathLibrary.VSize` (- (`Actor.K2_GetActorLocation` (`self.CurrentActor`)) (`Actor.K2_GetActorLocation` (`self.Player`)))) 150.0) (< (`KismetMathLibrary.DegAcos` (`KismetMathLibrary.Dot_VectorVector` (`KismetMathLibrary.Normal` (- (`Actor.K2_GetActorLocation` (`self.CurrentActor`)) (`SceneComponent.K2_GetComponentLocation` _camera))) (`SceneComponent.GetForwardVector` _camera))) 10.0)) (`self.CurrentActor`)))

(fn `UpdateViewportPosition`
  (bind (_screenposition _returnvalue) (`self.ProjectCurrentActor`))
  (bind _currentactor (`self.CurrentActor`))
  (bind _iconwidget (`self.IconWidget`))
  (bind _currentactor_2 (`self.CurrentActor`))
  (bind _camera (`/Game/Blueprints/FirstPersonCharacter/FirstPersonCharacter.Camera` (`self.Player`)))
  (bind _image_0 (`/Game/Blueprints/Widgets/Subtitle/BP_Icon.Image_0` _iconwidget))
  (if _returnvalue
    (`UserWidget.SetPositionInViewport` _iconwidget _screenposition true)
    (if (and (< (`KismetMathLibrary.VSize` (- (`Actor.K2_GetActorLocation` (`self.CurrentActor`)) (`Actor.K2_GetActorLocation` (`self.Player`)))) 150.0) (< (`KismetMathLibrary.DegAcos` (`KismetMathLibrary.Dot_VectorVector` (`KismetMathLibrary.Normal` (- (`Actor.K2_GetActorLocation` (`self.CurrentActor`)) (`SceneComponent.K2_GetComponentLocation` _camera))) (`SceneComponent.GetForwardVector` _camera))) 10.0))
      (bind _asinteractable_object (cast `InteractableObject` (`self.CurrentActor`)))
      (`Image.SetBrushFromTexture` _image_0 (`InteractableObject.InteractIcon` _asinteractable_object) false)
      (`/Engine/EditorBlueprintResources/StandardMacros.IsValid` _currentactor_2
        (:`Is Valid`
          (bind _asstatic_mesh_component (cast `StaticMeshComponent` (`Actor.GetComponentByClass` _currentactor_2 "/Script/Engine.PrimitiveComponent")))
          (`PrimitiveComponent.SetRenderCustomDepth` _asstatic_mesh_component true)))
      (else
        (bind _asbp_equipable (cast `/Game/Blueprints/Interactables/Equips/BP_Equipable` (`self.CurrentActor`))
          (:`then`
            (bind _returnvalue_2 (`/Game/Blueprints/Components/BP_Inventory.HasItem` (`/Game/Blueprints/FirstPersonCharacter/FirstPersonCharacter.BP_Inventory` (`self.Player`)) _asbp_equipable))
            (if _returnvalue_2
              (`Image.SetBrushFromTexture` (`/Game/Blueprints/Widgets/Subtitle/BP_Icon.Image_0` (`self.IconWidget`)) (`/Game/Blueprints/Interactables/Equips/BP_Equipable.InteractIcon_Override` _asbp_equipable) false)
              (else
                (`Image.SetBrushFromTexture` _image_0 "/Game/Icons/Circle_Button.Circle_Button" false :!label _label))))
          (:`CastFailed`
            (goto _label)))
        (`/Engine/EditorBlueprintResources/StandardMacros.IsValid` _currentactor
          (:`Is Valid`
            (bind _asstatic_mesh_component_2 (cast `StaticMeshComponent` (`Actor.GetComponentByClass` _currentactor "/Script/Engine.PrimitiveComponent")))
            (`PrimitiveComponent.SetRenderCustomDepth` _asstatic_mesh_component_2 false)))))))