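; Breath-holding component for the first-person character, tracking an air level that drains while breath is held.
; Tick drains the level toward zero or recharges it toward a maximum, using separate rate multipliers, while breath holding is allowed.
; A toggle event flips the holding state.
; ResetBreathState empties the air, makes player noise with heavy-breathing audio, and locks the mechanic for a delay; nothing here calls it automatically.
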(event `self.ReceiveTick`
  (params (DeltaSeconds :type "Float (single-precision)"))
  (if (`self.CanHoldBreath`)
    (if (`self.IsHoldingBreath`)
      (`self.DecreaseBreath` DeltaSeconds)
      (else
        (`self.RestoreBreath` DeltaSeconds)))))

(event `self.ToggleBreathState`
  ;[1 1 1] Toggle Breath State
  (if (`self.CanHoldBreath`)
    (if (`self.IsHoldingBreath`)
      (set `self.IsHoldingBreath` false)
      (else
        (set `self.IsHoldingBreath` true)))))

(event `self.ResetBreathState`
  ;[1 1 1] Reset Breathing State
  (set `self.CurrentAirIntake` 0.0)
  (set `self.IsHoldingBreath` false)
  (set `self.CanHoldBreath` false)
  (bind _asfirst_person_character (cast `/Game/Blueprints/FirstPersonCharacter` (`self.GetOwner`)))
  (`/Game/Blueprints/FirstPersonCharacter.PlayerMakeNoise` _asfirst_person_character)
  (`GameplayStatics.PlaySound2D` "/Game/Audio/Heavy_breathing_-_Y3P2.Heavy_breathing_-_Y3P2")
  (`KismetSystemLibrary.Delay` (`self.BreathResetDelay`))
  (set `self.CanHoldBreath` true))

(fn `DecreaseBreath`
  (params (Delta :type "Float (double-precision)"))
  (if (> (`self.CurrentAirIntake`) 0.0)
    (set `self.CurrentAirIntake` (- (`self.CurrentAirIntake`) (* Delta (`self.BreathDecreaseMultiplier`))))))

(fn `IncreaseBreath`)

(fn `RestoreBreath`
  (params (Delta :type "Float (double-precision)"))
  (if (< (`self.CurrentAirIntake`) (`self.MaxAirThreshold`))
    (set `self.CurrentAirIntake` (+ (`self.CurrentAirIntake`) (* Delta (`self.BreathRechargeMultiplier`))))))