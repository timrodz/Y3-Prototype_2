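; BP_ThrowableActor is a physics-simulated prop with a configurable mesh whose impacts draw the attention of nearby enemies.
; Impacts count only after a three-second startup delay and above a minimum speed, with the first one ignored.
; A hit passes its location to each EnemyAIController whose BP_EnemyCharacter is within hearing threshold, playing a randomized impact sound.
; A DoOnce throttles this, resetting a second after an enemy is alerted.
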(event `self.ReceiveBeginPlay`
  (`KismetSystemLibrary.Delay` 3.0)
  (set `self.Enabled` true)
  (set `self.CanMakeNoise` false))

(event `self.ReceiveHit`
  (params (MyComp :type "PrimitiveComponent Object Reference") (Other :type "Actor Object Reference") (OtherComp :type "PrimitiveComponent Object Reference") (bSelfMoved :type Boolean) (HitLocation :type "Vector Structure") (HitNormal :type "Vector Structure") (NormalImpulse :type "Vector Structure") (Hit :type "HitResult Structure (by ref)"))
  (`/Engine/EditorBlueprintResources/StandardMacros.CompareFloat` (`KismetMathLibrary.VSize` (`self.GetVelocity`)) 30.0
    (:`>`
      ;[0.1515 0.165 0.07084] Collision
      (if (`self.Enabled`)
        (if (`self.FirstHit`)
          (`KismetSystemLibrary.Delay` 1.0)
          (set `self.FirstHit` false)
          (else
            (`/Engine/EditorBlueprintResources/StandardMacros.DoOnce` false :!label _label
              (:`Completed`
                (bind _outactors (`GameplayStatics.GetAllActorsOfClass` "/Game/Blueprints/Enemy/BP_EnemyCharacter.BP_EnemyCharacter_C"))
                (for _array_element _outactors
                  (bind _hearingthreshold (`/Game/Blueprints/Enemy/BP_EnemyCharacter.GetHearingThreshold` _array_element))
                  (if (<= (`KismetMathLibrary.VSize` (- HitLocation (`self.K2_GetActorLocation` _array_element))) _hearingthreshold)
                    (bind _asenemy_aicontroller (cast `EnemyAIController` (`Pawn.GetController` _array_element)))
                    (`EnemyAIController.SetHeardNoiseLocation` _asenemy_aicontroller HitLocation)
                    (`GameplayStatics.PlaySoundAtLocation` (`self.OnHitSound`) HitLocation (struct) (`KismetMathLibrary.RandomFloatInRange` 0.6 1.25) (`KismetMathLibrary.RandomFloatInRange` 0.8 1.2))
                    (`KismetSystemLibrary.Delay` 1.0)
                    (goto _label :!via `Reset`)))))))))))

(fn `UserConstructionScript`
  (bind _staticmesh (`self.StaticMesh`))
  (`StaticMeshComponent.SetStaticMesh` _staticmesh (`self.Mesh`))
  (`PrimitiveComponent.SetSimulatePhysics` _staticmesh true))