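; Door interaction component that times how long an interaction with a door has lasted.
; StartInteracting stores the door reference and resets the timer, which Tick advances while the interaction is active.
; GetNormalisedTime returns elapsed time as an unclamped fraction of the total operating time.
; StopInteracting ends timing, resets the timer and returns that final fraction, leaving any action on the door outside this component.
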(event `self.ReceiveTick`
  (params (DeltaSeconds :type "Float (single-precision)"))
  (if (`self.isInteracting?`)
    (set `self.TimeSinceInteraction` (+ DeltaSeconds (`self.TimeSinceInteraction`)))
    (`self.GetNormalisedTime`)))

(fn `GetNormalisedTime`
  (returns (`Normalised Time` :type "Float (double-precision)"))
  (return (/ (`self.TimeSinceInteraction`) (`self.TotalTimeToOperate`))))

(fn `StartInteracting`
  (params (DoorRef :type "/Game/Blueprints/Interactables/Blueprint_Doorway Object Reference"))
  (set `self.isInteracting?` true)
  (set `self.TimeSinceInteraction` 0.0)
  (set `self.CurrentDoor` DoorRef))

(fn `StopInteracting`
  (returns (OpenSpeed :type "Float (double-precision)"))
  (set `self.isInteracting?` false)
  (bind _output_get (set `self.FinalTime` (/ (`self.TimeSinceInteraction`) (`self.TotalTimeToOperate`))))
  (set `self.TimeSinceInteraction` 0.0)
  (return _output_get))