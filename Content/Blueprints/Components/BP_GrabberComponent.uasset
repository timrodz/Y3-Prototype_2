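; BP_GrabberComponent is a grabber component Blueprint that adds audio feedback when a component is grabbed.
; The grab event plays a fixed grab sound at the grabbed component's world location.
; The release event is empty, and its throwing sound is left unconnected.
; An unconnected draft sketches choosing wood or glass sounds by component tag, with no sounds assigned yet.
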(event `self.OnReleaseComponent`
  (params (Component :type "PrimitiveComponent Object Reference"))
  ;[1 1 1] Cast to mesh and play sound based on mesh, or just play the same sound each time and don't cast
)

(event `self.OnGrabComponent`
  (params (Component :type "PrimitiveComponent Object Reference"))
  ;[1 1 1] Cast to mesh and play sound based on mesh, or just play the same sound each time and don't cast
  (`GameplayStatics.PlaySoundAtLocation` "/Game/Audio/Sounds/Items/grabbing-something-fast.grabbing-something-fast" (`SceneComponent.K2_GetComponentLocation` Component)))