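; Component that highlights items the player looks at, using a per-tick visibility line trace from the camera out to Range.
; Hit static mesh components tagged "Highlightable" get custom depth rendering, cleared when the trace hits an untagged component.
; Hit actors with a BP_MaterialSwapper get Highlight, with the previous swapper unhighlighted.
; A trace miss clears only the swapper highlight, and FireTorch hits print a debug string.
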(event `self.ReceiveTick`
  (params (DeltaSeconds :type "Float (single-precision)"))
  (bind _returnvalue (`GameplayStatics.GetPlayerCameraManager` 0))
  (bind _returnvalue_2 (`PlayerCameraManager.GetCameraLocation` _returnvalue))
  (bind (_outhit _returnvalue_3) (`KismetSystemLibrary.LineTraceSingle` _returnvalue_2 (+ _returnvalue_2 (* (`KismetMathLibrary.GetForwardVector` (`PlayerCameraManager.GetCameraRotation` _returnvalue)) (`self.Range`))) "TraceTypeQuery1"))
  (if _returnvalue_3
    (bind (_bblockinghit _binitialoverlap _time _location _impactpoint _normal _impactnormal _physmat _hitactor _hitcomponent) (`GameplayStatics.BreakHitResult` _outhit))
    (`self.DoHighlightableItemCheck` _returnvalue_3 _hitcomponent _hitcomponent _hitcomponent)
    (`self.CheckMaterialSwapper` _hitactor)
    (cast `/Game/Blueprints/Fires/FireTorch` _hitactor)
    (`KismetSystemLibrary.PrintString` "Hello")
    (else
      (`self.UnhighlightMaterialSwapper`))))

(fn `CheckMaterialSwapper`
  (params (self2 :type "Actor Object Reference"))
  (bind _returnvalue (`Actor.GetComponentByClass` self2 "/Game/Blueprints/Components/BP_MaterialSwapper.BP_MaterialSwapper_C"))
  (bind _materialswapperhit (`self.MaterialSwapperHit`))
  (`/Engine/EditorBlueprintResources/StandardMacros.IsValid` _materialswapperhit
    (:`Is Valid`
      (`/Game/Blueprints/Components/BP_MaterialSwapper.UnHighlight` _materialswapperhit))
    (:`Is Not Valid`
      _))
  (if (`KismetSystemLibrary.IsValid` _returnvalue)
    (set `self.MaterialSwapperHit` _returnvalue)
    (`/Game/Blueprints/Components/BP_MaterialSwapper.Highlight` (`self.MaterialSwapperHit`))))

(fn `DoHighlightableItemCheck`
  (params (Hit :type Boolean) (Object :type "Object Object Reference") (HitComponent :type "Object Object Reference") (ActorHit :type "ActorComponent Object Reference"))
  (bind _staticmeshhit (`self.StaticMeshHit`))
  (if Hit
    (if (`self.ComponentHasTag` ActorHit "Highlightable")
      (`self.DoHighlightCheck` (`self.StaticMeshHit`) Object HitComponent)
      (else
        (`/Engine/EditorBlueprintResources/StandardMacros.IsValid` _staticmeshhit :!label _label
          (:`Is Valid`
            (`PrimitiveComponent.SetRenderCustomDepth` _staticmeshhit false)
            (`PrimitiveComponent.SetCustomDepthStencilValue` _staticmeshhit 0)
            (set `self.StaticMeshHit` null)))))
    (else
      (goto _label))))

(fn `DoHighlightCheck`
  (params (InputObject :type "Object Object Reference") (Object :type "Object Object Reference") (Object2 :type "Object Object Reference"))
  (bind _staticmeshhit (`self.StaticMeshHit`))
  (`/Engine/EditorBlueprintResources/StandardMacros.IsValid` InputObject
    (:`Is Valid`
      (bind _asstatic_mesh_component (cast `StaticMeshComponent` Object2))
      (if (not (== (`self.StaticMeshHit`) _asstatic_mesh_component))
        (`PrimitiveComponent.SetRenderCustomDepth` _staticmeshhit false)
        (`PrimitiveComponent.SetCustomDepthStencilValue` _staticmeshhit 1)
        (bind _output_get (set `self.StaticMeshHit` _asstatic_mesh_component))
        (`PrimitiveComponent.SetRenderCustomDepth` _output_get true)
        (`PrimitiveComponent.SetCustomDepthStencilValue` _output_get 1)))
    (:`Is Not Valid`
      (bind _asstatic_mesh_component_2 (cast `StaticMeshComponent` Object))
      (bind _output_get_2 (set `self.StaticMeshHit` _asstatic_mesh_component_2))
      (`PrimitiveComponent.SetRenderCustomDepth` _output_get_2 true)
      (`PrimitiveComponent.SetCustomDepthStencilValue` _output_get_2 1))))

(fn `UnhighlightMaterialSwapper`
  (bind _materialswapperhit (`self.MaterialSwapperHit`))
  (`/Engine/EditorBlueprintResources/StandardMacros.IsValid` _materialswapperhit
    (:`Is Valid`
      (`/Game/Blueprints/Components/BP_MaterialSwapper.UnHighlight` _materialswapperhit)
      (set `self.MaterialSwapperHit` null))))