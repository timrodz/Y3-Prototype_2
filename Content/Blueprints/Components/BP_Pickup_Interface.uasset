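; Pickup Blueprint with a static mesh that can be switched between a highlighted and a normal look.
; The construction script caches dynamic material instances of the highlight material and the mesh's slot 0 material.
; Highlight and UnHighlight swap slot 0 between them, with a flag preventing repeat highlighting.
; Custom depth and stencil nodes are present but disconnected, so highlighting relies solely on the material swap.
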(event `Highlight`
  (if (not (`self.bIsHighlighted`))
    (`PrimitiveComponent.SetMaterial` (`self.StaticMesh`) 0 (`self.DynamicMaterial`))
    (set `self.bIsHighlighted` true)))

(event `UnHighlight`
  (`PrimitiveComponent.SetMaterial` (`self.StaticMesh`) 0 (`self.DefaultMaterial`))
  (set `self.bIsHighlighted` false))

(fn `UserConstructionScript`
  (bind _staticmesh (`self.StaticMesh`))
  (bind _returnvalue (`KismetMaterialLibrary.CreateDynamicMaterialInstance` (`self.HighlightMaterial`)))
  (set `self.DynamicMaterial` _returnvalue)
  (bind _returnvalue_2 (`PrimitiveComponent.CreateDynamicMaterialInstance` _staticmesh 0 (`PrimitiveComponent.GetMaterial` _staticmesh 0)))
  (set `self.DefaultMaterial` _returnvalue_2))