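; Inventory component for the first-person character that stores items in a keyed map and tracks the one held in the right hand.
; EquipItem looks up an item by key, snaps its root component to the component from GetEquipSlot, and records it as held.
; DropRightHand removes the held BP_Equipable by its ItemName through RemoveItem, which clears the hand reference, then calls its Drop.
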(event `self.ReceiveBeginPlay`
  (bind _asfirst_person_character (cast `/Game/Blueprints/FirstPersonCharacter/FirstPersonCharacter` (`self.GetOwner`)))
  (set `self.PlayerRef` _asfirst_person_character))

(fn `Add Item`
  (params (Key :type "String (by ref)") (Value :type "Actor Object Reference (by ref)"))
  (`BlueprintMapLibrary.Map_Add` (`self.Inventory`) Key Value))

(fn `DropRightHand`
  (bind _righhandattached (`self.RighHandAttached`))
  (`/Engine/EditorBlueprintResources/StandardMacros.IsValid` _righhandattached
    (:`Is Valid`
      (bind _asbp_equipable (cast `/Game/Blueprints/Interactables/Equips/BP_Equipable` _righhandattached))
      (`self.Remove Item` (`/Game/Blueprints/Interactables/Equips/BP_Equipable.ItemName` _asbp_equipable))
      (`/Game/Blueprints/Interactables/Equips/BP_Equipable.Drop` _asbp_equipable))))

(fn `Equip Item`
  (params (Key :type "String (by ref)"))
  (returns (Value :type "Actor Object Reference") (Found :type Boolean))
  (locals (HasItemKey :type Boolean) (FoundItem :type "Actor Object Reference"))
  (bind (_value _returnvalue) (`BlueprintMapLibrary.Map_Find` (`self.Inventory`) Key))
  (set `local.FoundItem` _value)
  (bind _output_get (set `local.HasItemKey` _returnvalue))
  (if _output_get
    (bind _returnvalue_2 (`SceneComponent.K2_AttachToComponent` (`Actor.K2_GetRootComponent` (`local.FoundItem`)) (`self.GetEquipSlot`) "None" "SnapToTarget" "SnapToTarget" "SnapToTarget" false))
    (if _returnvalue_2
      (bind _output_get_2 (set `self.RighHandAttached` (`local.FoundItem`)))
      (return _output_get_2 _returnvalue_2))
    (else
      (return null (`local.HasItemKey`)))))

(fn `Remove Item`
  (params (Key :type "String (by ref)"))
  (returns (Found :type Boolean) (Value :type "Actor Object Reference"))
  (bind _inventory (`self.Inventory`))
  (bind (_value _returnvalue) (`BlueprintMapLibrary.Map_Find` _inventory Key))
  (if _returnvalue
    (bind _returnvalue_2 (`BlueprintMapLibrary.Map_Remove` _inventory Key))
    (set `self.RighHandAttached` null)
    (return _returnvalue_2 _value)
    (else
      (return _returnvalue null))))