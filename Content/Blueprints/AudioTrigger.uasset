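; AudioTrigger is an actor that plays a sound when the first-person character overlaps it.
; After a configurable delay, it plays the sound at the position of a referenced location actor, with exposed volume, pitch, start time, attenuation and concurrency settings.
; An optional Destroy flag removes the trigger after a second delay; otherwise it stays and can fire again on later overlaps.
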(event `self.ReceiveActorBeginOverlap`
  (params (OtherActor :type "Actor Object Reference"))
  (cast `/Game/Blueprints/FirstPersonCharacter/FirstPersonCharacter` OtherActor)
  (`KismetSystemLibrary.Delay` (`self.SoundDelay`))
  (`GameplayStatics.PlaySoundAtLocation` (`self.Sound`) (`self.K2_GetActorLocation` (`self.SoundLocation`)) (struct) (`self.Volume`) (`self.Pitch`) (`self.Start Time`) (`self.Attenuation Setting`) (`self.Concurrency Setting`))
  (if (`self.bDestroy`)
    (`KismetSystemLibrary.Delay` (`self.DestroyDelay`))
    (`self.K2_DestroyActor`)))

(fn `UserConstructionScript`)