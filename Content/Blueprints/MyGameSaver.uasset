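; MyGameSaver is an actor that saves and restores a tracked set of actors through a debug save slot.
; Save stores the TrackActors references directly in a new CheckPointSystem save object and prints the write result.
; Load reads that object back, destroys every tracked actor, then calls SpawnActorCopy on each saved entry.
; Its event graph is empty, so both functions rely on external callers.
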(fn `Load`
  (locals (NewLocalVar_0 :type "Array of Actor Object Reference"))
  (bind _returnvalue (`GameplayStatics.LoadGameFromSlot` "DebugSave"))
  (bind _output_get (set `self.SaveGameInstance` _returnvalue))
  (bind _ascheck_point_system (cast `/Game/Blueprints/CheckPointSystem` _output_get))
  (for _array_element (`self.TrackActors`)
    (`self.K2_DestroyActor` _array_element))
  (for _array_element_2 (`/Game/Blueprints/CheckPointSystem.ActorsToSave` _ascheck_point_system)
    (`KismetSystemLibrary.PrintString` (`KismetSystemLibrary.GetDisplayName` _array_element_2))
    (`self.SpawnActorCopy` _array_element_2)))

(fn `Save`
  (bind _returnvalue (`GameplayStatics.CreateSaveGameObject` "/Game/Blueprints/CheckPointSystem.CheckPointSystem_C"))
  (bind _output_get (set `self.SaveGameInstance` _returnvalue))
  (bind _ascheck_point_system (cast `/Game/Blueprints/CheckPointSystem` _output_get))
  (set `/Game/Blueprints/CheckPointSystem.ActorsToSave` (`self.TrackActors`) _ascheck_point_system)
  (bind _returnvalue_2 (`GameplayStatics.SaveGameToSlot` _ascheck_point_system "DebugSave"))
  (`KismetSystemLibrary.PrintString` (`KismetStringLibrary.Conv_BoolToString` _returnvalue_2)))

(fn `UserConstructionScript`)