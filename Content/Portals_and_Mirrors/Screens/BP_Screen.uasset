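; BP_Screen is a screen actor that displays the view of its SceneCaptureComponent2D on a mesh.
; The construction script assigns the screen mesh and scales it by ScreenSize, with zero X scale to flatten it.
; On BeginPlay, InitSceneCapture creates a render target at the set Resolution, makes it the capture's target, and feeds it into a dynamic material instance through the TextureRT parameter.
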(event `self.ReceiveBeginPlay`
  (`self.InitSceneCapture`))

(fn `InitSceneCapture`
  (bind (_resolution_x _resolution_y) (`KismetMathLibrary.BreakVector2D` (`self.Resolution`)))
  (bind _returnvalue (`KismetRenderingLibrary.CreateRenderTarget2D` (`KismetMathLibrary.FTrunc` _resolution_x) (`KismetMathLibrary.FTrunc` _resolution_y)))
  (bind _output_get (set `self.RenderTarget` _returnvalue))
  (set `SceneCaptureComponent2D.TextureTarget` _output_get (`self.SceneCaptureComponent2D`))
  (bind _returnvalue_2 (`PrimitiveComponent.CreateDynamicMaterialInstance` (`self.ScreenMesh`) 0 (`self.ScreenMaterialAsset`)))
  (set `self.MID` _returnvalue_2)
  (`MaterialInstanceDynamic.SetTextureParameterValue` (`self.MID`) "TextureRT" (`self.RenderTarget`)))

(fn `UserConstructionScript`
  (bind (_x _y) (`KismetMathLibrary.BreakVector2D` (`self.ScreenSize`)))
  (`StaticMeshComponent.SetStaticMesh` (`self.ScreenMesh`) (`self.ScreenMeshAsset`))
  (`SceneComponent.SetRelativeScale3D` (`self.ScreenMesh`) (`KismetMathLibrary.MakeVector` 0.0 _x _y)))