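; BP_Mirror is a planar mirror actor that renders a real-time reflection with a SceneCapture2D.
; The construction script sizes the mirror mesh and content window from SurfaceSize.
; BeginPlay creates a viewport-sized or fixed-resolution render target and feeds it to the mirror's dynamic material.
; Each tick mirrors the player camera's transform across the actor's forward plane onto the capture and aligns its clip plane there.
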(event `self.ReceiveBeginPlay`
  (`self.InitSceneCapture`))

(event `self.ReceiveTick`
  (params (DeltaSeconds :type "Float (single-precision)"))
  (`self.UpdateSCC2DTransform`))

(fn `InitSceneCapture`
  (bind (_rt_resolution_x _rt_resolution_y) (`KismetMathLibrary.BreakVector2D` (`self.RT_Resolution`)))
  (bind (_sizex _sizey) (`PlayerController.GetViewportSize` (`GameplayStatics.GetPlayerController` 0)))
  (if (`self.RT_UseViewportSize`)
    (bind _returnvalue (`KismetRenderingLibrary.CreateRenderTarget2D` _sizex _sizey))
    (set `self.RenderTarget` _returnvalue)
    (else
      (bind _returnvalue_2 (`KismetRenderingLibrary.CreateRenderTarget2D` (`KismetMathLibrary.FTrunc` _rt_resolution_x) (`KismetMathLibrary.FTrunc` _rt_resolution_y)))
      (set `self.RenderTarget` _returnvalue_2)))
  (set `SceneCaptureComponent2D.TextureTarget` (`self.RenderTarget`) (`self.SceneCaptureComponent2D`))
  (bind _returnvalue_3 (`PrimitiveComponent.CreateDynamicMaterialInstance` (`self.MirrorMesh`) 0 (`self.MirrorMaterialAsset`)))
  (set `self.MID` _returnvalue_3)
  (`MaterialInstanceDynamic.SetTextureParameterValue` (`self.MID`) "TextureRT" (`self.RenderTarget`)))

(fn `UpdateSCC2DTransform`
  (bind _returnvalue (`self.GetTransform`))
  (bind _returnvalue_2 (`self.GetActorForwardVector`))
  (bind _scenecapturecomponent2d (`self.SceneCaptureComponent2D`))
  (bind (_returnvalue_location _returnvalue_rotation) (`KismetMathLibrary.BreakTransform` (`SceneComponent.K2_GetComponentToWorld` (`PlayerCameraManager.TransformComponent` (`GameplayStatics.GetPlayerCameraManager` 0)))))
  (bind (_x _y) (`KismetMathLibrary.GetAxes` _returnvalue_rotation))
  (set `SceneCaptureComponent2D.ClipPlaneBase` (`self.K2_GetActorLocation`) _scenecapturecomponent2d)
  (set `SceneCaptureComponent2D.ClipPlaneNormal` (`self.GetActorForwardVector`) _scenecapturecomponent2d)
  (set `self.SceneCaptureLocation` (`KismetMathLibrary.TransformLocation` (`KismetMathLibrary.MakeTransform` (.location _returnvalue) (.rotation _returnvalue) (`KismetMathLibrary.MakeVector` (* (.x (.scale _returnvalue)) -1.0) (.y (.scale _returnvalue)) (.z (.scale _returnvalue)))) (`KismetMathLibrary.InverseTransformLocation` _returnvalue _returnvalue_location)))
  (set `self.SceneCaptureRotation` (`KismetMathLibrary.MakeRotFromXY` (`KismetMathLibrary.MirrorVectorByNormal` _x _returnvalue_2) (`KismetMathLibrary.MirrorVectorByNormal` _y _returnvalue_2)))
  (`SceneComponent.K2_SetWorldTransform` _scenecapturecomponent2d (`KismetMathLibrary.MakeTransform` (`self.SceneCaptureLocation`) (`self.SceneCaptureRotation`) (1.0 1.0 -1.0)) false false))

(fn `UserConstructionScript`
  (bind (_surfacesize_x _surfacesize_y _surfacesize_z) (`KismetMathLibrary.BreakVector` (`self.SurfaceSize`)))
  (`StaticMeshComponent.SetStaticMesh` (`self.MirrorMesh`) (`self.MirrorMeshAsset`))
  (`SceneComponent.SetRelativeScale3D` (`self.MirrorMesh`) (`self.SurfaceSize`))
  (`SceneComponent.SetRelativeScale3D` (`self.SM_ContentWindow_01`) (`KismetMathLibrary.MakeVector` (* _surfacesize_x 0.01) (* _surfacesize_y 0.01) (* _surfacesize_z 0.01))))