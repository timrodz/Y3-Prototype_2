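; Physics prop that can pass through linked BP_Portals, carrying its linear velocity with it.
; While overlapping a portal, it shows a duplicate mesh transformed to the target portal, with clip-plane materials slicing both meshes at their portals.
; Each overlapping tick updates that visual, or, if the prop is not held and its origin is behind the portal plane, teleports it with converted location, rotation, scale and velocity.
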(event `self.ReceiveTick`
  (params (DeltaSeconds :type "Float (single-precision)"))
  (if (`self.IsOverlappingPortal`)
    (`self.TeleportationVisualization`)))

(event `self.StaticMesh.OnComponentBeginOverlap`
  (params (OverlappedComponent :type "PrimitiveComponent Object Reference") (OtherActor :type "Actor Object Reference") (OtherComp :type "PrimitiveComponent Object Reference") (OtherBodyIndex :type Integer) (bFromSweep :type Boolean) (SweepResult :type "HitResult Structure (by ref)"))
  (bind _currentportal (`self.CurrentPortal`))
  (bind _asbp_portal (cast `/Game/Portals_and_Mirrors/Portals/BP_Portal` OtherActor))
  (set `self.CurrentPortal` _asbp_portal)
  (set `self.IsOverlappingPortal` true)
  (`self.ToggleComponent` (`self.StaticMeshCopy`) true)
  (`/Game/Portals_and_Mirrors/Portals/BP_Portal.ToggleFrameCollision` _currentportal "NoCollision")
  (`/Game/Portals_and_Mirrors/Portals/BP_Portal.ToggleFrameCollision` (`/Game/Portals_and_Mirrors/Portals/BP_Portal.TargetPortal` _currentportal) "NoCollision")
  (`MaterialInstanceDynamic.SetScalarParameterValue` (`self.MID1`) "UseClipPlane" 1.0)
  (`MaterialInstanceDynamic.SetScalarParameterValue` (`self.MID2`) "UseClipPlane" 1.0))

(event `self.StaticMesh.OnComponentEndOverlap`
  (params (OverlappedComponent :type "PrimitiveComponent Object Reference") (OtherActor :type "Actor Object Reference") (OtherComp :type "PrimitiveComponent Object Reference") (OtherBodyIndex :type Integer))
  (bind _currentportal (`self.CurrentPortal`))
  (cast `/Game/Portals_and_Mirrors/Portals/BP_Portal` OtherActor)
  (set `self.IsOverlappingPortal` false)
  (`self.ToggleComponent` (`self.StaticMeshCopy`))
  (`/Game/Portals_and_Mirrors/Portals/BP_Portal.ToggleFrameCollision` _currentportal "NoCollision")
  (`/Game/Portals_and_Mirrors/Portals/BP_Portal.ToggleFrameCollision` (`/Game/Portals_and_Mirrors/Portals/BP_Portal.TargetPortal` _currentportal) "NoCollision")
  (`MaterialInstanceDynamic.SetScalarParameterValue` (`self.MID1`) "UseClipPlane" 0.0)
  (`MaterialInstanceDynamic.SetScalarParameterValue` (`self.MID2`) "UseClipPlane" 0.0)
  (set `self.CurrentPortal` null))

(fn `Teleportation`
  (locals (TargetLocation :type "Vector Structure") (TargetRotation :type "Rotator Structure") (TargetScale :type "Vector Structure" :default (1.0 1.0 1.0)))
  (bind _staticmesh (`self.StaticMesh`))
  (bind _staticmesh_2 (`self.StaticMesh`))
  (bind _currentportal (`self.CurrentPortal`))
  (bind _currentportal_2 (`self.CurrentPortal`))
  (bind _staticmesh_3 (`self.StaticMesh`))
  (bind _currentportal_3 (`self.CurrentPortal`))
  (bind _currentportal_4 (`self.CurrentPortal`))
  (bind _targetportal (`/Game/Portals_and_Mirrors/Portals/BP_Portal.TargetPortal` _currentportal))
  ;[1 1 1] Location
  (bind _newlocation (`/Game/Portals_and_Mirrors/Base/BP/BP_PortalsFunctions.PortalConvertLocationMirrored` _currentportal _targetportal (`SceneComponent.K2_GetComponentLocation` _staticmesh_3)))
  (bind _output_get (set `local.TargetLocation` (+ _newlocation (* (`self.GetActorForwardVector` _targetportal) 10.0))))
  (`SceneComponent.K2_SetWorldLocation` _staticmesh_3 _output_get false true)
  ;[1 1 1] Rotation
  (bind _newrotation (`/Game/Portals_and_Mirrors/Base/BP/BP_PortalsFunctions.PortalConvertRotation` _currentportal_2 (`/Game/Portals_and_Mirrors/Portals/BP_Portal.TargetPortal` _currentportal_2) (`SceneComponent.K2_GetComponentRotation` _staticmesh_2)))
  (bind _output_get_2 (set `local.TargetRotation` _newrotation))
  (`SceneComponent.K2_SetWorldRotation` _staticmesh_2 _output_get_2 false false)
  ;[1 0 0] Scale
  (set `local.TargetScale` (/ (`self.GetActorScale3D` (`/Game/Portals_and_Mirrors/Portals/BP_Portal.TargetPortal` _currentportal_3)) (`self.GetActorScale3D` _currentportal_3)))
  (if (not (== (`local.TargetScale`) (1.0 1.0 1.0)))
    (`SceneComponent.SetWorldScale3D` (`self.StaticMesh`) (`local.TargetScale`)))
  ;[1 0 0] This works somehow...
  (bind _returnvalue (`PrimitiveComponent.GetPhysicsLinearVelocity` _staticmesh "None"))
  (bind _output_get_3 (set `self.VelocityPrev` _returnvalue))
  (bind _newvelocity (`/Game/Portals_and_Mirrors/Base/BP/BP_PortalsFunctions.PortalConvertVelocity` _currentportal_4 (`/Game/Portals_and_Mirrors/Portals/BP_Portal.TargetPortal` _currentportal_4) _output_get_3))
  (bind _output_get_4 (set `self.VelocityNew` _newvelocity))
  (`PrimitiveComponent.SetPhysicsLinearVelocity` _staticmesh _output_get_4 false "None"))

(fn `TeleportationVisualization`
  (bind _returnvalue (`self.K2_GetActorLocation`))
  (bind _currentportal (`self.CurrentPortal`))
  (bind _returnvalue_2 (`self.GetActorForwardVector` _currentportal))
  (if (`self.IsHeld`)
    (`self.UpdateComponents` :!label _label)
    (else
      (bind _output_get (set `self.ProjectedDistance` (`KismetMathLibrary.Dot_VectorVector` (- _returnvalue (`KismetMathLibrary.ProjectPointOnToPlane` _returnvalue (`self.K2_GetActorLocation` _currentportal) _returnvalue_2)) _returnvalue_2)))
      (if (< _output_get 0.0)
        (`self.Teleportation`)
        (else
          (goto _label))))))

(fn `ToggleComponent`
  (params (Component :type "PrimitiveComponent Object Reference") (On :type Boolean))
  (if On
    (`SceneComponent.SetVisibility` Component true false)
    (else
      (`SceneComponent.SetVisibility` Component false false))))

(fn `UpdateComponents`
  (bind _currentportal (`self.CurrentPortal`))
  (bind _currentportal_2 (`self.CurrentPortal`))
  (bind _mid2 (`self.MID2`))
  (bind _mid1 (`self.MID1`))
  (bind _currentportal_3 (`self.CurrentPortal`))
  (bind _currentportal_4 (`self.CurrentPortal`))
  (bind _targetportal (`/Game/Portals_and_Mirrors/Portals/BP_Portal.TargetPortal` (`self.CurrentPortal`)))
  (bind _targetportal_2 (`/Game/Portals_and_Mirrors/Portals/BP_Portal.TargetPortal` _currentportal_4))
  ;[1 1 1] Update material clip plane
  (`MaterialInstanceDynamic.SetVectorParameterValue` _mid1 "ClipPlaneBase" (`KismetMathLibrary.Conv_VectorToLinearColor` (`self.K2_GetActorLocation` _currentportal_3)))
  (`MaterialInstanceDynamic.SetVectorParameterValue` _mid1 "ClipPlaneNormal" (`KismetMathLibrary.Conv_VectorToLinearColor` (`self.GetActorForwardVector` _currentportal_3)))
  ;[1 1 1] Location
  (bind _newlocation (`/Game/Portals_and_Mirrors/Base/BP/BP_PortalsFunctions.PortalConvertLocation` _currentportal (`/Game/Portals_and_Mirrors/Portals/BP_Portal.TargetPortal` _currentportal) (`SceneComponent.K2_GetComponentLocation` (`self.StaticMesh`))))
  (`SceneComponent.K2_SetWorldLocation` (`self.StaticMeshCopy`) _newlocation false false)
  ;[1 1 1] Rotation
  (bind _newrotation (`/Game/Portals_and_Mirrors/Base/BP/BP_PortalsFunctions.PortalConvertRotation` _currentportal_2 (`/Game/Portals_and_Mirrors/Portals/BP_Portal.TargetPortal` _currentportal_2) (`SceneComponent.K2_GetComponentRotation` (`self.StaticMesh`))))
  (`SceneComponent.K2_SetWorldRotation` (`self.StaticMeshCopy`) _newrotation false false)
  ;[1 1 1] Scale
  (if (not (== (`self.GetActorScale3D` _currentportal_4) (`self.GetActorScale3D` _targetportal_2)))
    (`SceneComponent.SetWorldScale3D` (`self.StaticMeshCopy`) (/ (`self.GetActorScale3D` _targetportal_2) (`self.GetActorScale3D` _currentportal_4))))
  ;[1 1 1] Update material clip plane
  (`MaterialInstanceDynamic.SetVectorParameterValue` _mid2 "ClipPlaneBase" (`KismetMathLibrary.Conv_VectorToLinearColor` (`self.K2_GetActorLocation` _targetportal)))
  (`MaterialInstanceDynamic.SetVectorParameterValue` _mid2 "ClipPlaneNormal" (`KismetMathLibrary.Conv_VectorToLinearColor` (`self.GetActorForwardVector` _targetportal))))

(fn `UserConstructionScript`
  (bind _meshasset (`self.MeshAsset`))
  (bind _materialasset (`self.MaterialAsset`))
  (`|ExecutionSequence`
    (:`then_0`
      (`StaticMeshComponent.SetStaticMesh` (`self.StaticMesh`) _meshasset)
      (bind _returnvalue (`KismetMaterialLibrary.CreateDynamicMaterialInstance` _materialasset))
      (bind _output_get (set `self.MID1` _returnvalue))
      (`PrimitiveComponent.SetMaterial` (`self.StaticMesh`) 0 _output_get))
    (:`then_1`
      (`StaticMeshComponent.SetStaticMesh` (`self.StaticMeshCopy`) _meshasset)
      (bind _returnvalue_2 (`KismetMaterialLibrary.CreateDynamicMaterialInstance` _materialasset))
      (bind _output_get_2 (set `self.MID2` _returnvalue_2))
      (`PrimitiveComponent.SetMaterial` (`self.StaticMeshCopy`) 0 _output_get_2))))