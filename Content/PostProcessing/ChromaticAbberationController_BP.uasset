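; Actor Blueprint that controls a post-process effect, named for chromatic aberration, through the blend weight of its PostProcess component.
; Enable and Disable switch the effect fully on or off, while SetBlendWeight applies any given weight.
; A Sine timeline is wired to drive the blend weight, but nothing starts it, so changes come only through those functions.
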(fn `Disable`
  (set `PostProcessComponent.BlendWeight` 0.0 (`self.PostProcess`)))

(fn `Enable`
  (set `PostProcessComponent.BlendWeight` 1.0 (`self.PostProcess`)))

(fn `SetBlendWeight`
  (params (BlendWeight :type "Float (double-precision)"))
  (set `PostProcessComponent.BlendWeight` BlendWeight (`self.PostProcess`)))

(fn `UserConstructionScript`)