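; Inspectable, collectible polaroid actor whose photo is a live render of a scene capture.
; On BeginPlay it gives mesh material slot 1 a dynamic instance fed by a new render target, then has the linked SceneCaptureBP render into it.
; Capture re-renders between pre- and post-capture calls, and EditorCapture triggers a plain capture.
; Inspect events forward to begin and end handlers, and ending inspection marks it collected.
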(event `self.OnEndInspect`
  (`self.EndInspect`)
  (set `self.bCollected` true))

(event `self.OnBeginInspect`
  (params (Actor :type "Actor Object Reference"))
  (`self.BeginInspect` Actor))

(event `self.ReceiveBeginPlay`
  (bind _scenecapturebp (`self.SceneCaptureBP`))
  (bind _returnvalue (`PrimitiveComponent.CreateDynamicMaterialInstance` (`self.StaticMesh`) 1 (`self.Material`)))
  (`/Engine/EditorBlueprintResources/StandardMacros.IsValid` _returnvalue
    (:`Is Valid`
      (bind _output_get (set `self.MaterialInstance` _returnvalue))
      (`PrimitiveComponent.SetMaterial` (`self.StaticMesh`) 1 _output_get)
      (bind _returnvalue_2 (`KismetRenderingLibrary.CreateRenderTarget2D` 1024 1024))
      (bind _output_get_2 (set `self.RenderTarget` _returnvalue_2))
      (`MaterialInstanceDynamic.SetTextureParameterValue` _output_get "RenderTarget" _output_get_2)
      (bind _output_get_3 (set `SceneCaptureComponent2D.TextureTarget` _output_get_2 (`SceneCapture2D.CaptureComponent2D` _scenecapturebp)))
      (`/Game/Assets/2D/SceneCapture_2D_BP.Capture` :`self` _scenecapturebp :`TextureTarget` _output_get_3))))

(event `Capture`
  (`self.PreCapture`)
  (`/Game/Assets/2D/SceneCapture_2D_BP.Capture` :`self` (`self.SceneCaptureBP`) :`TextureTarget` (`self.RenderTarget`))
  (`self.PostCapture`))

(fn `EditorCapture`
  (`/Game/Assets/2D/SceneCapture_2D_BP.Capture` :`self` (`self.SceneCaptureBP`) :`TextureTarget` (`self.RenderTarget`)))

(fn `UserConstructionScript`
  (set `self.OriginalLocation` (`SceneComponent.K2_GetComponentLocation` (`self.StaticMesh`)))
  (set `self.OriginalRotation` (`SceneComponent.K2_GetComponentRotation` (`self.StaticMesh`))))