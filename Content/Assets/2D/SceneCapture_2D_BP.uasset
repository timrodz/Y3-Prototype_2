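; SceneCapture_2D_BP is a scene capture Blueprint that renders the scene to a render target and exports it to a file.
; Capture calls CaptureScene only when OverideLocation is true, leaving its target, location and rotation inputs unused.
; ExportRenderTargetToFile writes the component's render target to a hardcoded local repository path under a given file name.
; Logic to assign the target and match the first-person camera's transform is disconnected.
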(event `Capture`
  (params (TextureTarget :type "TextureRenderTarget2D Object Reference") (bOverideLocation :type Boolean) (OverrideLocation :type "Vector Structure") (OverrideRotation :type "Rotator Structure"))
  (if bOverideLocation
    (`SceneCaptureComponent2D.CaptureScene` (`self.CaptureComponent2D`))))

(event `ExportRenderTargetToFile`
  (params (FileName :type String))
  (`KismetRenderingLibrary.ExportRenderTarget` (`SceneCaptureComponent2D.TextureTarget` (`self.CaptureComponent2D`)) "D:\\Source Tree - Repositories\\Y3-Prototype_2" FileName))

(fn `UserConstructionScript`)